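; Scrap Blueprint ("poubelle", trash) that stores abandoned grappling-hook and swing experiments; none of its logic runs.
; Grapple fragments cover deprecated physics constraints, a height check against the grab point, timeline velocity boosts and a speed-limited swing on the player capsule.
; A separate debug snippet looks up a hit mesh's material by collision face index and prints name comparisons.
; Unconnected vector-math nodes remain, and the construction script is empty.
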(fn `UserConstructionScript`)