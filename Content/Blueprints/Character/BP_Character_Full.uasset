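; BP_Character_Full is the merged form of the player character, which can split into separate top and bottom characters.
; On BeginPlay it plays a timeline squash on its sprite as fusion feedback.
; Separate spawns both halves with its facing, velocity and camera trigger, partners them, possesses the top with matching camera rotation, then destroys itself.
; Respawn teleports it to the camera manager's checkpoint, if valid; Pull is empty.
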(event `self.ReceiveBeginPlay`
  (`parent.ReceiveBeginPlay`)
  (set `self.SpriteBaseScale` (`SceneComponent.RelativeScale3D` (`self.Sprite`)))
  (`self.FusionSqueeze`) ; le corps de squash lors de la création (après avoir fusionné)
)

(event `FusionSqueeze`
  (`TimelineComponent.SetPlayRate` (`self.FusionSqueezeAnim`) (`self.FusionSqueezeRate`))
  (bind (_direction _alpha) (`Timeline|FusionSqueezeAnim` :!via `PlayFromStart`)
    (:`Update`
      (`SceneComponent.SetRelativeScale3D` (`self.Sprite`) (`KismetMathLibrary.VLerp` (`self.SpriteBaseScale`) (* (`self.SpriteBaseScale`) (`self.FusionSqueezeFactor`)) _alpha)))))

(fn `Pull`)

(fn `Respawn`
  (`parent.Respawn`)
  (bind (_asbp_camera_manager _pawntarget _uideathref _checkpoint) (`/Game/Blueprints/Library/BPFL_Fonction_Library.GetCameraManager`))
  (`/Engine/EditorBlueprintResources/StandardMacros.IsValid` _checkpoint
    (:`Is Valid`
      (`/Game/Blueprints/Objects/BP_Checkpoint.TpToCheckPoint` _checkpoint self))))

(fn `Separate`
  (bind _returnvalue (`self.GetTransform`))
  (bind _returnvalue_2 (`self.GetVelocity`))
  (bind _ismovingfront (`self.IsMovingFront`))
  (bind _currentcameratrigger (`self.CurrentCameraTrigger`))
  (bind _isfacingright (`self.IsFacingRight`))
  (bind _isfacingfront (`self.IsFacingFront`))
  (cast `/Game/Blueprints/BP_Player_Controller` (`GameplayStatics.GetPlayerController` 0))
  (`parent.Separate`)
  (`PrimitiveComponent.SetCollisionEnabled` (`self.CapsuleComponent`) "NoCollision")
  (bind _returnvalue_3 (`|SpawnActorFromClass` "/Game/Blueprints/Character/BP_Character_Bottom.BP_Character_Bottom_C" (`KismetMathLibrary.MakeTransform` (`KismetMathLibrary.TransformLocation` _returnvalue (0.0 0.0 -10.0))) "Undefined" "MultiplyWithRoot" null _isfacingright _isfacingfront _ismovingfront _returnvalue_2 (0.0 0.0 0.0) _currentcameratrigger null))
  (bind _returnvalue_4 (`|SpawnActorFromClass` "/Game/Blueprints/Character/BP_Character_Top.BP_Character_Top_C" (`KismetMathLibrary.MakeTransform` (`KismetMathLibrary.TransformLocation` _returnvalue (0.0 0.0 18.0))) "Undefined" "MultiplyWithRoot" null _isfacingright _isfacingfront _ismovingfront _returnvalue_2 (0.0 0.0 0.0) _currentcameratrigger null))
  (`/Game/Blueprints/Character/BP_Character_Top.SetPartner` _returnvalue_4 _returnvalue_3)
  (bind _asbp_player_controller (cast `/Game/Blueprints/BP_Player_Controller` (`GameplayStatics.GetPlayerController` 0)))
  (`Controller.Possess` _asbp_player_controller _returnvalue_4)
  (`self.SetCamZRotation` _returnvalue_4 (.yaw (`SpringArmComponent.GetTargetRotation` (`self.SpringArm`))))
  (`self.K2_DestroyActor`))

(fn `UserConstructionScript`)