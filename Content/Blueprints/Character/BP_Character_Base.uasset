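; Base character for a flipbook-sprite game, handling movement setup, idle/walk animation and a debug dash.
; Jumps gain coyote time via a falling timer in CanJumpInternal, plus velocity-scaled trace buffering that replays on landing with a sprite squeeze.
; A looping timer keeps depth-of-field focus on the sprite.
; Tick eases clamped spring-arm yaw tilt toward the camera manager's target by curve, mirrored to the BPC_Death partner; depth speed boost is disconnected.
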(event `self.ReceiveBeginPlay`
  (bind _currentcameratrigger (`self.CurrentCameraTrigger`))
  (`|ExecutionSequence`
    (:`then_0`
      (set `CharacterMovementComponent.JumpZVelocity` (`self.CharacterJumpHeight`) (`self.CharacterMovement`))
      (set `CharacterMovementComponent.MaxWalkSpeed` (`self.CharacterSpeed`) (`self.CharacterMovement`))
      (set `self.BaseScale` (`SceneComponent.RelativeScale3D` (`self.Sprite`))))
    (:`then_1`
      (`self.HandleRotation`)
      (bind (_asbp_camera_manager _pawntarget) (`/Game/Blueprints/Library/BPFL_Fonction_Library.GetCameraManager`))
      (bind _output_get (set `self.CamManager` _asbp_camera_manager))
      (`/Engine/EditorBlueprintResources/StandardMacros.IsValid` _pawntarget
        (:`Is Not Valid`
          (set `/Game/Blueprints/BP_Camera_Manager.PawnTarget` self _output_get))))
    (:`then_2`
      (`KismetSystemLibrary.K2_SetTimer` null "FocusUpdate" 0.1 true)
      (`/Engine/EditorBlueprintResources/StandardMacros.IsValid` _currentcameratrigger
        (:`Is Valid`
          (`/Game/Blueprints/Objects/BP_CameraTrigger.InstantCamUpdate` _currentcameratrigger self)
          (`self.FocusUpdate`))))))

(event `Key|RightMouseButton`
  (params (Key :type "Key Structure"))
  ;[1 1 1] debug dash
  (:`Pressed`
    (if (`self.IsFacingRight`)
      (`self.LaunchCharacter` (1000.0 0.0 500.0))
      (else
        (`self.LaunchCharacter` (-1000.0 0.0 500.0))))))

(event `self.ReceiveTick`
  (params (DeltaSeconds :type "Float (single-precision)"))
  (`self.HandleAnimation`)
  (`self.CamTiltTick`)
  (`self.SpeedBoostOnYAxis`)
  (bind (_outhit _returnvalue) (`KismetSystemLibrary.LineTraceSingle` (`SceneComponent.K2_GetComponentLocation` (`self.RaySource`)) (`SceneComponent.K2_GetComponentLocation` (`self.RaySourceEnd`)) "TraceTypeQuery1"))
  (set `self.Grounded` _returnvalue))

(event `FocusUpdate`
  (bind _camera (`self.Camera`))
  ;[1 1 1] autoDOF
  (bind _output_get (set `self.FocusDistance` (`KismetMathLibrary.VSize` (- (`SceneComponent.K2_GetComponentLocation` (`self.Sprite`)) (`SceneComponent.K2_GetComponentLocation` _camera)))))
  (set `CameraComponent.PostProcessSettings` (make `PostProcessSettings` :`DepthOfFieldFstop` 1.0 :`DepthOfFieldMinFstop` 11.0 :`AmbientOcclusionTemporalBlendWeight` 0.0 :`DepthOfFieldSensorWidth` (`self.Sensor Width (Mm)`) :`DepthOfFieldFocalDistance` _output_get) _camera))

(event `self.K2_OnMovementModeChanged`
  (params (PrevMovementMode :type "EMovementMode Enum" :default "MOVE_None") (NewMovementMode :type "EMovementMode Enum" :default "MOVE_None") (PrevCustomMode :type Byte) (NewCustomMode :type Byte))
  ;[1 1 1] Coyote Time & Jump Buffering
  (if (`|EnumEquality` NewMovementMode "MOVE_Falling")
    (bind _returnvalue (`KismetSystemLibrary.K2_SetTimerDelegate` (delegate `CoyoteTimePassed`) (`self.CoyoteTimeDuration`)))
    (set `self.CoyoteTime` _returnvalue)))

(event `CoyoteTimePassed`
  ;[1 1 1] Coyote Time & Jump Buffering
)

(event `self.OnLanded`
  (params (Hit :type "HitResult Structure (by ref)"))
  ;[1 1 1] Coyote Time & Jump Buffering
  (`KismetSystemLibrary.K2_ClearAndInvalidateTimerHandle` (`self.CoyoteTime`))
  (if (`self.JumpBuffered`)
    (`self.JumpSqueeze`)
    (`KismetSystemLibrary.Delay` 0.001)
    (`self.Jump`)
    (set `self.JumpBuffered` false)))

(event `RayTraceToPlayer`
  (bind _returnvalue (`SceneComponent.K2_GetComponentLocation` (`self.Camera`)))
  ;[1 1 1] raycast qui pointe le joueur
  (`KismetSystemLibrary.LineTraceSingleForObjects` :`Start` _returnvalue :`End` (+ _returnvalue (* (`KismetMathLibrary.GetForwardVector` (`KismetMathLibrary.FindLookAtRotation` _returnvalue (`SceneComponent.K2_GetComponentLocation` (`self.CapsuleComponent`)))) 2000.0)) :`ObjectTypes` (`|MakeArray` "ObjectTypeQuery3" :!type "EObjectTypeQuery Enum") :`bIgnoreSelf` false))

(event `BufferJump`
  (bind _returnvalue (`SceneComponent.K2_GetComponentLocation` (`self.RaySourceEnd`)))
  ;[1 1 1] Coyote Time & Jump Buffering
  (bind (_outhit _returnvalue_2) (`KismetSystemLibrary.LineTraceSingle` _returnvalue (+ _returnvalue (`KismetMathLibrary.MakeVector` 0.0 0.0 (`KismetMathLibrary.FClamp` (* (`self.JumpBufferDistanceFactor`) (.z (`self.GetVelocity`))) -100.0 0.0))) "TraceTypeQuery1"))
  (set `self.JumpBuffered` _returnvalue_2))

(event `JumpSqueeze`
  ;[1 1 1] JumpSqueeze
  (`TimelineComponent.SetPlayRate` (`self.JumpSqueezeAnim`) (`self.JumpSqueezeSpeed`))
  (bind (_direction _alpha) (`Timeline|JumpSqueezeAnim` :!via `PlayFromStart`)
    (:`Update`
      (`SceneComponent.SetRelativeScale3D` (`self.Sprite`) (`KismetMathLibrary.VLerp` (`self.BaseScale`) (* (`self.BaseScale`) (`self.SqueezeFactor`)) _alpha)))))

(event `TiltCam`
  (params (A :type "Float (double-precision)"))
  (bind _cammanager (`self.CamManager`))
  (bind _tiltcammaxangle (`self.TiltCamMaxAngle`))
  (bind _returnvalue (- (`/Game/Blueprints/BP_Camera_Manager.FuturCamTilt` _cammanager) (`/Game/Blueprints/BP_Camera_Manager.BaseCamTilt` _cammanager)))
  ;[1 1 1] TiltCam
  ;;[1 1 1] reset si demi tour en plein mouvement (attention un input renvoie zero au début de l'appuie)
  (if (and (!= A 0.0) (!= A (/ _returnvalue (`KismetMathLibrary.Abs` _returnvalue))))
    (`self.ResetBaseCam`))
  (set `/Game/Blueprints/BP_Camera_Manager.FuturCamTilt` (`KismetMathLibrary.FClamp` (+ (* A (`self.TiltCamSpeed`)) (`/Game/Blueprints/BP_Camera_Manager.FuturCamTilt` (`self.CamManager`))) (- -90.0 _tiltcammaxangle) (+ -90.0 _tiltcammaxangle)) (`self.CamManager`)))

(event `HandleAnimation`
  (bind (_returnvalue_x _returnvalue_y _returnvalue_z) (`KismetMathLibrary.BreakVector` (`self.GetVelocity`)))
  ;[1 1 1] handle animation
  (if (`NavMovementComponent.IsFalling` (`self.CharacterMovement`))
    (`PaperFlipbookComponent.SetFlipbook` (`self.Sprite`) (select `bool` (< _returnvalue_z 0.0) :`false` (`self.IdleAnim`) :`true` (`self.WalkAnim`)))
    (else
      (`PaperFlipbookComponent.SetFlipbook` (`self.Sprite`) (select `bool` (> (`KismetMathLibrary.VSize` (`MovementComponent.Velocity` (`self.CharacterMovement`))) 0.0) :`false` (`self.IdleAnim`) :`true` (`self.WalkAnim`))))))

(event `CamTiltTick`
  (bind _cammanager (`self.CamManager`))
  (bind _cammanager_2 (`self.CamManager`))
  (bind _tiltcammaxangle (`self.TiltCamMaxAngle`))
  (bind _basecamtilt (`/Game/Blueprints/BP_Camera_Manager.BaseCamTilt` _cammanager))
  (bind _yaw (.yaw (`SpringArmComponent.GetTargetRotation` (`self.SpringArm`))))
  (bind _returnvalue (- (`/Game/Blueprints/BP_Camera_Manager.FuturCamTilt` _cammanager_2) (`/Game/Blueprints/BP_Camera_Manager.BaseCamTilt` _cammanager_2)))
  (bind _returnvalue_2 (/ (`KismetMathLibrary.Abs` (- (/ _yaw _basecamtilt) 1.0)) (`KismetMathLibrary.Abs` (- (/ (`/Game/Blueprints/BP_Camera_Manager.FuturCamTilt` _cammanager) _basecamtilt) 1.0))))
  ;[1 1 1] TiltCam
  (if (!= (`/Game/Blueprints/BP_Camera_Manager.FuturCamTilt` (`self.CamManager`)) _yaw)
    (`self.SetCamZRotation` (`KismetMathLibrary.SelectFloat` (`KismetMathLibrary.FClamp` (+ _yaw (* (`CurveFloat.GetFloatValue` (`self.curveCAmTilt`) _returnvalue_2) (/ _returnvalue (`KismetMathLibrary.Abs` _returnvalue)) 0.2)) (- -90.0 _tiltcammaxangle) (+ -90.0 _tiltcammaxangle)) (`/Game/Blueprints/BP_Camera_Manager.FuturCamTilt` (`self.CamManager`)) (<= _returnvalue_2 0.995)))
    (else
      (`self.ResetBaseCam`))))

(event `SetCamZRotation`
  (params (`New Rotation Z` :type "Float (single-precision)"))
  (bind _returnvalue (`self.GetComponentByClass` "/Game/Blueprints/Character/Components/BPC_Death.BPC_Death_C"))
  (bind _springarm (`self.SpringArm`))
  (bind _partnerindeath (`/Game/Blueprints/Character/Components/BPC_Death.PartnerInDeath` _returnvalue))
  ;[1 1 1] TiltCam
  (`|ExecutionSequence`
    (:`then_0`
      (`SceneComponent.K2_SetWorldRotation` _springarm (`KismetMathLibrary.MakeRotator` (.roll (`SpringArmComponent.GetTargetRotation` _springarm)) (.pitch (`SpringArmComponent.GetTargetRotation` _springarm)) `New Rotation Z`) false false))
    (:`then_1`
      ;;[1 1 1] le player actuellement controlée update son partenaire aussi s'il en as un
      (if (== (`/Game/Blueprints/Library/BPFL_Fonction_Library.CastToPlayerCharacter`) self)
        (`/Engine/EditorBlueprintResources/StandardMacros.IsValid` _returnvalue
          (:`Is Valid`
            (`/Engine/EditorBlueprintResources/StandardMacros.IsValid` _partnerindeath
              (:`Is Valid`
                (`self.SetCamZRotation` _partnerindeath `New Rotation Z`)))))))))

(event `ResetBaseCam`
  ;[1 1 1] TiltCam
  (set `/Game/Blueprints/BP_Camera_Manager.BaseCamTilt` (.yaw (`SpringArmComponent.GetTargetRotation` (`self.SpringArm`))) (`self.CamManager`)))

(event `HandleRotation`
  (bind _sprite (`self.Sprite`))
  ;[1 1 1] handle rotation
  (if (`self.IsFacingRight`)
    (`SceneComponent.K2_SetRelativeRotation` :`self` _sprite)
    (else
      (`SceneComponent.K2_SetRelativeRotation` _sprite (struct :`Yaw` 180.0) false false))))

(event `ResetCamTilt`
  ;[1 1 1] reset
  (`self.ResetBaseCam`)
  (set `/Game/Blueprints/BP_Camera_Manager.FuturCamTilt` -90.0 (`self.CamManager`)))

(event `SpeedBoostOnYAxis`
  ;[1 1 1] Augmenter la vitesse si tu bouge en profondeur
)

(fn `CanJumpInternal`
  (returns (ReturnValue :type Boolean))
  (bind _returnvalue (`parent.CanJumpInternal`))
  (return (or _returnvalue (> (`KismetSystemLibrary.K2_GetTimerRemainingTimeHandle` (`self.CoyoteTime`)) 0.0))))

(fn `Interact`
  (`/Game/Blueprints/Objects/InputObjects/BP_Interactable.Interract` (`self.Interactable`)))

(fn `Respawn`)

(fn `Separate`)

(fn `UserConstructionScript`
  (`CapsuleComponent.SetCapsuleHalfHeight` (`self.CapsuleComponent`) (`self.CharacterHeight`) true))