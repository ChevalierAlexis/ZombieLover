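; BP_Character_Top is the top half of a splittable character, paired with BP_Character_Bottom as death partner and respawning it alongside itself.
; On BeginPlay it launches itself using its initial velocity, facing and depth movement.
; Separate hands possession to the first bottom half found, restoring that half's velocity afterwards.
; The handover waits for a camera blend if the bottom was recently rendered, otherwise possesses halfway through a timeline-driven screen fade.
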(event `MySeparate`
  (params (BlendTime :type "Float (single-precision)") (Target :type "PlayerController Object Reference") (InPawn :type "Pawn Object Reference"))
  (if (`self.WasRecentlyRendered` InPawn 0.0)
    (`PlayerController.SetViewTargetWithBlend` Target InPawn BlendTime "VTBlend_EaseInOut" 2.0 false)
    (`KismetSystemLibrary.Delay` BlendTime)
    ;[1 1 1] Se souvenir de la velocité de la partie juste avant de la possess (donc après le delay)
    (bind _outactors (`GameplayStatics.GetAllActorsOfClass` "/Game/Blueprints/Character/BP_Character_Bottom.BP_Character_Bottom_C" :!label _label))
    (bind _output (`|GetArrayItem` _outactors))
    (bind _output_get (set `/Game/Blueprints/Character/BP_Character_Base.OldVelocity` (`self.GetVelocity` _output) _output))
    (`Controller.Possess` Target InPawn)
    (set `MovementComponent.Velocity` _output_get (`Character.CharacterMovement` _output))
    (else
      ;[1 1 1] Fade
      (`|ExecutionSequence`
        (:`then_0`
          (`KismetSystemLibrary.Delay` (/ BlendTime 2.0))
          (goto _label))
        (:`then_1`
          (`TimelineComponent.SetPlayRate` (`self.fading`) (/ 1.0 BlendTime))
          (bind (_direction _alpha) (`Timeline|Fading` :!via `PlayFromStart`)
            (:`Update`
              (`PlayerCameraManager.SetManualCameraFade` (`GameplayStatics.GetPlayerCameraManager` 0) _alpha (struct :`A` 1.0) false))))))))

(event `self.ReceiveBeginPlay`
  (`parent.ReceiveBeginPlay`)
  (`|ExecutionSequence`
    (:`then_0`
      (if (`self.IsMovingFront`)
        ;[1 1 1] lauch vers avant ou arrière s'il bougeait  en profondeur
        (if (`self.IsFacingRight`)
          (set `self.LaunchX` 1.0)
          (else
            (bind _output_get (set `self.LaunchX` -1.0))))
        (if (`self.IsFacingFront`)
          (set `self.LaunchY` 1.0)
          (else
            (bind _output_get_2 (set `self.LaunchY` -1.0))))
        (`self.LaunchCharacter` (`self.InitialVelocity`))
        (`self.LaunchCharacter` (`KismetMathLibrary.MakeVector` (* _output_get 20.0) (* _output_get_2 70.0) (`self.LaunchHeight`)) false true)
        (else
          ;[1 1 1] lauch vers droite ou gauche s'il bougeait pas en profondeur
          (`self.JumpSqueeze`)
          (if (`self.IsFacingRight`)
            (set `self.LaunchX` 1.0)
            (else
              (bind _output_get_3 (set `self.LaunchX` -1.0))))
          (`self.LaunchCharacter` (`self.InitialVelocity`))
          (`self.LaunchCharacter` (`KismetMathLibrary.MakeVector` (* _output_get_3 70.0) 0.0 (`self.LaunchHeight`)) false true))))))

(event `SetPartner`
  (params (BottomRef :type "/Game/Blueprints/Character/BP_Character_Bottom Object Reference"))
  ;[1 1 1] setPartner
  (bind _output_get (set `/Game/Blueprints/Character/Components/BPC_Death.PartnerInDeath` BottomRef (`self.BPC_Death`)))
  (`/Game/Blueprints/Character/BP_Character_Bottom.SetPartner` BottomRef self))

(fn `MergeObject`
  (params (ObjectToMerge :type "Object Object Reference")))

(fn `Respawn`
  (`parent.Respawn`)
  (bind _asbp_character_bottom (cast `/Game/Blueprints/Character/BP_Character_Bottom` (`/Game/Blueprints/Character/Components/BPC_Death.PartnerInDeath` (`self.BPC_Death`))))
  (`/Game/Blueprints/Character/BP_Character_Bottom.Respawn` _asbp_character_bottom))

(fn `Separate`
  (`parent.Separate`)
  (bind _outactors (`GameplayStatics.GetAllActorsOfClass` "/Game/Blueprints/Character/BP_Character_Bottom.BP_Character_Bottom_C"))
  (bind _asbp_player_controller (cast `/Game/Blueprints/BP_Player_Controller` (`GameplayStatics.GetPlayerController` 0)))
  (`self.MySeparate` (`self.camTransitionSpeed`) _asbp_player_controller (`|GetArrayItem` _outactors)))

(fn `UserConstructionScript`
  (`parent.UserConstructionScript`))