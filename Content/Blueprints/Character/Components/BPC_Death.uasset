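; BPC_Death is a character component that tracks death and links it to a partner actor.
; GetKilled first calls Die on the BPC_Death of PartnerInDeath, if both are valid, then calls its own Die.
; Die sets IsDead once and prints it, with no other death behavior.
; The partner receives Die rather than GetKilled, so death does not propagate further along a chain of partners.
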(event `self.ReceiveBeginPlay`
  (set `self.Owner` (`self.GetOwner`)))

(event `GetKilled`
  (bind _partnerindeath (`self.PartnerInDeath`))
  (bind _returnvalue (`Actor.GetComponentByClass` _partnerindeath "BPC_Death_C"))
  (`|ExecutionSequence`
    (:`then_0`
      (`/Engine/EditorBlueprintResources/StandardMacros.IsValid` _partnerindeath
        (:`Is Valid`
          (`/Engine/EditorBlueprintResources/StandardMacros.IsValid` _returnvalue
            (:`Is Valid`
              (`self.Die` _returnvalue))))))
    (:`then_1`
      (`self.Die`))))

(event `Die`
  (if (not (`self.IsDead`))
    (bind _output_get (set `self.IsDead` true))
    (`KismetSystemLibrary.PrintString` (`KismetStringLibrary.Conv_BoolToString` _output_get))))