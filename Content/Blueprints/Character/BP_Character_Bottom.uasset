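; Lower half of the splittable player character, launched on spawn, with a debug-key kick animation.
; When the top half overlaps MergeCollision without rising, both halves are replaced by a possessed BP_Character_Full.
; Separate switches control to the top, blending the camera or fading if it is off-screen, and preserves its velocity through possession.
; Respawn force-merges with the death component's partner before respawning the full character; object merging is stubbed.
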(event OnComponentBeginOverlap(MergeCollision)
  (params (OverlappedComponent :type Primitive%20Component%20Object%20Reference) (OtherActor :type Actor%20Object%20Reference) (OtherComp :type Primitive%20Component%20Object%20Reference) (OtherBodyIndex :type Integer) (bFromSweep :type Boolean) (SweepResult :type Hit%20Result%20Structure%20%28by%20ref%29))
  ;[1 1 1] Merge Character or Object
  (bind _asbp_character_top (Utilities|Casting|CastToBP_Character_Top OtherActor))
  (Variables|Default|SetTopWantToMerge true))

(event OnComponentEndOverlap(MergeCollision)
  (params (OverlappedComponent :type Primitive%20Component%20Object%20Reference) (OtherActor :type Actor%20Object%20Reference) (OtherComp :type Primitive%20Component%20Object%20Reference) (OtherBodyIndex :type Integer))
  ;[1 1 1] Merge Character or Object
  (Utilities|Casting|CastToBP_Character_Top OtherActor)
  (Variables|Default|SetTopWantToMerge false))

(event Custom|MySeparate
  (params (BlendTime :type Float%20%28single-precision%29) (Target :type Player%20Controller%20Object%20Reference) (InPawn :type Pawn%20Object%20Reference))
  ;[1 1 1] Switch
  (if (Class|Actor|WasRecentlyRendered InPawn 0.0)
    (Game|Player|SetViewTargetwithBlend Target InPawn BlendTime "VTBlend_EaseInOut" 2.0 false)
    (Utilities|FlowControl|Delay BlendTime)
    ;;[1 1 1] Se souvenir de la velocité de la partie juste avant de la possess (donc après le delay)
    (bind _outactors (Actor|GetAllActorsOfClass "/Game/Blueprints/Character/BP_Character_Top.BP_Character_Top_C" :!label _label))
    (bind _output_get (Variables|/Game/Blueprints/Character/BP_Character_Base.BP_Character_Base_C|SetOldVelocity (Utilities|Array|Get(acopy) _outactors) (Transformation|GetVelocity (Utilities|Array|Get(acopy) _outactors))))
    (Pawn|Possess Target InPawn)
    (Variables|/Script/Engine.MovementComponent|SetVelocity (Variables|/Script/Engine.Character|GetCharacterMovement (Utilities|Array|Get(acopy) _outactors)) _output_get)
    (else
      (Utilities|FlowControl|Sequence
        (:then_0
          (Utilities|FlowControl|Delay (/ BlendTime 2.0))
          (goto _label))
        (:then_1
          (Components|Timeline|SetPlayRate (Variables|Default|GetFading) (/ 1.0 BlendTime))
          (bind _alpha (Timeline|Fading PlayFromStart)
            (:Update
              (Class|PlayerCameraManager|SetManualCameraFade (Game|GetPlayerCameraManager 0) _alpha "(R=0.000000,G=0.000000,B=0.000000,A=1.000000)" false))))))))

(event Custom|SetPartner
  (params (TopRef :type BP%20Character%20Top%20Object%20Reference))
  ;[1 1 1] SetPartner
  (Variables|/Game/Blueprints/Character/Components/BPC_Death.BPC_Death_C|SetPartnerInDeath (Variables|Default|GetBPC_Death) TopRef))

(event Custom|Kick
  (Variables|Default|SetIsSpecialAnimPlaying true)
  (Sprite|SetFlipbook (Variables|Default|GetSprite) "/Game/Assets/2D/Characters/ZombieLowerHalf/Kick/PFB_Kick_WIP.PFB_Kick_WIP")
  (Components|Timeline|SetLooping (Variables|Default|GetSprite) false))

(event EventBeginPlay
  (|CallParentFunction)
  (Character|LaunchCharacter (Variables|Default|GetInitialVelocity) false false))

(event Collision|EventActorBeginOverlap
  (params (OtherActor :type Actor%20Object%20Reference)))

(event EventTick
  (params (DeltaSeconds :type Float%20%28single-precision%29))
  (|CallParentFunction DeltaSeconds)
  (if (Variables|Default|GetTopWantToMerge)
    (Utilities|IsValid (stale OnComponentBeginOverlap(MergeCollision) _asbp_character_top)
      (:Is%20Valid
        (if (<= (.Z (Math|Vector|BreakVector (Transformation|GetVelocity (stale OnComponentBeginOverlap(MergeCollision) _asbp_character_top)))) 0.0)
          (CallFunction|MergeCharacter (stale OnComponentBeginOverlap(MergeCollision) _asbp_character_top) false))))))

(event Input|KeyboardEvents|DebugKeyF
  (params (Key :type Key%20Structure :default "None") (ActionValue :type Input%20Action%20Value%20Structure))
  (:Pressed
    (CallFunction|Kick)))

(fn ConstructionScript
  (|CallParentFunction))

(fn Separate
  (|CallParentFunction)
  (bind _outactors (Actor|GetAllActorsOfClass "/Game/Blueprints/Character/BP_Character_Top.BP_Character_Top_C"))
  (bind _asbp_player_controller (Utilities|Casting|CastToBP_Player_Controller (Game|GetPlayerController 0)))
  (CallFunction|MySeparate (Variables|Default|GetcamTransitionSpeed) _asbp_player_controller (Utilities|Array|Get(acopy) _outactors)))

(fn MergeCharacter
  (params (UpperHalfRef :type BP%20Character%20Top%20Object%20Reference) (DoRespawn :type Boolean))
  (Variables|Default|SetDoRespawn DoRespawn)
  (bind _output_get (Variables|Default|SetIsFacingRight (Variables|/Game/Blueprints/Character/BP_Character_Base.BP_Character_Base_C|GetIsFacingRight UpperHalfRef)))
  (Collision|SetCollisionEnabled (Variables|/Script/Engine.Character|GetCapsuleComponent UpperHalfRef) "NoCollision")
  (Actor|DestroyActor UpperHalfRef)
  ;[1 1 1] pour que le full spawn au même endroit que les jambes les jambes doivent pas interférer (cassez vous wesh)
  (Collision|SetCollisionEnabled (Variables|Default|GetCapsuleComponent) "NoCollision")
  (bind _returnvalue (Game|SpawnActorfromClass "/Game/Blueprints/Character/BP_Character_Full.BP_Character_Full_C" (Math|Transform|MakeTransform (Math|Transform|TransformLocation (Transformation|GetActorTransform) "0.000000,0.000000,10.000000")) "Undefined" "MultiplyWithRoot" 0 _output_get false false "0.000000,0.000000,0.000000" "0.000000,0.000000,0.000000" (Variables|Default|GetCurrentCameraTrigger) 0))
  (Default|SetCamZRotation _returnvalue (.Yaw (Math|Rotator|BreakRotator (Class|SpringArmComponent|GetTargetRotation (Variables|Default|GetSpringArm)))))
  (bind _asbp_player_controller (Utilities|Casting|CastToBP_Player_Controller (Game|GetPlayerController 0)))
  (Pawn|Possess _asbp_player_controller _returnvalue)
  (if (Variables|Default|GetDoRespawn)
    (Default|Respawn _returnvalue))
  (Actor|DestroyActor))

(fn MergeObject
  (params (ObjectToMerge :type %20Object%20Reference)))

(fn Respawn
  (|CallParentFunction)
  (bind _asbp_character_top (Utilities|Casting|CastToBP_Character_Top (Variables|/Game/Blueprints/Character/Components/BPC_Death.BPC_Death_C|GetPartnerInDeath (Variables|Default|GetBPC_Death))))
  (CallFunction|MergeCharacter _asbp_character_top true))