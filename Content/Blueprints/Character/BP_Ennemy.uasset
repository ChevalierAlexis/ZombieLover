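; Enemy Blueprint, driven by AIC_Enemy_Controller, that is set to either patrol or guard.
; On BeginPlay it sets the controller's IsGuarding Blackboard key to the inverse of IsPatroling.
; It then prints French setup warnings when the first PatrolItinirary point contradicts that mode, treating a zero vector as unset.
; The Construction Script records the actor's location as GuardLocation.
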(event `self.ReceiveBeginPlay`
  (bind _asaic_enemy_controller (cast `/Game/Blueprints/AI/AIC_Enemy_Controller` (`self.GetController`)))
  (`BlackboardComponent.SetValueAsBool` (`AIController.Blackboard` _asaic_enemy_controller) (`self.IsGuarding`) (not (`self.IsPatroling`)))
  (if (`self.IsPatroling`)
    (if (== (`|GetArrayItem` (`self.PatrolItinirary`)) (0.0 0.0 0.0))
      (`KismetSystemLibrary.PrintString` "Pas d'itinéraire défini dans \"PatrolItinirary\""))
    (elif (!= (`|GetArrayItem` (`self.PatrolItinirary`)) (0.0 0.0 0.0))
      (`KismetSystemLibrary.PrintString` "Un itinéraire est défini mais le mode patrouille n'est pas activé. Pour ce faire, mettez \"IsPatroling\" sur True."))))

(fn `UserConstructionScript`
  (set `self.GuardLocation` (`self.K2_GetActorLocation`)))