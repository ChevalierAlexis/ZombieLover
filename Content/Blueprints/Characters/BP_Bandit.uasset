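; Bandit enemy with a Paper2D sprite, driven by AIC_Enemy_Controller, that either patrols or guards.
; On BeginPlay it sets the guarding flag in the blackboard, then either copies the nearest BP_Patrol's points into its itinerary or stores its position as GuardLocation.
; Tick flips the flipbook from RotateValue's sign and clears line of sight and player target while the player is invisible.
; An itinerary validation debug block is unconnected.
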(event `self.ReceiveBeginPlay`
  (bind _asaic_enemy_controller (cast `/Game/Blueprints/AI/AIC_Enemy_Controller` (`self.GetController`)))
  (set `self.bUseControllerRotationYaw` false)
  (bind _blackboard1 (`/Game/Blueprints/AI/AIC_Enemy_Controller.Blackboard1` _asaic_enemy_controller))
  (`BlackboardComponent.SetValueAsBool` _blackboard1 (`self.IsGuarding`) (not (`self.IsPatroling`)))
  (if (`self.IsPatroling`)
    ;[1 1 1] Charge l'itinéraire
    (`KismetArrayLibrary.Array_Clear` (`self.PatrolItinirary`))
    (bind _outactors (`GameplayStatics.GetAllActorsOfClass` "/Game/Blueprints/AI/BP_Patrol.BP_Patrol_C"))
    (bind _asbp_patrol (cast `/Game/Blueprints/AI/BP_Patrol` (`.ReturnValue` (`GameplayStatics.FindNearestActor` (`self.K2_GetActorLocation`) _outactors))))
    (bind _output_get (set `self.Patrol` _asbp_patrol))
    (for _array_element (`/Game/Blueprints/AI/BP_Patrol.PatrolPoints` _output_get)
      (`KismetArrayLibrary.Array_Add` (`self.PatrolItinirary`) (`self.K2_GetActorLocation` _array_element)))
    (else
      (`BlackboardComponent.SetValueAsVector` _blackboard1 "GuardLocation" (`self.K2_GetActorLocation`)))))

(event `self.ReceiveTick`
  (params (DeltaSeconds :type "Float (single-precision)"))
  ;[1 1 1] Gère la rotation du sprite
  (if (< (`self.RotateValue`) 0.0)
    (`SceneComponent.K2_SetRelativeRotation` (`self.PaperFlipbook`) (struct :`Yaw` 180.0) false false)
    (else
      (`SceneComponent.K2_SetRelativeRotation` :`self` (`self.PaperFlipbook`))))
  ;[1 1 1] Si le joueur est caché, vider la vision
  (if (`/Game/Blueprints/Characters/BP_Character_Base.IsInvisible` (`/Game/Blueprints/Library/BPFL_Fonction_Library.CastToPlayerCharacter`))
    (bind _asaic_enemy_controller (cast `/Game/Blueprints/AI/AIC_Enemy_Controller` (`self.GetController`)))
    (bind _blackboard1 (`/Game/Blueprints/AI/AIC_Enemy_Controller.Blackboard1` _asaic_enemy_controller))
    (`BlackboardComponent.SetValueAsBool` _blackboard1 "HasLineOfSight" false)
    (`BlackboardComponent.SetValueAsObject` _blackboard1 "Player" null)))

(fn `UserConstructionScript`
  (set `self.GuardLocation` (`self.K2_GetActorLocation`)))