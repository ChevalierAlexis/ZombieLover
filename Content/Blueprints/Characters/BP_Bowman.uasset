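; BP_Bowman is a PaperZD archer enemy that patrols or guards, driven by an AI controller's blackboard.
; BeginPlay seeds wait and guard keys, loading the farthest BP_Patrol's points when patrolling, despite a comment saying nearest.
; Tick flips the sprite by RotateValue and clears player sight while the player is invisible.
; FireBow launches BP_Projectile using X/Y offsets to the nearest BP_Character_Base, then clears the animation's attack flag.
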(event `self.ReceiveBeginPlay`
  (bind _asbp_aic_bowman_controller (cast `/Game/Blueprints/AI/BP_AIC_Bowman_Controller` (`self.GetController`)))
  (set `self.bUseControllerRotationYaw` false)
  (bind _blackboard1 (`/Game/Blueprints/AI/BP_AIC_Bowman_Controller.Blackboard1` _asbp_aic_bowman_controller))
  (`BlackboardComponent.SetValueAsFloat` _blackboard1 (`self.WaitTime`) (`self.WaitTimeValue`))
  (`BlackboardComponent.SetValueAsBool` _blackboard1 (`self.IsGuarding`) (not (`self.IsPatroling`)))
  ;[1 1 1] Trouve la patrouille la plus proche
  (if (`self.IsPatroling`)
    (bind _outactors (`GameplayStatics.GetAllActorsOfClass` "/Game/Blueprints/AI/BP_Patrol.BP_Patrol_C"))
    (for (_array_element _array_index) _outactors
      (bind _returnvalue (`self.GetDistanceTo` _array_element self))
      (if (> _returnvalue (`self.PatrolDistance`))
        (set `self.PatrolDistance` _returnvalue)
        (set `self.PatrolChoiceIndex` _array_index)))
    ;[1 1 1] Charge l'itinéraire
    (bind _output_get (set `self.Patrol` (`|GetArrayItem` _outactors (`self.PatrolChoiceIndex`))))
    (for _array_element_2 (`/Game/Blueprints/AI/BP_Patrol.PatrolPoints` _output_get)
      (`KismetArrayLibrary.Array_Add` (`self.PatrolItinirary`) (`self.K2_GetActorLocation` _array_element_2)))
    (else
      (`BlackboardComponent.SetValueAsVector` _blackboard1 "GuardLocation" (`self.K2_GetActorLocation`)))))

(event `self.ReceiveTick`
  (params (DeltaSeconds :type "Float (single-precision)"))
  ;[1 1 1] Gère la rotation du sprite
  (if (< (`self.RotateValue`) 0.0)
    (`SceneComponent.K2_SetRelativeRotation` (`self.PaperFlipbook`) (struct :`Yaw` 180.0) false false)
    (else
      (`SceneComponent.K2_SetRelativeRotation` :`self` (`self.PaperFlipbook`))))
  ;[1 1 1] Si le joueur est caché, vider la vision
  (if (`/Game/Blueprints/Characters/BP_Character_Base.IsInvisible` (`/Game/Blueprints/Library/BPFL_Fonction_Library.CastToPlayerCharacter`))
    (bind _asbp_aic_enemy_controller (cast `/Game/Blueprints/AI/BP_AIC_Enemy_Controller` (`self.GetController`)))
    (bind _blackboard1 (`/Game/Blueprints/AI/BP_AIC_Enemy_Controller.Blackboard1` _asbp_aic_enemy_controller))
    (`BlackboardComponent.SetValueAsBool` _blackboard1 "HasLineOfSight" false)
    (`BlackboardComponent.SetValueAsObject` _blackboard1 "Player" null)))

(event `FireBow`
  (bind _returnvalue (`SceneComponent.K2_GetComponentLocation` (`self.PaperFlipbook`)))
  (bind _outactors (`GameplayStatics.GetAllActorsOfClass` "/Game/Blueprints/Characters/BP_Character_Base.BP_Character_Base_C"))
  (bind (_distance _returnvalue_2) (`GameplayStatics.FindNearestActor` _returnvalue _outactors))
  (set `self.Target` _returnvalue_2)
  (`KismetSystemLibrary.PrintString` "Boulet")
  (bind (_returnvalue_x _returnvalue_y) (`KismetMathLibrary.BreakVector` (- (`self.K2_GetActorLocation` _returnvalue_2) (`self.K2_GetActorLocation`))))
  (`|SpawnActorFromClass` "/Game/Blueprints/Objects/BP_Projectile.BP_Projectile_C" (`KismetMathLibrary.MakeTransform` (+ _returnvalue (0.0 0.0 100.0))) "Undefined" "MultiplyWithRoot" null 0.0 (0.0 0.0 0.0) 500.0 _returnvalue_x _returnvalue_y self)
  (bind _asabp_pzd_bowman (cast `/Game/Animation/Bowman/ABP_PZD_Bowman` (`PaperZDAnimationComponent.AnimInstance` (`self.PaperZDAnimation`))))
  (set `/Game/Animation/Bowman/ABP_PZD_Bowman.IsAttacking` false _asabp_pzd_bowman))

(fn `UserConstructionScript`
  (set `self.GuardLocation` (`self.K2_GetActorLocation`)))