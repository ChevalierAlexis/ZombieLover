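; BPC_Death is an actor component that handles its owner's death and a linked partner's death.
; On BeginPlay it assigns the nearest BP_Checkpoint to the camera manager if none is set.
; GetKilled flags both the owner and PartnerInDeath as dead through their BPC_Death components, then shows the death UI through the camera manager.
; Die only sets IsDead, and UnPopUiDeath hides the UI.
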(event `self.ReceiveBeginPlay`
  (set `self.Owner` (`self.GetOwner`))
  (bind _asbp_camera_manager (`/Game/Blueprints/Library/BPFL_Fonction_Library.GetCameraManager`))
  (bind _output_get (set `self.CameraManagerRef` _asbp_camera_manager))
  (`/Engine/EditorBlueprintResources/StandardMacros.IsValid` (`/Game/Blueprints/BP_Camera_Manager.CheckPoint` _output_get)
    (:`Is Not Valid`
      (bind _returnvalue (`/Game/Blueprints/Library/BPFL_Fonction_Library.FindNearestActorOfClass` "/Game/Blueprints/Objects/BP_Checkpoint.BP_Checkpoint_C" (`SceneComponent.K2_GetComponentLocation` (`Actor.RootComponent` (`self.Owner`)))))
      (bind _asbp_checkpoint (cast `/Game/Blueprints/Objects/BP_Checkpoint` _returnvalue))
      (set `/Game/Blueprints/BP_Camera_Manager.CheckPoint` _asbp_checkpoint (`self.CameraManagerRef`)))))

(event `GetKilled`
  (bind _partnerindeath (`self.PartnerInDeath`))
  (bind _returnvalue (`Actor.GetComponentByClass` _partnerindeath "BPC_Death_C"))
  (`|ExecutionSequence`
    (:`then_0`
      (`KismetSystemLibrary.PrintString` "GetKilled")
      (`/Engine/EditorBlueprintResources/StandardMacros.IsValid` _partnerindeath
        (:`Is Valid`
          (`/Engine/EditorBlueprintResources/StandardMacros.IsValid` _returnvalue
            (:`Is Valid`
              (`self.Die` _returnvalue)
              ;[1 1 1] Si on ne controlle pas ce pawn, affiche l'écran de mort pour la partie controllée
              (if (== (`Controller.K2_GetPawn` (`GameplayStatics.GetPlayerController` 0)) (`self.GetOwner`))
                (`KismetSystemLibrary.PrintString` "Same")
                (else
                  (`KismetSystemLibrary.PrintString` "Different")
                  (`/Game/Blueprints/BP_Camera_Manager.PopDeathUi` (`self.CameraManagerRef`) true))))))))
    (:`then_1`
      (`self.Die`)
      (`/Game/Blueprints/BP_Camera_Manager.PopDeathUi` (`self.CameraManagerRef`) true))))

(event `Die`
  (if (not (`self.IsDead`))
    (set `self.IsDead` true)))

(event `UnPopUiDeath`
  (`/Game/Blueprints/BP_Camera_Manager.PopDeathUi` (`self.CameraManagerRef`) false))