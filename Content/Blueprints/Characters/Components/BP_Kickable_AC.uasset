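; Kickable actor component that knocks its owner along a launch direction when kicked and handles kick recoil for characters.
; GetKicked launches Character owners or impulses a static mesh on other actors, with up-kicks giving a mostly vertical pop whose horizontal push reverses for BP_Character_Top.
; DrawBack launches BP_Character_Base owners with force shaped by kick type and grounded state, flipping their facing when airborne.
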(event `self.ReceiveBeginPlay`)

(event `GetKicked`
  (params (LaunchDirection :type "Vector Structure") (UpKick :type Boolean))
  (bind _returnvalue (`self.GetOwner`))
  (bind _returnvalue_2 (not UpKick))
  (bind _ejectionforce (`self.EjectionForce`))
  (bind _returnvalue_3 (* (`KismetMathLibrary.MakeVector` LaunchDirection_X LaunchDirection_Y (/ (`self.ZLaunch`) _ejectionforce)) _ejectionforce))
  (bind _returnvalue_4 (`KismetMathLibrary.SelectVector` _returnvalue_3 (`KismetMathLibrary.MakeVector` (* LaunchDirection_X 40.0) (* LaunchDirection_Y 40.0) 250.0) _returnvalue_2))
  (bind _ascharacter (cast `Character` _returnvalue)
    (:`then`
      (bind _asbp_character_top (cast `/Game/Blueprints/Characters/BP_Character_Top` _returnvalue)
        (:`then`
          (`Character.LaunchCharacter` _asbp_character_top (`KismetMathLibrary.SelectVector` _returnvalue_3 (`KismetMathLibrary.MakeVector` (* LaunchDirection_X -50.0) (* LaunchDirection_Y -50.0) 250.0) _returnvalue_2) false false))
        (:`CastFailed`
          (`Character.LaunchCharacter` _ascharacter _returnvalue_4 false false))))
    (:`CastFailed`
      (`PrimitiveComponent.AddImpulse` (`Actor.GetComponentByClass` _returnvalue "/Script/Engine.StaticMeshComponent") (* _returnvalue_4 400.0) "None" false))))

(event `DrawBack`
  (params (LaunchDirection :type "Vector Structure") (UpKick :type Boolean) (Grounded :type Boolean))
  (bind _returnvalue (`self.GetOwner`))
  (bind _returnvalue_2 (* (`KismetMathLibrary.MakeVector` LaunchDirection_X LaunchDirection_Y (* LaunchDirection_Z (`KismetMathLibrary.SelectFloat` 1.0 0.2 UpKick))) (`self.DrawBackForce`)))
  (if UpKick
    (set `self.DrawBackForce` 300.0)
    (else
      (set `self.DrawBackForce` 400.0)))
  (bind _asbp_character_base (cast `/Game/Blueprints/Characters/BP_Character_Base` _returnvalue))
  (`Character.LaunchCharacter` _asbp_character_base (`KismetMathLibrary.SelectVector` _returnvalue_2 (/ _returnvalue_2 (`KismetMathLibrary.SelectFloat` 4.0 1.6 UpKick)) (not Grounded)) false (< (.z (`Actor.GetVelocity` _returnvalue)) 1.0))
  (if (not (`/Game/Blueprints/Characters/BP_Character_Base.Grounded` _asbp_character_base))
    (set `/Game/Blueprints/Characters/BP_Character_Base.IsFacingRight` (not (`/Game/Blueprints/Characters/BP_Character_Base.IsFacingRight` _asbp_character_base)) _asbp_character_base)
    (`/Game/Blueprints/Characters/BP_Character_Base.HandleRotation` _asbp_character_base)))