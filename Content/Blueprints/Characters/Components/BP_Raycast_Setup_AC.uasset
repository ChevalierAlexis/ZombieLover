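; Actor component that detects the physical surface its owner walks on and stores it in SurfaceWalkedOn.
; An OnTick dispatcher appears to run Initialization until vertical velocity is zero, then switch to CheckSurface.
; Initialization adds tagged Start and End static mesh markers, setting End's height just below a trace hit toward a fixed low world point.
; CheckSurface traces between the markers with complex collision and one-frame debug drawing.
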(event `self.ReceiveBeginPlay`
  (add `self.OnTick` (`|CreateDelegate` :!event `Initialization`)))

(event `self.ReceiveTick`
  (params (DeltaSeconds :type "Float (single-precision)"))
  (`self.OnTick`))

(event `CheckSurface`
  (bind _returnvalue (`self.GetOwner`))
  (bind _outhit (`KismetSystemLibrary.LineTraceSingle` :`Start` (`SceneComponent.K2_GetComponentLocation` (`|GetArrayItem` (`Actor.GetComponentsByTag` _returnvalue "/Script/Engine.StaticMeshComponent" "Start"))) :`End` (`SceneComponent.K2_GetComponentLocation` (`|GetArrayItem` (`Actor.GetComponentsByTag` _returnvalue "/Script/Engine.StaticMeshComponent" "End"))) :`TraceChannel` "TraceTypeQuery1" :`bTraceComplex` true :`DrawDebugType` "ForOneFrame"))
  (set `self.SurfaceWalkedOn` (`GameplayStatics.GetSurfaceType` _outhit)))

(event `Initialization`
  (bind (_returnvalue_x _returnvalue_y _returnvalue_z) (`KismetMathLibrary.BreakVector` (`Actor.GetVelocity` (`self.GetOwner`))))
  (if (== _returnvalue_z 0.0)
    ;[1 1 1] Ajoute l'origine du raycast
    (bind _returnvalue (`|AddComponentByClass` (`self.GetOwner`) "/Script/Engine.StaticMeshComponent" false (`KismetMathLibrary.MakeTransform` (0.0 0.0 0.0))))
    (`KismetArrayLibrary.Array_Add` (`ActorComponent.ComponentTags` _returnvalue) "Start")
    (`StaticMeshComponent.SetStaticMesh` _returnvalue null)
    ;[1 1 1] raycast pour identifier le bas du personnage et poser la fin du raycast
    (bind _outhit (`KismetSystemLibrary.LineTraceSingle` (`SceneComponent.K2_GetComponentLocation` _returnvalue) (0.0 0.0 -5000.0) "TraceTypeQuery1"))
    (bind (_returnvalue_x_2 _returnvalue_y_2 _returnvalue_z_2) (`KismetMathLibrary.BreakVector` (`SceneComponent.K2_GetComponentLocation` _returnvalue)))
    (bind _returnvalue_2 (`|AddComponentByClass` (`self.GetOwner`) "/Script/Engine.StaticMeshComponent" false (`KismetMathLibrary.MakeTransform` (`KismetMathLibrary.MakeVector` 0.0 0.0 (- (- (.z (`.Location` (`GameplayStatics.BreakHitResult` _outhit))) _returnvalue_z_2) 1.0)))))
    (`KismetArrayLibrary.Array_Add` (`ActorComponent.ComponentTags` _returnvalue_2) "End")
    (`StaticMeshComponent.SetStaticMesh` _returnvalue_2 null)
    (set `self.IsInitialized` true)
    (add `self.OnTick` (`|CreateDelegate` :!event `CheckSurface`))
    (remove `self.OnTick` (`|CreateDelegate` :!event `Initialization`))))