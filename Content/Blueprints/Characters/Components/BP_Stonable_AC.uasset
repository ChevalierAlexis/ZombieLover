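; Stonable actor component for BP_Chicken that, on activation, knocks the chicken and makes it drop what it carries.
; OnActivation sends an upward launch through the chicken's kickable component, then detaches the held key at its world position and starts it falling under physics with zeroed velocity.
; Without a key, it detaches and simulates any other attached object.
; An unconnected delayed check for stopping key physics never runs.
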(event `self.ReceiveTick`
  (params (DeltaSeconds :type "Float (single-precision)")))

(fn `OnActivation`
  (set `self.Activated` true)
  (bind _asbp_chicken (cast `/Game/Blueprints/Objects/BP_Chicken` (`self.GetOwner`)))
  (`/Game/Blueprints/Characters/Components/BP_Kickable_AC.GetKicked` (`/Game/Blueprints/Objects/BP_Chicken.BP_Kickable_AC` _asbp_chicken) (0.0 0.0 10.0) false)
  (bind _keytoattach (`/Game/Blueprints/Objects/BP_Chicken.KeyToAttach` _asbp_chicken))
  (`/Engine/EditorBlueprintResources/StandardMacros.IsValid` _keytoattach
    (:`Is Valid`
      (bind _key (`/Game/Blueprints/Objects/InputObjects/BP_Key.Key` _keytoattach))
      (set `self.Location` (`SceneComponent.K2_GetComponentLocation` _key))
      (`Actor.K2_DetachFromActor` _keytoattach "KeepRelative" "KeepRelative" "KeepRelative")
      (`SceneComponent.K2_SetWorldLocation` _key (`self.Location`) true false)
      (bind _capsule (`/Game/Blueprints/Objects/InputObjects/BP_Key.Capsule` _keytoattach))
      (`PrimitiveComponent.SetSimulatePhysics` _capsule true)
      (set `/Game/Blueprints/Objects/InputObjects/BP_Key.IsFalling` true _keytoattach)
      (`PrimitiveComponent.SetPhysicsLinearVelocity` _capsule (0.0 0.0 0.0) false "None")
      (set `/Game/Blueprints/Objects/BP_Chicken.KeyToAttach` null _asbp_chicken))
    (:`Is Not Valid`
      (`/Engine/EditorBlueprintResources/StandardMacros.IsValid` (`/Game/Blueprints/Objects/BP_Chicken.ObjectToAttach` _asbp_chicken)
        (:`Is Valid`
          (bind _toattach (`/Game/Blueprints/Objects/BP_Chicken.ToAttach` _asbp_chicken))
          (`SceneComponent.K2_DetachFromComponent` _toattach "KeepRelative" "KeepRelative" "KeepRelative" true)
          (`PrimitiveComponent.SetSimulatePhysics` _toattach true))))))