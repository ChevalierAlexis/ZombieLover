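; Actor component on BP_Character_Top that lets the player grapple onto grab points while airborne.
; Jump or interaction input attaches to the nearest targeted point, or releases the current one, with a small launch steered by right-axis input.
; While hooked, Tick pins the cable to the hook, applies CalculateForceToAdd_2's force and sets air control.
; A line trace detects ground, which releases the grapple.
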(event `self.ReceiveBeginPlay`
  ;[1 1 1] Définit le joueur
  (bind _asbp_character_top (cast `/Game/Blueprints/Characters/BP_Character_Top` (`self.GetOwner`)))
  (bind _output_get (set `self.OwningActor` _asbp_character_top))
  (`/Game/Blueprints/Characters/BP_Character_Top.Clean Bind Event To Timeline` _output_get (`|CreateDelegate` :!event `BindedToTimelineZipRetract`)))

(event `self.ReceiveTick`
  (params (DeltaSeconds :type "Float (single-precision)"))
  (bind _grabpointhooked (`self.GrabPointHooked`))
  (bind _owningactor (`self.OwningActor`))
  (bind _owningactor_2 (`self.OwningActor`))
  (bind _grabpointhooked_2 (`self.GrabPointHooked`))
  (bind _returnvalue (`Actor.K2_GetActorLocation` _owningactor))
  (bind _charactermovement (`Character.CharacterMovement` _owningactor_2))
  (bind _returnvalue_2 (`SceneComponent.K2_GetComponentLocation` (`/Game/Blueprints/Objects/InputObjects/Bp_New_Grab_Point.HookPoint` _grabpointhooked)))
  (bind _returnvalue_3 (- _returnvalue _returnvalue_2))
  (`|ExecutionSequence`
    (:`then_0`
      (`/Engine/EditorBlueprintResources/StandardMacros.IsValid` _grabpointhooked_2
        (:`Is Valid`
          (`SceneComponent.K2_SetWorldLocation` (`/Game/Blueprints/Characters/BP_Character_Top.GrappleCable` (`self.OwningActor`)) (`SceneComponent.K2_GetComponentLocation` (`/Game/Blueprints/Objects/InputObjects/Bp_New_Grab_Point.HookPoint` _grabpointhooked_2)) false false)
          (set `CableComponent.EndLocation` (0.0 -3.0 0.0) (`/Game/Blueprints/Characters/BP_Character_Top.GrappleCable` _owningactor_2))
          (`CharacterMovementComponent.AddForce` _charactermovement (+ (* (* (`KismetMathLibrary.Normal` _returnvalue_3) (`KismetMathLibrary.Dot_VectorVector` (* (`Actor.GetVelocity` _owningactor) 100.0) _returnvalue_3)) -2.0) (* (`KismetMathLibrary.GetDirectionUnitVector` _returnvalue _returnvalue_2) (* (`KismetMathLibrary.FClamp` (/ (`Actor.GetDistanceTo` _owningactor _grabpointhooked) 100.0) 1.0 10000000.0) 60000.0))))
          (set `CharacterMovementComponent.AirControl` 2.0 _charactermovement))))
    (:`then_1`
      (if (`self.IsOnGround`)
        (`self.AttachDetachGrap` null)))))

(event `SetGrabPoint`
  (params (GrabPoint :type "/Game/Blueprints/Objects/InputObjects/BP_Grab_Point Object Reference"))
  (set `self.GrabPoint` GrabPoint))

(event `AttachDetachGrap`
  (params (GrabPointHooked :type "/Game/Blueprints/Objects/InputObjects/Bp_New_Grab_Point Object Reference"))
  (bind _returnvalue (`KismetSystemLibrary.IsValid` GrabPointHooked))
  (bind _owningactor (`self.OwningActor`))
  (`SceneComponent.SetVisibility` (`/Game/Blueprints/Characters/BP_Character_Top.GrappleCable` _owningactor) _returnvalue false)
  (set `self.GrabPointHooked` GrabPointHooked)
  (if _returnvalue
    (`/Game/Blueprints/Characters/BP_Character_Top.BloodTrailMove` _owningactor)))

(event `EnhancedInput|/Game/Inputs/InputActions/IA_Move_Right`
  (params (ActionValue :type "Float (double-precision)") (ElapsedSeconds :type "Float (double-precision)") (TriggeredSeconds :type "Float (double-precision)") (InputAction :type "InputAction Object Reference" :default "/Game/Inputs/InputActions/IA_Move_Right.IA_Move_Right"))
  (:`Triggered`
    (set `self.moveright` ActionValue :!label _label))
  (:`Completed`
    (goto _label)))

(event `EnhancedInput|/Game/Inputs/InputActions/IA_Jump`
  (params (ActionValue :type Boolean) (ElapsedSeconds :type "Float (double-precision)") (TriggeredSeconds :type "Float (double-precision)") (InputAction :type "InputAction Object Reference" :default "/Game/Inputs/InputActions/IA_Jump.IA_Jump"))
  (bind _grabpointhooked (`self.GrabPointHooked`))
  (:`Triggered`
    (if (not (`self.IsOnGround`)) :!label _label_2
      (bind _asbp_new_grab_point (`/Game/Blueprints/Characters/BP_Character_Top.Find Nearest Grab Point` (`self.OwningActor`)))
      (`/Engine/EditorBlueprintResources/StandardMacros.IsValid` _asbp_new_grab_point
        (:`Is Valid`
          (if (== _grabpointhooked _asbp_new_grab_point)
            (`self.AttachDetachGrap` null :!label _label_3)
            (`Character.LaunchCharacter` (`self.OwningActor`) (`KismetMathLibrary.MakeVector` (* (`self.moveright`) 50.0) 0.0 100.0) false false :!label _label_4)
            (elif (`/Game/Blueprints/Objects/InputObjects/Bp_New_Grab_Point.Targeted` _asbp_new_grab_point)
              (`self.AttachDetachGrap` _asbp_new_grab_point)
              (goto _label_4))))
        (:`Is Not Valid`
          (`/Engine/EditorBlueprintResources/StandardMacros.IsValid` _grabpointhooked
            (:`Is Valid`
              (goto _label_3))))))))

(event `EnhancedInput|/Game/Inputs/InputActions/IA_Interaction`
  (params (ActionValue :type Boolean) (ElapsedSeconds :type "Float (double-precision)") (TriggeredSeconds :type "Float (double-precision)") (InputAction :type "InputAction Object Reference" :default "/Game/Inputs/InputActions/IA_Interaction.IA_Interaction"))
  (:`Started`
    (goto _label_2)))

(event `EnhancedInput|/Game/Inputs/InputActions/IA_Jump_Stop`
  (params (ActionValue :type Boolean) (ElapsedSeconds :type "Float (double-precision)") (TriggeredSeconds :type "Float (double-precision)") (InputAction :type "InputAction Object Reference" :default "/Game/Inputs/InputActions/IA_Jump_Stop.IA_Jump_Stop"))
  ;[1 1 1] Comment
)

(fn `BindedToTimelineZipRetract`
  (params (Alpha :type "Float (double-precision)"))
  (set `CableComponent.CableLength` (`KismetMathLibrary.Lerp` (`self.CableTempLength`) 0.0 Alpha) (`/Game/Blueprints/Characters/BP_Character_Top.GrappleCable` (`self.OwningActor`))))

(fn `IsOnGround`
  (returns (ReturnValue :type Boolean))
  (bind _owningactor (`self.OwningActor`))
  (bind (_outhit _returnvalue) (`KismetSystemLibrary.LineTraceSingle` (`SceneComponent.K2_GetComponentLocation` (`/Game/Blueprints/Characters/BP_Character_Base.RaySource` _owningactor)) (`SceneComponent.K2_GetComponentLocation` (`/Game/Blueprints/Characters/BP_Character_Base.RaySourceEnd` _owningactor)) "TraceTypeQuery1"))
  (return _returnvalue))