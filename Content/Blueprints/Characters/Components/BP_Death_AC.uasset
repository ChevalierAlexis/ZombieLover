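; Actor component that handles its owner's death, plus death of an optional linked PartnerInDeath.
; GetKilled kills both; character owners play a death animation, then after a delay, if the current player is dead, show death UI and respawn checkpoint objects.
; Other owners are hidden, lose collision and AI behavior, and optionally respawn instantly as copies at their starting transform.
; BeginPlay defaults the camera manager's checkpoint to the nearest one.
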(event `self.ReceiveBeginPlay`
  (bind _output_get (set `self.Owner` (`self.GetOwner`)))
  (set `self.SpawnPoint` (`Actor.GetTransform` _output_get))
  (bind _output_get_2 (set `self.CameraManagerRef` (`/Game/Blueprints/Library/BPFL_Fonction_Library.GetCameraManager`)))
  (`/Engine/EditorBlueprintResources/StandardMacros.IsValid` (`/Game/Blueprints/CameraManager/BP_Camera_Manager.CheckPoint` _output_get_2)
    (:`Is Not Valid`
      (bind _returnvalue (`/Game/Blueprints/Library/BPFL_Fonction_Library.FindNearestActorOfClass` "/Game/Blueprints/Objects/LevelDesignZones/BP_Checkpoint.BP_Checkpoint_C" (`SceneComponent.K2_GetComponentLocation` (`Actor.RootComponent` (`self.Owner`)))))
      (bind _asbp_checkpoint (cast `/Game/Blueprints/Objects/LevelDesignZones/BP_Checkpoint` _returnvalue))
      (set `/Game/Blueprints/CameraManager/BP_Camera_Manager.CheckPoint` _asbp_checkpoint (`self.CameraManagerRef`)))))

(event `GetKilled`
  (bind _returnvalue (`Actor.GetComponentByClass` (`self.PartnerInDeath`) "BP_Death_AC_C"))
  (if (not (`self.IsDead`))
    (`|ExecutionSequence`
      (:`then_0`
        (`/Engine/EditorBlueprintResources/StandardMacros.IsValid` (`self.PartnerInDeath`)
          (:`Is Valid`
            (`/Engine/EditorBlueprintResources/StandardMacros.IsValid` _returnvalue
              (:`Is Valid`
                (`self.Die` _returnvalue))))))
      (:`then_1`
        (`self.Die`)
        (bind _asbp_character_base (cast `/Game/Blueprints/Characters/BP_Character_Base` (`self.Owner`)))
        (`/Game/Blueprints/Characters/BP_Character_Base.SpawnDeathAnim` _asbp_character_base)
        (`KismetSystemLibrary.Delay` 2.0)
        (if (not (`/Game/Blueprints/Library/BPFL_Fonction_Library.Is Current Player Alive`))
          (`/Game/Blueprints/CameraManager/BP_Camera_Manager.PopDeathUi` (`self.CameraManagerRef`) true)
          (`/Game/Blueprints/Objects/LevelDesignZones/BP_Checkpoint.RespawnObjects` (`.CheckPoint` (`/Game/Blueprints/Library/BPFL_Fonction_Library.GetCameraManager`))))))))

(event `Die`
  (bind _owner (`self.Owner`))
  (bind _returnvalue (`AIBlueprintHelperLibrary.GetAIController` (`self.Owner`)))
  (set `self.IsDead` true)
  (cast `/Game/Blueprints/Characters/BP_Character_Base` _owner
    (:`CastFailed`
      (if (not (not (`self.DoInstantRespawn`)))
        (`|SpawnActorFromClass` (`GameplayStatics.GetObjectClass` _owner) (`KismetMathLibrary.MakeTransform` (+ (.location (`self.SpawnPoint`)) (0.0 0.0 10.0)) (.rotation (`self.SpawnPoint`)) (.scale (`self.SpawnPoint`))) "AdjustIfPossibleButAlwaysSpawn" "MultiplyWithRoot" null null))
      (`Actor.SetActorHiddenInGame` (`self.Owner`) true)
      (`Actor.SetActorEnableCollision` (`self.Owner`) false)
      (`/Engine/EditorBlueprintResources/StandardMacros.IsValid` _returnvalue
        (:`Is Valid`
          (`self.Deactivate` (`Actor.GetComponentByClass` _returnvalue "/Script/AIModule.BehaviorTreeComponent"))
          (set `MovementComponent.Velocity` (0.0 0.0 0.0) (`Actor.GetComponentByClass` (`self.Owner`) "/Script/Engine.CharacterMovementComponent")))))))

(event `UnPopUiDeath`
  (`/Game/Blueprints/CameraManager/BP_Camera_Manager.PopDeathUi` (`self.CameraManagerRef`) false))