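; BP_Character_Full is the merged form of the player character, which can separate into top and bottom halves.
; On BeginPlay it plays a fusion squash, with a timeline lerping the sprite scale between its base and a squeezed factor.
; Separate disables capsule collision, spawns both halves at vertical offsets with facing state passed on, has the player controller possess the top, then destroys itself.
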(event `self.ReceiveBeginPlay`
  (`parent.ReceiveBeginPlay`)
  (set `self.SpriteBaseScale` (`SceneComponent.RelativeScale3D` (`self.Sprite`)))
  (`self.FusionSqueeze`) ; le corps de squash lors de la création (après avoir fusionné)
)

(event `FusionSqueeze`
  (`TimelineComponent.SetPlayRate` (`self.FusionSqueezeAnim`) (`self.FusionSqueezeRate`))
  (bind (_direction _alpha) (`Timeline|FusionSqueezeAnim` :!via `PlayFromStart`)
    (:`Update`
      (`SceneComponent.SetRelativeScale3D` (`self.Sprite`) (`KismetMathLibrary.VLerp` (`self.SpriteBaseScale`) (* (`self.SpriteBaseScale`) (`self.FusionSqueezeFactor`)) _alpha)))))

(fn `Separate`
  (bind _returnvalue (`self.GetTransform`))
  (bind _ismovingfront (`self.IsMovingFront`))
  (bind _isfacingright (`self.IsFacingRight`))
  (bind _isfacingfront (`self.IsFacingFront`))
  (`parent.Separate`)
  (`PrimitiveComponent.SetCollisionEnabled` (`self.CapsuleComponent`) "NoCollision")
  (`|SpawnActorFromClass` "/Game/Blueprints/Characters/BP_Character_Bottom.BP_Character_Bottom_C" (`KismetMathLibrary.MakeTransform` (`KismetMathLibrary.TransformLocation` _returnvalue (0.0 0.0 -10.0))) "Undefined" "MultiplyWithRoot" null _isfacingright _isfacingfront _ismovingfront null)
  (bind _returnvalue_2 (`|SpawnActorFromClass` "/Game/Blueprints/Characters/BP_Character_Top.BP_Character_Top_C" (`KismetMathLibrary.MakeTransform` (`KismetMathLibrary.TransformLocation` _returnvalue (0.0 0.0 18.0))) "Undefined" "MultiplyWithRoot" null _isfacingright _isfacingfront _ismovingfront null))
  (bind _asbp_player_controller (cast `/Game/Blueprints/BP_Player_Controller` (`GameplayStatics.GetPlayerController` 0)))
  (`Controller.Possess` _asbp_player_controller _returnvalue_2)
  (`self.K2_DestroyActor`))

(fn `UserConstructionScript`
  (`parent.UserConstructionScript`))