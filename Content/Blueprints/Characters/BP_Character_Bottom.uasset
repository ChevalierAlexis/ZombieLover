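; Lower-half zombie Paper2D character that can kick, hand control to the top half, and re-fuse with it.
; A falling top half overlapping MergeCollision triggers MergeCharacter, replacing both halves with a possessed BP_Character_Full.
; Interact charges a kick; release sphere-traces for BPC_Kickable targets, using hold time to choose an up-kick and recoiling on hits.
; Separate blends the camera or fades by distance before possessing the top; Respawn rebuilds the full body at the checkpoint.
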(event `self.ReceiveBeginPlay`
  (`parent.ReceiveBeginPlay`)
  (`self.LaunchCharacter` (`self.InitialVelocity`))
  (`KismetSystemLibrary.Delay` 0.05)
  (`NiagaraFunctionLibrary.SpawnSystemAtLocation` (`self.BloodBurstParticle`) (`SceneComponent.GetSocketLocation` (`self.Sprite`) "BloodSource")))

(event `self.ReceiveTick`
  (params (DeltaSeconds :type "Float (single-precision)"))
  (bind _returnvalue (`SceneComponent.K2_GetComponentLocation` (`self.CapsuleComponent`)))
  (`parent.ReceiveTick` DeltaSeconds)
  (if (`self.TopWantToMerge`)
    (`/Engine/EditorBlueprintResources/StandardMacros.IsValid` (stale `self.MergeCollision.OnComponentBeginOverlap` _asbp_character_top)
      (:`Is Valid`
        (if (<= (.z (`self.GetVelocity` (stale `self.MergeCollision.OnComponentBeginOverlap` _asbp_character_top))) -0.1)
          (bind (_outhit _returnvalue_2) (`KismetSystemLibrary.SphereTraceSingle` _returnvalue (+ _returnvalue (`KismetMathLibrary.MakeVector` 0.0 0.0 30.0)) 5.5 "TraceTypeQuery1" false (`|MakeArray` (stale `self.MergeCollision.OnComponentBeginOverlap` _asbp_character_top) :!type "Actor Object Reference") "None" true (struct :`R` 1.0 :`A` 1.0) (struct :`G` 1.0 :`A` 1.0) 1.0))
          (if (and (not _returnvalue_2) (== (`/Game/Blueprints/Library/BPFL_Fonction_Library.CastToPlayerCharacter`) (stale `self.MergeCollision.OnComponentBeginOverlap` _asbp_character_top)))
            (`/Game/Blueprints/Characters/BP_Character_Top.FastCamBlend` (stale `self.MergeCollision.OnComponentBeginOverlap` _asbp_character_top))
            (`KismetSystemLibrary.Delay` 0.05))
          (`self.MergeCharacter` (stale `self.MergeCollision.OnComponentBeginOverlap` _asbp_character_top)))))))

(event `self.MergeCollision.OnComponentBeginOverlap`
  (params (OverlappedComponent :type "PrimitiveComponent Object Reference") (OtherActor :type "Actor Object Reference") (OtherComp :type "PrimitiveComponent Object Reference") (OtherBodyIndex :type Integer) (bFromSweep :type Boolean) (SweepResult :type "HitResult Structure (by ref)"))
  ;[1 1 1] Merge Character or Object
  (bind _asbp_character_top (cast `/Game/Blueprints/Characters/BP_Character_Top` OtherActor))
  (set `self.TopWantToMerge` true))

(event `self.MergeCollision.OnComponentEndOverlap`
  (params (OverlappedComponent :type "PrimitiveComponent Object Reference") (OtherActor :type "Actor Object Reference") (OtherComp :type "PrimitiveComponent Object Reference") (OtherBodyIndex :type Integer))
  ;[1 1 1] Merge Character or Object
  (cast `/Game/Blueprints/Characters/BP_Character_Top` OtherActor)
  (set `self.TopWantToMerge` false))

(event `SetPartner`
  (params (TopRef :type "/Game/Blueprints/Characters/BP_Character_Top Object Reference"))
  ;[1 1 1] SetPartner
  (set `/Game/Blueprints/Characters/Components/BP_Death_AC.PartnerInDeath` TopRef (`self.BP_Death_AC`)))

(event `AddDuration`
  ;[1 1 1] kick
  (if (stale `ChargeKick` _output_get) :!label _label
    (set `self.HoldDuration` (+ (`self.HoldDuration`) 0.05))
    (`KismetSystemLibrary.Delay` 0.05)
    (`self.AddDuration`)))

(event `ChargeKick`
  ;[1 1 1] kick
  (set `self.HoldDuration` 0.0)
  (set `CharacterMovementComponent.MaxWalkSpeed` (* (`self.CharacterSpeed`) 0.3) (`self.CharacterMovement`))
  (set `self.IsSpecialAnimPlaying` true)
  (`PaperZDAnimInstance.JumpToNode` (`PaperZDAnimationComponent.AnimInstance` (`self.PaperZDAnimation`)) "Kick" "Locomotion")
  (`PaperFlipbookComponent.SetFlipbook` (`self.Sprite`) (`self.HoldKickAnim`))
  (`PaperFlipbookComponent.SetLooping` (`self.Sprite`) false)
  (bind _output_get (set `self.IsCharging` true))
  (goto _label))

(event `MySeparate`
  (params (BlendTime :type "Float (single-precision)") (Target :type "PlayerController Object Reference") (InPawn :type "Pawn Object Reference"))
  ;[1 1 1] Switch
  (if (< (`self.GetDistanceTo` InPawn self) 500.0)
    (`PlayerController.SetViewTargetWithBlend` Target InPawn BlendTime "VTBlend_EaseInOut" 2.0 false)
    (`KismetSystemLibrary.Delay` BlendTime)
    ;;[1 1 1] Se souvenir de la velocité de la partie juste avant de la possess (donc après le delay)
    (bind _outactors (`GameplayStatics.GetAllActorsOfClass` "/Game/Blueprints/Characters/BP_Character_Top.BP_Character_Top_C" :!label _label_2))
    (bind _output (`|GetArrayItem` _outactors))
    (bind _output_get (set `/Game/Blueprints/Characters/BP_Character_Base.OldVelocity` (`self.GetVelocity` _output) _output))
    (`Controller.Possess` Target InPawn)
    (set `MovementComponent.Velocity` _output_get (`Character.CharacterMovement` _output))
    (else
      (`|ExecutionSequence`
        (:`then_0`
          (`KismetSystemLibrary.Delay` (/ BlendTime 2.0))
          (goto _label_2))
        (:`then_1`
          (`TimelineComponent.SetPlayRate` (`self.Fading`) (/ 1.0 BlendTime))
          (bind (_direction _alpha) (`Timeline|Fading` :!via `PlayFromStart`)
            (:`Update`
              (`PlayerCameraManager.SetManualCameraFade` (`GameplayStatics.GetPlayerCameraManager` 0) _alpha (struct :`A` 1.0) false))))))))

(event `ReleaseKick`
  (bind _returnvalue (<= (`self.HoldDuration`) 0.2))
  ;[1 1 1] kick
  (set `self.IsCharging` false)
  (`self.KickLaunch` _returnvalue)
  (if _returnvalue
    (set `CharacterMovementComponent.MaxWalkSpeed` (`self.CharacterSpeed`) (`self.CharacterMovement`) :!label _label_3)
    (else
      (`KismetSystemLibrary.Delay` 0.15)
      (if (not (`self.IsCharging`))
        (goto _label_3)))))

(fn `Interact`
  (`self.ChargeKick`))

(fn `KickLaunch`
  (params (UpKick :type Boolean))
  (locals (HitSomething :type Boolean) (DrawBackPoint :type "Vector Structure"))
  (bind _returnvalue (`SceneComponent.K2_GetComponentLocation` (`self.CapsuleComponent`)))
  (bind _returnvalue_2 (`KismetMathLibrary.GetForwardVector` (`SceneComponent.K2_GetComponentRotation` (`self.Sprite`))))
  (bind _outactors (`GameplayStatics.GetAllActorsWithTag` "KickIgnore"))
  (bind _outhits (`KismetSystemLibrary.SphereTraceMulti` (+ _returnvalue (* _returnvalue_2 2.0)) (+ _returnvalue (* _returnvalue_2 10.0)) 8.0 "TraceTypeQuery2" false _outactors "None" true (struct :`R` 1.0 :`A` 1.0) (struct :`G` 1.0 :`A` 1.0) 1.0))
  (if (`KismetArrayLibrary.Array_IsNotEmpty` _outhits)
    (for _array_element _outhits
      (bind (_bblockinghit _binitialoverlap _time _distance _location _impactpoint _normal _impactnormal _physmat _hitactor _hitcomponent) (`GameplayStatics.BreakHitResult` _array_element))
      (bind _componenttags (`ActorComponent.ComponentTags` _hitcomponent))
      (bind _returnvalue_3 (`KismetArrayLibrary.Array_IsEmpty` _componenttags))
      (if _returnvalue_3
        (`|ExecutionSequence`
          (:`then_0`
            (set `local.HitSomething` true :!label _label))
          (:`then_1`
            (set `local.DrawBackPoint` _impactnormal :!label _label_2)
            (`/Engine/EditorBlueprintResources/StandardMacros.IsValid` _hitactor
              (:`Is Valid`
                (bind _returnvalue_4 (`self.GetComponentByClass` _hitactor "/Game/Blueprints/Characters/Components/BPC_Kickable.BPC_Kickable_C"))
                (`/Engine/EditorBlueprintResources/StandardMacros.IsValid` _returnvalue_4
                  (:`Is Valid`
                    (if _returnvalue_3
                      (`/Game/Blueprints/Characters/Components/BPC_Kickable.GetKicked` _returnvalue_4 (`KismetMathLibrary.GetDirectionUnitVector` (`SceneComponent.K2_GetComponentLocation` (`self.Sprite`)) (`self.K2_GetActorLocation` _hitactor)) UpKick :!label _label_3)
                      (else
                        (bind _returnvalue_5 (== (stale _array_element_2) "KickIgnore"))
                        (if (not _returnvalue_5)
                          (goto _label_3))))))))))
        (else
          (for _array_element_2 _componenttags
            (if (not _returnvalue_5)
              (goto _label)))
          (goto _label_2))))
    (if (`local.HitSomething`)
      (set `local.HitSomething` false)
      (`|ExecutionSequence`
        (:`then_0`
          ;[1 1 1] FX
          (`NiagaraFunctionLibrary.SpawnSystemAtLocation` (`self.KickParticle`) (`SceneComponent.GetSocketLocation` (`self.Sprite`) "HitPos")))
        (:`then_1`
          ;[1 1 1] DrawBack
          (`/Game/Blueprints/Characters/Components/BPC_Kickable.DrawBack` (`self.BPC_Kickable`) (`KismetMathLibrary.GetDirectionUnitVector` (0.0 0.0 0.0) (`local.DrawBackPoint`)) UpKick (`self.Grounded`)))))))

(fn `MergeCharacter`
  (params (UpperHalfRef :type "/Game/Blueprints/Characters/BP_Character_Top Object Reference") (DoRespawn :type Boolean))
  (if (not (`/Game/Blueprints/Characters/BP_Character_Top.IsRaging` UpperHalfRef))
    (set `self.DoRespawn` DoRespawn)
    (bind _asbp_character_base (cast `/Game/Blueprints/Characters/BP_Character_Base` (`Controller.K2_GetPawn` (`/Game/Blueprints/Library/BPFL_Fonction_Library.GetZombiePlayerController`))))
    (`PrimitiveComponent.SetCollisionEnabled` (`Character.CapsuleComponent` UpperHalfRef) "NoCollision")
    (`PrimitiveComponent.SetCollisionEnabled` (`self.CapsuleComponent`) "NoCollision")
    (bind _returnvalue (`|SpawnActorFromClass` "/Game/Blueprints/Characters/BP_Character_Full.BP_Character_Full_C" (`KismetMathLibrary.MakeTransform` (`KismetMathLibrary.TransformLocation` (`self.GetTransform`) (0.0 0.0 10.0))) "AdjustIfPossibleButDontSpawnIfColliding" "MultiplyWithRoot" null (`/Game/Blueprints/Characters/BP_Character_Base.IsFacingRight` _asbp_character_base) false false (0.0 0.0 0.0) (0.0 0.0 0.0) (`self.CurrentCameraTrigger`) null))
    (`/Engine/EditorBlueprintResources/StandardMacros.IsValid` _returnvalue
      (:`Is Valid`
        (`self.K2_DestroyActor` UpperHalfRef)
        (`self.SetCamZRotation` _returnvalue (.yaw (`SpringArmComponent.GetTargetRotation` (`self.SpringArm`))))
        (bind _asbp_player_controller (cast `/Game/Blueprints/Controllers/BP_Player_Controller` (`GameplayStatics.GetPlayerController` 0)))
        (`Controller.Possess` _asbp_player_controller _returnvalue)
        (if (`self.DoRespawn`)
          (`/Game/Blueprints/Characters/BP_Character_Full.Respawn` _returnvalue))
        (bind _returnvalue_2 (`|GetDataTableRow` "/Game/Sound/DT_Sound_List.DT_Sound_List" "A_Zombie_Fusion")
          (:`then`
            (`GameplayStatics.PlaySound2D` (break `/Game/Blueprints/Structures/SSound` _returnvalue_2) 1.0 1.0 0.0 null null)
            (`self.K2_DestroyActor`))))
      (:`Is Not Valid`
        (`PrimitiveComponent.SetCollisionEnabled` (`Character.CapsuleComponent` UpperHalfRef) "QueryAndPhysics")
        (`PrimitiveComponent.SetCollisionEnabled` (`self.CapsuleComponent`) "QueryAndPhysics")
        (set `self.DoRespawn` false)
        (`/Game/Blueprints/Characters/BP_Character_Top.FastCamBlendReverse` UpperHalfRef)))))

(fn `MergeObject`
  (params (ObjectToMerge :type "Object Object Reference")))

(fn `Respawn`
  (`parent.Respawn`)
  (bind (_asbp_camera_manager _pawntarget _checkpoint) (`/Game/Blueprints/Library/BPFL_Fonction_Library.GetCameraManager`))
  (`/Engine/EditorBlueprintResources/StandardMacros.IsValid` _checkpoint
    (:`Is Valid`
      (`/Game/Blueprints/Objects/BP_Checkpoint.TpToCheckPoint` _checkpoint self)
      (bind _asbp_character_top (cast `/Game/Blueprints/Characters/BP_Character_Top` (`/Game/Blueprints/Characters/Components/BP_Death_AC.PartnerInDeath` (`self.BP_Death_AC`))))
      (if (`/Game/Blueprints/Characters/BP_Character_Top.IsRaging` _asbp_character_top)
        (`self.K2_DestroyActor` _asbp_character_top)
        (bind _returnvalue (`|SpawnActorFromClass` "/Game/Blueprints/Characters/BP_Character_Full.BP_Character_Full_C" (`KismetMathLibrary.MakeTransform` (`SceneComponent.K2_GetComponentLocation` (`/Game/Blueprints/Objects/BP_Checkpoint.PaperFlipbook` _checkpoint))) "Undefined" "MultiplyWithRoot" null true false false (0.0 0.0 0.0) (0.0 0.0 0.0) null null))
        (`Controller.Possess` (`/Game/Blueprints/Library/BPFL_Fonction_Library.GetZombiePlayerController`) _returnvalue)
        (bind _outactors (`GameplayStatics.GetAllActorsOfClass` "/Game/Blueprints/AI/BP_Control_Loss_Start.BP_Control_Loss_Start_C"))
        (`/Game/Blueprints/AI/BP_Control_Loss_Start.Reset` (`|GetArrayItem` _outactors))
        (`self.K2_DestroyActor`)
        (else
          (`self.MergeCharacter` _asbp_character_top true))))))

(fn `Separate`
  (`parent.Separate`)
  (bind _outactors (`GameplayStatics.GetAllActorsOfClass` "/Game/Blueprints/Characters/BP_Character_Top.BP_Character_Top_C"))
  (bind _asbp_player_controller (cast `/Game/Blueprints/Controllers/BP_Player_Controller` (`GameplayStatics.GetPlayerController` 0)))
  (`self.MySeparate` (`self.camTransitionSpeed`) _asbp_player_controller (`|GetArrayItem` _outactors)))

(fn `StopInteract`
  (`self.ReleaseKick`))

(fn `UserConstructionScript`
  (`parent.UserConstructionScript`))