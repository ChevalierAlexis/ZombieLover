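; Playable top half of a split character, partnered with BP_Character_Bottom for control handoff and linked respawn.
; On spawn it can launch off the separation, and jumps add a clamped directional boost.
; Grapple component state rotates and offsets the sprite and toggles the hanging capsule, with a timeline-driven blood trail to the hook.
; Separate blends the camera to the bottom half, fading when distant, then possesses it while preserving its velocity.
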(event `self.ReceiveBeginPlay`
  (bind _initialvelocity (`self.InitialVelocity`))
  (bind _launchheight (`self.LaunchHeight`))
  ;[1 1 1 1 48] begin
  (`parent.ReceiveBeginPlay`)
  (`PrimitiveComponent.SetCollisionEnabled` (`self.CapsuleHanging`) "NoCollision")
  (`self.ZipLineUsed`
    (:`then`
      (set `CharacterMovementComponent.GravityScale` 0.0 (`self.CharacterMovement`)))
    (:`else`
      (if (`self.LaunchOnSeparate`)
        (`self.LaunchCharacter` (`KismetMathLibrary.SelectVector` (`KismetMathLibrary.SelectVector` (`KismetMathLibrary.MakeVector` 60.0 0.0 _launchheight) (`KismetMathLibrary.MakeVector` -60.0 0.0 _launchheight) (`self.IsFacingRight`)) (`KismetMathLibrary.MakeVector` (.x (* _initialvelocity (1.0 1.0 0.0))) (.y (* _initialvelocity (1.0 1.0 0.0))) (`self.LaunchHeight`)) (== _initialvelocity (0.0 0.0 0.0))))
        (else
          (`KismetSystemLibrary.Delay` 0.1)
          (if (> (`self.ClimbCount`) 0)
            (`CharacterMovementComponent.SetMovementMode` (`self.CharacterMovement`) "MOVE_Flying" 0)))))))

(event `self.ReceiveTick`
  (params (DeltaSeconds :type "Float (single-precision)"))
  (bind (_returnvalue_x _returnvalue_y _returnvalue_z) (`KismetMathLibrary.BreakVector` (`SceneComponent.K2_GetComponentLocation` (`self.Sprite`))))
  (bind _grabpointhooked (`/Game/Blueprints/Characters/Components/BP_Grapple_AC.GrabPointHooked` (`self.BP_Grapple_AC`)))
  (bind (_returnvalue_x_2 _returnvalue_y_2 _returnvalue_z_2) (`KismetMathLibrary.BreakVector` (`SceneComponent.K2_GetComponentLocation` (`/Game/Blueprints/Objects/InputObjects/Bp_New_Grab_Point.HookPoint` _grabpointhooked))))
  (bind (_returnvalue1_roll _returnvalue1_pitch _returnvalue1_yaw) (`KismetMathLibrary.BreakRotator` (`/Game/Blueprints/Library/BPFL_Fonction_Library.Get rotation` (`KismetMathLibrary.MakeVector` _returnvalue_x_2 _returnvalue_y_2 _returnvalue_z_2) (`KismetMathLibrary.MakeVector` _returnvalue_x _returnvalue_y_2 _returnvalue_z))))
  (`parent.ReceiveTick` DeltaSeconds)
  (`/Engine/EditorBlueprintResources/StandardMacros.IsValid` _grabpointhooked
    (:`Is Valid`
      (`KismetSystemLibrary.PrintString` (`KismetStringLibrary.Conv_DoubleToString` _returnvalue1_pitch))
      (`SceneComponent.K2_SetRelativeRotation` (`self.Sprite`) (`KismetMathLibrary.MakeRotator` 0.0 (+ _returnvalue1_pitch 90.0) (`KismetMathLibrary.SelectFloat` 180.0 0.0 (> (`KismetMathLibrary.Abs` _returnvalue1_yaw) 90.0))) false false))))

(event `BloodTrailMove`
  (bind _bloodtrail (`self.BloodTrail`))
  (bind _grabpointhooked (`/Game/Blueprints/Characters/Components/BP_Grapple_AC.GrabPointHooked` (`self.BP_Grapple_AC`)))
  (bind _returnvalue (+ (`SceneComponent.K2_GetComponentLocation` (`self.Sprite`)) (0.0 0.0 10.0)))
  (bind _returnvalue_2 (`SceneComponent.K2_GetComponentLocation` (`/Game/Blueprints/Objects/InputObjects/Bp_New_Grab_Point.HookPoint` (`/Game/Blueprints/Characters/Components/BP_Grapple_AC.GrabPointHooked` (`self.BP_Grapple_AC`)))))
  ;[1 1 1] bloodgrapple
  (`TimelineComponent.SetPlayRate` (`self.linearTimeline`) 10.0)
  (`NiagaraFunctionLibrary.SpawnSystemAtLocation` "/Game/FX/Zombie/NS_Blood_Spark.NS_Blood_Spark" _returnvalue)
  (`ActorComponent.Activate` (`self.BloodTrail`) false)
  (bind (_direction _newtrack_0) (`Timeline|linearTimeline` :!via `PlayFromStart`)
    (:`Update`
      (`/Engine/EditorBlueprintResources/StandardMacros.IsValid` _grabpointhooked
        (:`Is Valid`
          (`SceneComponent.K2_SetWorldLocation` _bloodtrail (`KismetMathLibrary.VLerp` _returnvalue _returnvalue_2 _newtrack_0) false false))))
    (:`Finished`
      (`ActorComponent.Deactivate` _bloodtrail)
      (`/Engine/EditorBlueprintResources/StandardMacros.IsValid` _grabpointhooked
        (:`Is Valid`
          (`NiagaraFunctionLibrary.SpawnSystemAtLocation` "/Game/FX/Zombie/NS_Blood_Spark.NS_Blood_Spark" _returnvalue_2))))))

(event `self.BP_Grapple_AC.AdjustSprite`
  (bind _capsulehanging (`self.CapsuleHanging`))
  (bind _returnvalue (`KismetSystemLibrary.IsValid` (`/Game/Blueprints/Characters/Components/BP_Grapple_AC.GrabPointHooked` (`self.BP_Grapple_AC`))))
  ;[1 1 1] adjust sprite position when hanging up
  (`SceneComponent.K2_SetRelativeLocation` (`self.Sprite`) (`KismetMathLibrary.MakeVector` 0.0 0.0 (`KismetMathLibrary.SelectFloat` 0.0 -12.0 _returnvalue)) false false)
  (`SceneComponent.K2_SetRelativeLocation` (`self.RaySourceEnd`) (`KismetMathLibrary.MakeVector` 0.0 0.0 (`KismetMathLibrary.SelectFloat` -33.0 -6.0 _returnvalue)) false false)
  (if _returnvalue
    (`PrimitiveComponent.SetCollisionEnabled` _capsulehanging "QueryAndPhysics")
    (else
      (`PrimitiveComponent.SetCollisionEnabled` _capsulehanging "NoCollision")
      (`self.HandleRotation`))))

(event `MySeparate`
  (params (BlendTime :type "Float (single-precision)") (Target :type "PlayerController Object Reference") (InPawn :type "Pawn Object Reference"))
  ;[1 1 1 1 48] Separate
  (if (< (`self.GetDistanceTo` InPawn self) 500.0)
    (`PlayerController.SetViewTargetWithBlend` Target InPawn BlendTime "VTBlend_EaseInOut" 2.0 false)
    (`KismetSystemLibrary.Delay` BlendTime)
    ;;[1 1 1] Se souvenir de la velocité de la partie juste avant de la possess (donc après le delay)
    (bind _outactors (`GameplayStatics.GetAllActorsOfClass` "/Game/Blueprints/Characters/BP_Character_Bottom.BP_Character_Bottom_C" :!label _label))
    (bind _output (`|GetArrayItem` _outactors))
    (bind _output_get (set `/Game/Blueprints/Characters/BP_Character_Base.OldVelocity` (`self.GetVelocity` _output) _output))
    (`Controller.Possess` Target InPawn)
    (set `MovementComponent.Velocity` _output_get (`Character.CharacterMovement` _output))
    (else
      ;;[1 1 1] Fade
      (`|ExecutionSequence`
        (:`then_0`
          (`KismetSystemLibrary.Delay` (/ BlendTime 2.0))
          (goto _label))
        (:`then_1`
          (`TimelineComponent.SetPlayRate` (`self.Fading_0`) (/ 1.0 BlendTime))
          (bind (_direction _alpha) (`Timeline|Fading_0` :!via `PlayFromStart`)
            (:`Update`
              (`PlayerCameraManager.SetManualCameraFade` (`GameplayStatics.GetPlayerCameraManager` 0) _alpha (struct :`A` 1.0) false))))))))

(event `SetPartner`
  (params (BottomRef :type "/Game/Blueprints/Characters/BP_Character_Bottom Object Reference"))
  ;[1 1 1] setPartner
  (set `/Game/Blueprints/Characters/Components/BP_Death_AC.PartnerInDeath` BottomRef (`self.BP_Death_AC`))
  (`/Game/Blueprints/Characters/BP_Character_Bottom.SetPartner` BottomRef self))

(event `self.OnJumped`
  ;[1 1 1] Boost Jump
  (`self.LaunchCharacter` (`KismetMathLibrary.MakeVector` (`KismetMathLibrary.FClamp` (+ (* (`self.BoostJump`) (`|GetInputActionValue`)) (.x (`self.GetVelocity`))) -200.0 200.0) (`KismetMathLibrary.FClamp` (+ (.y (`self.GetVelocity`)) (* (`self.BoostJump`) (`|GetInputActionValue`))) -200.0 200.0)) true))

(event `Clear`
  (bind _splinemeshcomponents (`self.SplineMeshComponents`))
  (for _array_element _splinemeshcomponents
    (`ActorComponent.K2_DestroyComponent` _array_element))
  (`KismetArrayLibrary.Array_Clear` _splinemeshcomponents))

(event `FastCamBlend`
  ;[1 1 1] cam effect
  (bind _asbp_player_controller (cast `/Game/Blueprints/Controllers/BP_Player_Controller` (`GameplayStatics.GetPlayerController` 0)))
  (`PlayerController.SetViewTargetWithBlend` _asbp_player_controller (`/Game/Blueprints/Characters/Components/BP_Death_AC.PartnerInDeath` (`self.BP_Death_AC`)) 0.05 "VTBlend_EaseInOut" 2.0 false))

(event `FastCamBlendReverse`
  ;[1 1 1] cam effect
  (`/Engine/EditorBlueprintResources/StandardMacros.IsValid` (stale `FastCamBlend` _asbp_player_controller)
    (:`Is Valid`
      (`PlayerController.SetViewTargetWithBlend` (stale `FastCamBlend` _asbp_player_controller) self 0.05 "VTBlend_EaseInOut" 2.0 false))))

(event `FallingEvent`
  (if (not (`NavMovementComponent.IsFalling` (`self.CharacterMovement`)))
    (`/Game/Blueprints/Library/BPFL_Fonction_Library.PlaySound` self "A_Zombie_Top_Falling")
    (remove `self.OnTick` (delegate `FallingEvent`))))

(fn `Clean Bind Event To Timeline`
  (params (Event :type "Delegate (by ref)"))
  (clear `self.UpdateTimeline`)
  (add `self.UpdateTimeline` Event))

(fn `Find Nearest Grab Point`
  (returns (`AsBp New Grab Point` :type "/Game/Blueprints/Objects/InputObjects/Bp_New_Grab_Point Object Reference"))
  (bind _returnvalue (`/Game/Blueprints/Library/BPFL_Fonction_Library.FindNearestActorOfClass` "/Game/Blueprints/Objects/InputObjects/Bp_New_Grab_Point.Bp_New_Grab_Point_C" (`SceneComponent.K2_GetComponentLocation` (`self.CapsuleComponent`))))
  (`/Engine/EditorBlueprintResources/StandardMacros.IsValid` _returnvalue
    (:`Is Valid`
      (if (< (`self.GetDistanceTo` _returnvalue) (`self.GrabRange`))
        (bind _asbp_new_grab_point (cast `/Game/Blueprints/Objects/InputObjects/Bp_New_Grab_Point` _returnvalue))
        (return _asbp_new_grab_point)
        (else
          (return null))))))

(fn `MergeObject`
  (params (ObjectToMerge :type "Object Object Reference")))

(fn `Respawn`
  (`parent.Respawn`)
  (bind _asbp_character_bottom (cast `/Game/Blueprints/Characters/BP_Character_Bottom` (`/Game/Blueprints/Characters/Components/BP_Death_AC.PartnerInDeath` (`self.BP_Death_AC`))))
  (`/Game/Blueprints/Characters/BP_Character_Bottom.Respawn` _asbp_character_bottom))

(fn `Separate`
  (params (ControlTop :type Boolean))
  (`parent.Separate` true)
  (bind _outactors (`GameplayStatics.GetAllActorsOfClass` "/Game/Blueprints/Characters/BP_Character_Bottom.BP_Character_Bottom_C"))
  (bind _asbp_player_controller (cast `/Game/Blueprints/Controllers/BP_Player_Controller` (`GameplayStatics.GetPlayerController` 0)))
  (`self.MySeparate` (`self.camTransitionSpeed`) _asbp_player_controller (`|GetArrayItem` _outactors)))

(fn `UserConstructionScript`
  (`parent.UserConstructionScript`))