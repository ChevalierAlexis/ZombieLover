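; Base flipbook-sprite character, handling movement feel, camera, animation, interaction with objects or carrots, and death/respawn.
; Jumps use timer-based coyote time, velocity-scaled trace buffering and timeline squash-and-stretch.
; A timer refreshes depth-of-field focus on the sprite, while Tick eases spring-arm yaw toward the camera manager's tilt, mirrored to any PartnerInDeath.
; Also provides sprite shake, fade-to-black fast travel and a right-click debug dash with trajectory preview.
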(event `self.ReceiveBeginPlay`
  (bind (_asbp_camera_manager _pawntarget) (`/Game/Blueprints/Library/BPFL_Fonction_Library.GetCameraManager`))
  (bind _currentcameratrigger (`self.CurrentCameraTrigger`))
  (bind _sprite (`self.Sprite`))
  (`|ExecutionSequence`
    (:`then_0`
      (set `CharacterMovementComponent.JumpZVelocity` (`self.CharacterJumpHeight`) (`self.CharacterMovement`))
      (set `CharacterMovementComponent.MaxWalkSpeed` (`self.CharacterSpeed`) (`self.CharacterMovement`))
      (set `self.BaseScale` (`SceneComponent.RelativeScale3D` _sprite))
      (set `self.BaseSpriteRelativeLocation` (`SceneComponent.RelativeLocation` _sprite))
      (`self.FocusUpdate`))
    (:`then_1`
      (`self.HandleRotation`)
      (bind _output_get (set `self.CamManager` _asbp_camera_manager))
      (`/Engine/EditorBlueprintResources/StandardMacros.IsValid` _pawntarget
        (:`Is Not Valid`
          (set `/Game/Blueprints/CameraManager/BP_Camera_Manager.PawnTarget` self _output_get))))
    (:`then_2`
      (`KismetSystemLibrary.K2_SetTimer` null "FocusUpdate" 0.1 true)
      (`/Engine/EditorBlueprintResources/StandardMacros.IsValid` _currentcameratrigger
        (:`Is Valid`
          (`/Game/Blueprints/Objects/LevelDesignZones/BP_CameraTrigger.InstantCamUpdate` _currentcameratrigger self)
          (`self.FocusUpdate`)
          (`/Game/Blueprints/Library/BPFL_Fonction_Library.PlaySound` null "A_Zombie_FullBody_Walk"))))))

(event `loop`
  ;[1 1 1] debug dash
  (if (`self.MouseIsDown`)
    (set `self.Debug Dash Force` (+ (`self.Debug Dash Force`) 0.1) :!label _label)
    (`GameplayStatics.Blueprint_PredictProjectilePath_ByObjectType` :`StartPos` (`SceneComponent.K2_GetComponentLocation` (`self.Sprite`)) :`LaunchVelocity` (* (`self.Debug Dash Force`) (`KismetMathLibrary.MakeVector` (`KismetMathLibrary.SelectFloat` 0.0 (`KismetMathLibrary.SelectFloat` 100.0 -100.0 (`self.IsFacingRight`)) (== (`|GetInputActionValue`) 0.0)) 0.0 50.0)) :`ObjectTypes` (`|MakeArray` "ObjectTypeQuery4" :!type "EObjectTypeQuery Enum") :`DrawDebugType` "ForDuration" :`DrawDebugTime` 0.02 :`SimFrequency` 100.0 :`MaxSimTime` 0.1)
    (`KismetSystemLibrary.Delay` 0.01)
    (`self.loop`)))

(event `Key|RightMouseButton`
  (params (Key :type "Key Structure"))
  ;[1 1 1] debug dash
  (:`Pressed`
    (set `self.MouseIsDown` true)
    (goto _label))
  (:`Released`
    (set `self.MouseIsDown` false)
    (if (`/Game/Blueprints/Library/BPFL_Fonction_Library.Is Current Player Alive`)
      (`self.LaunchCharacter` (* (`self.Debug Dash Force`) (`KismetMathLibrary.MakeVector` (`KismetMathLibrary.SelectFloat` 0.0 (`KismetMathLibrary.SelectFloat` 100.0 -100.0 (`self.IsFacingRight`)) (== (`|GetInputActionValue`) 0.0)) 0.0 50.0)))
      (set `self.Debug Dash Force` 5.0))))

(event `self.ReceiveTick`
  (params (DeltaSeconds :type "Float (single-precision)"))
  (`self.HandleAnimation`)
  (`self.CamTiltTick`)
  (`self.OnTick`))

(event `FocusUpdate`
  (bind _camera (`self.Camera`))
  ;[1 1 1] autoDOF
  (bind _output_get (set `self.FocusDistance` (`KismetMathLibrary.VSize` (- (`SceneComponent.K2_GetComponentLocation` (`self.Sprite`)) (`SceneComponent.K2_GetComponentLocation` _camera)))))
  (set `CameraComponent.PostProcessSettings` (make `PostProcessSettings` :`DepthOfFieldFstop` 1.0 :`DepthOfFieldMinFstop` 11.0 :`AmbientOcclusionTemporalBlendWeight` 0.0 :`DepthOfFieldSensorWidth` (`self.Sensor Width (Mm)`) :`DepthOfFieldFocalDistance` _output_get) _camera))

(event `FastTravelTo`
  (params (Time :type "Float (single-precision)") (NewLocation :type "Vector Structure"))
  (`TimelineComponent.SetPlayRate` (`self.Fading`) (/ 1.0 Time))
  (set `/Game/Blueprints/CameraManager/BP_Camera_Manager.IsInCinematic` true (`/Game/Blueprints/Library/BPFL_Fonction_Library.GetCameraManager`))
  (bind (_direction _alpha) (`Timeline|Fading` :!label _label_2)
    (:`Update`
      (`PlayerCameraManager.SetManualCameraFade` (`GameplayStatics.GetPlayerCameraManager` 0) _alpha (struct :`A` 1.0) false))
    (:`Finished`
      (`/Engine/EditorBlueprintResources/StandardMacros.FlipFlop`
        (:`A`
          (`self.K2_SetActorLocation` NewLocation false true)
          (goto _label_2 :!via `Reverse`))
        (:`B`
          (set `/Game/Blueprints/CameraManager/BP_Camera_Manager.IsInCinematic` false (`/Game/Blueprints/Library/BPFL_Fonction_Library.GetCameraManager`)))))))

(event `RayTraceToPlayer`
  ;[1 1 1] A supprimer ?
  ;;[1 1 1] raycast qui pointe le joueur
)

(event `self.K2_OnMovementModeChanged`
  (params (PrevMovementMode :type "EMovementMode Enum" :default "MOVE_None") (NewMovementMode :type "EMovementMode Enum" :default "MOVE_None") (PrevCustomMode :type Byte) (NewCustomMode :type Byte))
  ;[1 1 1] Coyote Time & Jump Buffering
  (if (`|EnumEquality` NewMovementMode "MOVE_Falling")
    (bind _returnvalue (`KismetSystemLibrary.K2_SetTimerDelegate` (delegate `CoyoteTimePassed`) (`self.CoyoteTimeDuration`)))
    (set `self.CoyoteTime` _returnvalue)))

(event `JumpSqueeze`
  ;[1 1 1] JumpSqueeze
  (`TimelineComponent.SetPlayRate` (`self.JumpSqueezeAnim`) (`self.JumpSqueezeSpeed`))
  (bind (_direction _alpha) (`Timeline|JumpSqueezeAnim` :!via `PlayFromStart`)
    (:`Update`
      (`SceneComponent.SetRelativeScale3D` (`self.Sprite`) (`KismetMathLibrary.VLerp` (`self.BaseScale`) (* (`self.BaseScale`) (`self.SqueezeFactorJump`)) _alpha)))))

(event `CoyoteTimePassed`
  ;[1 1 1] Coyote Time & Jump Buffering
)

(event `SpeedBoostOnYAxis`
  ;[1 1 1] A supprimer ?
  ;;[1 1 1] Augmenter la vitesse si tu bouge en profondeur
)

(event `self.OnLanded`
  (params (Hit :type "HitResult Structure (by ref)"))
  ;[1 1 1] Coyote Time & Jump Buffering
  (`self.LandSqueeze`)
  (`KismetSystemLibrary.K2_ClearAndInvalidateTimerHandle` (`self.CoyoteTime`))
  (if (`self.JumpBuffered`)
    (`self.JumpSqueeze`)
    (`KismetSystemLibrary.Delay` 0.001)
    (`self.Jump`)
    (set `self.JumpBuffered` false)))

(event `LandSqueeze`
  ;[1 1 1] LandSqueeze
  (`TimelineComponent.SetPlayRate` (`self.LandSqueezeAnimation`) (`self.JumpSqueezeSpeed`))
  (bind (_direction _alpha) (`Timeline|LandSqueezeAnimation` :!via `PlayFromStart`)
    (:`Update`
      (`SceneComponent.SetRelativeScale3D` (`self.Sprite`) (`KismetMathLibrary.VLerp` (`self.BaseScale`) (* (`self.BaseScale`) (`self.SqueezeFactorLand`)) _alpha)))))

(event `BufferJump`
  (bind _returnvalue (`SceneComponent.K2_GetComponentLocation` (`self.RaySourceEnd`)))
  ;[1 1 1] Coyote Time & Jump Buffering
  (bind (_outhit _returnvalue_2) (`KismetSystemLibrary.LineTraceSingle` _returnvalue (+ _returnvalue (`KismetMathLibrary.MakeVector` 0.0 0.0 (`KismetMathLibrary.FClamp` (* (`self.JumpBufferDistanceFactor`) (.z (`self.GetVelocity`))) -100.0 0.0))) "TraceTypeQuery1"))
  (set `self.JumpBuffered` _returnvalue_2))

(event `HandleRotation`
  (bind _sprite (`self.Sprite`))
  ;[1 1 1] handle rotation
  (if (`self.IsFacingRight`)
    (`SceneComponent.K2_SetRelativeRotation` :`self` _sprite)
    (else
      (`SceneComponent.K2_SetRelativeRotation` _sprite (struct :`Yaw` 180.0) false false))))

(event `HandleAnimation`
  (bind (_returnvalue_x _returnvalue_y _returnvalue_z) (`KismetMathLibrary.BreakVector` (`self.GetVelocity`)))
  ;[1 1 1] A supprimer ?
  ;;[1 1 1] handle animation
  (if (`self.IsSpecialAnimPlaying`)
    _
    (elif (`NavMovementComponent.IsFalling` (`self.CharacterMovement`))
      (`PaperFlipbookComponent.SetFlipbook` (`self.Sprite`) (select `bool` (< _returnvalue_z 0.0) :`false` (`self.IdleAnim`) :`true` (`self.WalkAnim`)))
      (else
        (`PaperFlipbookComponent.SetFlipbook` (`self.Sprite`) (select `bool` (> (`KismetMathLibrary.VSize` (`MovementComponent.Velocity` (`self.CharacterMovement`))) 0.0) :`false` (`self.IdleAnim`) :`true` (`self.WalkAnim`)))))))

(event `TiltCam`
  (params (A :type "Float (double-precision)"))
  (bind _cammanager (`self.CamManager`))
  (bind _tiltcammaxangle (`self.TiltCamMaxAngle`))
  (bind _returnvalue (- (`/Game/Blueprints/CameraManager/BP_Camera_Manager.FuturCamTilt` _cammanager) (`/Game/Blueprints/CameraManager/BP_Camera_Manager.BaseCamTilt` _cammanager)))
  ;[1 1 1] TiltCam
  ;;[1 1 1] reset si demi tour en plein mouvement (attention un input renvoie zero au début de l'appuie)
  (if (and (!= A 0.0) (!= A (/ _returnvalue (`KismetMathLibrary.Abs` _returnvalue))))
    (`self.ResetBaseCam`))
  (set `/Game/Blueprints/CameraManager/BP_Camera_Manager.FuturCamTilt` (`KismetMathLibrary.FClamp` (+ (* A (`self.TiltCamSpeed`)) (`/Game/Blueprints/CameraManager/BP_Camera_Manager.FuturCamTilt` (`self.CamManager`))) (- -90.0 _tiltcammaxangle) (+ -90.0 _tiltcammaxangle)) (`self.CamManager`)))

(event `ResetToIdle`
  (bind _sprite (`self.Sprite`))
  ;[1 1 1] A supprimer ?
  ;;[1 1 1] handle animation
  (set `self.IsSpecialAnimPlaying` false)
  (`PaperFlipbookComponent.SetLooping` _sprite true)
  (if (not (`PaperFlipbookComponent.IsPlaying` _sprite))
    (`PaperFlipbookComponent.Play` _sprite)))

(event `CamTiltTick`
  (bind _cammanager (`self.CamManager`))
  (bind _cammanager_2 (`self.CamManager`))
  (bind _tiltcammaxangle (`self.TiltCamMaxAngle`))
  (bind _basecamtilt (`/Game/Blueprints/CameraManager/BP_Camera_Manager.BaseCamTilt` _cammanager))
  (bind _yaw (.yaw (`SpringArmComponent.GetTargetRotation` (`self.SpringArm`))))
  (bind _returnvalue (- (`/Game/Blueprints/CameraManager/BP_Camera_Manager.FuturCamTilt` _cammanager_2) (`/Game/Blueprints/CameraManager/BP_Camera_Manager.BaseCamTilt` _cammanager_2)))
  (bind _returnvalue_2 (/ (`KismetMathLibrary.Abs` (- (/ _yaw _basecamtilt) 1.0)) (`KismetMathLibrary.Abs` (- (/ (`/Game/Blueprints/CameraManager/BP_Camera_Manager.FuturCamTilt` _cammanager) _basecamtilt) 1.0))))
  ;[1 1 1] TiltCam
  (if (!= (`/Game/Blueprints/CameraManager/BP_Camera_Manager.FuturCamTilt` (`self.CamManager`)) _yaw)
    (`self.SetCamZRotation` (`KismetMathLibrary.SelectFloat` (`KismetMathLibrary.FClamp` (+ _yaw (* (`CurveFloat.GetFloatValue` (`self.curveCAmTilt`) _returnvalue_2) (/ _returnvalue (`KismetMathLibrary.Abs` _returnvalue)) 0.28)) (- -90.0 _tiltcammaxangle) (+ -90.0 _tiltcammaxangle)) (`/Game/Blueprints/CameraManager/BP_Camera_Manager.FuturCamTilt` (`self.CamManager`)) (<= _returnvalue_2 0.995)))
    (else
      (`self.ResetBaseCam`))))

(event `ShakeForDuration`
  (params (Interval :type "Float (single-precision)" :default 0.06) (Duration :type "Float (single-precision)" :default 2.0))
  (`KismetSystemLibrary.K2_ClearTimer` null "ShakeSpriteHorizontal")
  (`KismetSystemLibrary.K2_ClearTimer` null "ClearShake")
  (`KismetSystemLibrary.K2_SetTimer` null "ShakeSpriteHorizontal" Interval true)
  (`KismetSystemLibrary.K2_SetTimer` null "ClearShake" Duration))

(event `SetCamZRotation`
  (params (`New Rotation Z` :type "Float (single-precision)"))
  (bind _returnvalue (`self.GetComponentByClass` "/Game/Blueprints/Characters/Components/BP_Death_AC.BP_Death_AC_C"))
  (bind _springarm (`self.SpringArm`))
  (bind _partnerindeath (`/Game/Blueprints/Characters/Components/BP_Death_AC.PartnerInDeath` _returnvalue))
  ;[1 1 1] TiltCam
  (`|ExecutionSequence`
    (:`then_0`
      (`SceneComponent.K2_SetWorldRotation` _springarm (`KismetMathLibrary.MakeRotator` (.roll (`SpringArmComponent.GetTargetRotation` _springarm)) (.pitch (`SpringArmComponent.GetTargetRotation` _springarm)) `New Rotation Z`) false false))
    (:`then_1`
      ;;[1 1 1] le player actuellement controlée update son partenaire aussi s'il en as un
      (if (== (`/Game/Blueprints/Library/BPFL_Fonction_Library.CastToPlayerCharacter`) self)
        (`/Engine/EditorBlueprintResources/StandardMacros.IsValid` _returnvalue
          (:`Is Valid`
            (`/Engine/EditorBlueprintResources/StandardMacros.IsValid` _partnerindeath
              (:`Is Valid`
                (`self.SetCamZRotation` _partnerindeath `New Rotation Z`)))))))))

(event `ResetBaseCam`
  ;[1 1 1] TiltCam
  (set `/Game/Blueprints/CameraManager/BP_Camera_Manager.BaseCamTilt` (.yaw (`SpringArmComponent.GetTargetRotation` (`self.SpringArm`))) (`self.CamManager`)))

(event `ShakeSpriteHorizontal`
  (bind (_basespriterelativelocation_x _basespriterelativelocation_y _basespriterelativelocation_z) (`KismetMathLibrary.BreakVector` (`self.BaseSpriteRelativeLocation`)))
  (bind _isa (`/Engine/EditorBlueprintResources/StandardMacros.FlipFlop`)
    (:`A`
      _)
    (:`B`
      _))
  (`SceneComponent.K2_SetRelativeLocation` (`self.Sprite`) (`KismetMathLibrary.MakeVector` (+ (`KismetMathLibrary.SelectFloat` -1.0 1.0 _isa) _basespriterelativelocation_x) _basespriterelativelocation_y _basespriterelativelocation_z) false false))

(event `ClearShake`
  (`KismetSystemLibrary.K2_ClearTimer` null "ShakeSpriteHorizontal")
  (`SceneComponent.K2_SetRelativeLocation` (`self.Sprite`) (`self.BaseSpriteRelativeLocation`) false false))

(event `ResetCamTilt`
  ;[1 1 1] TiltCam
  ;;[1 1 1] reset
  (`self.ResetBaseCam`)
  (set `/Game/Blueprints/CameraManager/BP_Camera_Manager.FuturCamTilt` -90.0 (`self.CamManager`)))

(fn `CanJumpInternal`
  (returns (ReturnValue :type Boolean))
  (bind _returnvalue (`parent.CanJumpInternal`))
  (return (or _returnvalue (> (`KismetSystemLibrary.K2_GetTimerRemainingTimeHandle` (`self.CoyoteTime`)) 0.0))))

(fn `FindCarrot`
  (returns (`AsBP Carrot` :type "/Game/Blueprints/Objects/BP_Carrot Object Reference"))
  (bind _returnvalue (`/Game/Blueprints/Library/BPFL_Fonction_Library.FindNearestActorOfClass` "/Game/Blueprints/Objects/BP_Carrot.BP_Carrot_C" (`SceneComponent.K2_GetComponentLocation` (`self.CapsuleComponent`))))
  (`/Engine/EditorBlueprintResources/StandardMacros.IsValid` _returnvalue
    (:`Is Valid`
      (if (< (`self.GetDistanceTo` _returnvalue) 30.0)
        (bind _asbp_carrot (cast `/Game/Blueprints/Objects/BP_Carrot` _returnvalue)
          (:`then`
            (return _asbp_carrot))
          (:`CastFailed`
            (return null)))))))

(fn `Get IA_Move`
  (returns (IA_Move_Right :type "Float (double-precision)") (IA_Move_Front :type "Float (double-precision)"))
  (return (`|GetInputActionValue`) (`|GetInputActionValue`)))

(fn `Interact`
  (bind _interactable (`self.Interactable`))
  (`/Engine/EditorBlueprintResources/StandardMacros.IsValid` _interactable
    (:`Is Valid`
      (`/Game/Blueprints/Objects/InputObjects/BP_Interactable.Interract` _interactable))
    (:`Is Not Valid`
      (bind _asbp_carrot (`self.FindCarrot`))
      (`/Engine/EditorBlueprintResources/StandardMacros.IsValid` _asbp_carrot
        (:`Is Valid`
          (if (not (`self.IsEatingCarrot`))
            (set `self.IsEatingCarrot` true)
            (`self.K2_DestroyActor` _asbp_carrot)))))))

(fn `IsOnGround`
  (returns (Grounded :type Boolean))
  (bind _outactors (`GameplayStatics.GetAllActorsWithTag` "KickIgnore"))
  (bind _outhits (`KismetSystemLibrary.SphereTraceMulti` (`SceneComponent.K2_GetComponentLocation` (`self.RaySource`)) (`SceneComponent.K2_GetComponentLocation` (`self.RaySourceEnd`)) 1.0 "TraceTypeQuery1" false _outactors "None" true (struct :`R` 1.0 :`A` 1.0) (struct :`G` 1.0 :`A` 1.0) 1.0))
  (return (`KismetArrayLibrary.Array_IsNotEmpty` _outhits)))

(fn `Respawn`
  (`SceneComponent.SetHiddenInGame` (`self.Sprite`) false false)
  (`PrimitiveComponent.SetCollisionEnabled` (`self.CapsuleComponent`) "QueryAndPhysics")
  (set `CharacterMovementComponent.GravityScale` 1.0 (`self.CharacterMovement`)))

(fn `Separate`
  (params (ControlTop :type Boolean :default true)))

(fn `SetA`
  (params (Object :type "Pawn Object Reference"))
  (bind (_returnvalue_x _returnvalue_y _returnvalue_z) (`KismetMathLibrary.BreakVector` (`self.K2_GetActorLocation` Object)))
  (`SceneComponent.SetVisibility` (`self.A`) (`KismetSystemLibrary.IsValid` Object) false)
  (`/Engine/EditorBlueprintResources/StandardMacros.IsValid` Object
    (:`Is Valid`
      (`SceneComponent.K2_SetWorldLocation` (`self.A`) (`KismetMathLibrary.MakeVector` _returnvalue_x _returnvalue_y (+ _returnvalue_z 15.0)) false false))))

(fn `SpawnDeathAnim`
  (bind _charactermovement (`self.CharacterMovement`))
  (`/Game/Blueprints/Library/BPFL_Fonction_Library.PlaySound` self "A_Zombie_Death")
  (`SceneComponent.SetHiddenInGame` (`self.Sprite`) true false)
  (`PrimitiveComponent.SetCollisionEnabled` (`self.CapsuleComponent`) "NoCollision")
  (set `CharacterMovementComponent.GravityScale` 0.0 _charactermovement)
  (set `MovementComponent.Velocity` (0.0 0.0 0.0) _charactermovement)
  (`NiagaraFunctionLibrary.SpawnSystemAtLocation` (`self.DeathParticle`) (`SceneComponent.GetSocketLocation` (`self.Sprite`) "DeathAnchor")))

(fn `StopInteract`)

(fn `UserConstructionScript`
  (`CapsuleComponent.SetCapsuleHalfHeight` (`self.CapsuleComponent`) (`self.CharacterHeight`) true))