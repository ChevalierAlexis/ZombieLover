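; BP_Control_Loss_Start is a trigger volume that makes the player lose control of the Top half of the character, which turns into a raging AI.
; A Full or Top character overlap fires it once until Reset, separating a full body, possessing the nearest Bottom and unbinding separation events.
; The nearest Top is tagged, possessed by a spawned rage AI controller given the nearest patrol, and gains a kill component.
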(event `self.Box.OnComponentBeginOverlap`
  (params (OverlappedComponent :type "PrimitiveComponent Object Reference") (OtherActor :type "Actor Object Reference") (OtherComp :type "PrimitiveComponent Object Reference") (OtherBodyIndex :type Integer) (bFromSweep :type Boolean) (SweepResult :type "HitResult Structure (by ref)"))
  (bind _asbp_player_controller (`/Game/Blueprints/Library/BPFL_Fonction_Library.GetZombiePlayerController`))
  (bind _character_top (`self.Character_Top`))
  (bind _character_top_2 (`self.Character_Top`))
  ;[1 1 1] Le bottom ne trigger pas la zone
  (bind _asbp_character_full (cast `/Game/Blueprints/Characters/BP_Character_Full` OtherActor)
    (:`then`
      _)
    (:`CastFailed`
      (cast `/Game/Blueprints/Characters/BP_Character_Top` OtherActor)))
  (set `self.Other_Actor` OtherActor)
  (`/Engine/EditorBlueprintResources/StandardMacros.DoOnce` false :!label _label
    (:`Completed`
      ;[1 1 1] separe si le corps est complet
      (`/Engine/EditorBlueprintResources/StandardMacros.IsValid` _asbp_character_full
        (:`Is Valid`
          (`/Game/Blueprints/Characters/BP_Character_Base.Separate` _asbp_character_full))
        (:`Is Not Valid`
          _))
      ;[1 1 1] Posséder le bottom et bloquer le switch
      (bind _returnvalue (`/Game/Blueprints/Library/BPFL_Fonction_Library.FindNearestActorOfClass` "/Game/Blueprints/Characters/BP_Character_Bottom.BP_Character_Bottom_C" (`SceneComponent.K2_GetComponentLocation` (`self.Box`))))
      (bind _asbp_character_bottom (cast `/Game/Blueprints/Characters/BP_Character_Bottom` _returnvalue))
      (`Controller.Possess` _asbp_player_controller _asbp_character_bottom)
      (clear `/Game/Blueprints/Controllers/BP_Player_Controller.OnSeparation` _asbp_player_controller)
      ;[1 1 1] Donner un tag au Top
      (bind _returnvalue_2 (`/Game/Blueprints/Library/BPFL_Fonction_Library.FindNearestActorOfClass` "/Game/Blueprints/Characters/BP_Character_Top.BP_Character_Top_C" (`self.K2_GetActorLocation`)))
      (bind _asbp_character_top (cast `/Game/Blueprints/Characters/BP_Character_Top` _returnvalue_2))
      (bind _output_get (set `self.Character_Top` _asbp_character_top))
      (`KismetArrayLibrary.Array_Add` (`Actor.Tags` _output_get) "Booyah")
      ;[1 1 1] Spawn controller and possess + add component kill
      (bind _returnvalue_3 (`|SpawnActorFromClass` "/Game/Blueprints/AI/BP_AIC_Rage_Controller.BP_AIC_Rage_Controller_C" (`KismetMathLibrary.MakeTransform` (0.0 0.0 0.0)) "Undefined" "MultiplyWithRoot" null null))
      (`Controller.Possess` _returnvalue_3 _character_top_2)
      (bind _returnvalue_4 (`/Game/Blueprints/Library/BPFL_Fonction_Library.FindNearestActorOfClass` "/Game/Blueprints/AI/BP_Patrol.BP_Patrol_C" (`self.K2_GetActorLocation` _character_top_2)))
      (bind _asbp_patrol (cast `/Game/Blueprints/AI/BP_Patrol` _returnvalue_4))
      (set `/Game/Blueprints/AI/BP_AIC_Rage_Controller.Patrol` _asbp_patrol _returnvalue_3)
      (`AddComponent|NODE_AddBPC_Kill-0` :`self` _character_top)
      (set `/Game/Blueprints/Characters/BP_Character_Top.IsRaging` true _character_top))))

(event `Reset`
  (goto _label :!via `Reset`))

(fn `UserConstructionScript`
  (`BoxComponent.SetBoxExtent` (`self.Box`) (`self.BoxSize`) true))