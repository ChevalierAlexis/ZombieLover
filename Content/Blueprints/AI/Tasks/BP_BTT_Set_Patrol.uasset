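; Behavior tree task that assigns a patrol route to a patrolling BP_Ennemy.
; When the enemy's IsPatroling flag is set, it clears the itinerary, stores the nearest BP_Patrol actor on the enemy and copies that patrol's point locations into PatrolItinirary.
; The task finishes successfully whether or not the enemy patrols; a failed cast stops it without calling FinishExecute.
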(event `self.ReceiveExecuteAI`
  (params (OwnerController :type "AIController Object Reference") (ControlledPawn :type "Pawn Object Reference"))
  (bind _asbp_ennemy (cast `/Game/Blueprints/Characters/BP_Ennemy` ControlledPawn))
  (if (`/Game/Blueprints/Characters/BP_Ennemy.IsPatroling` _asbp_ennemy)
    (set `self.As BP Ennemy` _asbp_ennemy)
    (`KismetArrayLibrary.Array_Clear` (`/Game/Blueprints/Characters/BP_Ennemy.PatrolItinirary` (`self.As BP Ennemy`)))
    (bind _outactors (`GameplayStatics.GetAllActorsOfClass` "/Game/Blueprints/AI/BP_Patrol.BP_Patrol_C"))
    (bind _asbp_patrol (cast `/Game/Blueprints/AI/BP_Patrol` (`.ReturnValue` (`GameplayStatics.FindNearestActor` (`Actor.K2_GetActorLocation` (`self.As BP Ennemy`)) _outactors))))
    (bind _output_get (set `/Game/Blueprints/Characters/BP_Ennemy.Patrol` _asbp_patrol (`self.As BP Ennemy`)))
    (for _array_element (`/Game/Blueprints/AI/BP_Patrol.PatrolPoints` _output_get)
      (`KismetArrayLibrary.Array_Add` (`/Game/Blueprints/Characters/BP_Ennemy.PatrolItinirary` (`self.As BP Ennemy`)) (`Actor.K2_GetActorLocation` _array_element)))
    (`self.FinishExecute` true)
    (else
      (`self.FinishExecute` true))))