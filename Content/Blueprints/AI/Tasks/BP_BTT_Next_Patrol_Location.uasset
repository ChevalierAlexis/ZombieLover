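; Behavior tree task that advances a BP_Ennemy to its next patrol point.
; It steps PatrolIndex through PatrolItinirary, either resetting to zero in Loop mode or ping-ponging via PatrolDirection and the PatrolReverse flag.
; The selected point is stored as GuardLocation on the enemy and blackboard.
; Bounds checks trigger only at -1 or array length, so the lookup can use an out-of-range index.
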(event `self.ReceiveExecuteAI`
  (params (OwnerController :type "AIController Object Reference") (ControlledPawn :type "Pawn Object Reference"))
  (bind _ennemyref (`self.EnnemyRef`))
  (bind _ennemyref_2 (`self.EnnemyRef`))
  (bind _ennemyref_3 (`self.EnnemyRef`))
  (bind _asbp_ennemy (cast `/Game/Blueprints/Characters/BP_Ennemy` ControlledPawn))
  (bind _output_get (set `self.EnnemyRef` _asbp_ennemy))
  (bind _output_get_2 (set `self.Patrol` (`/Game/Blueprints/Characters/BP_Ennemy.Patrol` _output_get)))
  (if (`/Game/Blueprints/AI/BP_Patrol.Loop` _output_get_2)
    (if (== (`/Game/Blueprints/Characters/BP_Ennemy.PatrolIndex` _ennemyref) (`KismetArrayLibrary.Array_Length` (`/Game/Blueprints/Characters/BP_Ennemy.PatrolItinirary` _ennemyref)))
      (bind _output_get_3 (set `/Game/Blueprints/Characters/BP_Ennemy.PatrolIndex` 0 _ennemyref_2))
      (bind _output_get_4 (set `/Game/Blueprints/Characters/BP_Ennemy.GuardLocation` (`|GetArrayItem` (`/Game/Blueprints/Characters/BP_Ennemy.PatrolItinirary` _ennemyref_2) _output_get_3) (`self.EnnemyRef`)))
      (`BTFunctionLibrary.SetBlackboardValueAsVector` (make `BlackboardKeySelector` _ "GuardLocation" "/Script/AIModule.BlackboardKeyType_Vector") _output_get_4)
      (else
        (bind _output_get_5 (set `/Game/Blueprints/Characters/BP_Ennemy.PatrolIndex` (+ (`/Game/Blueprints/Characters/BP_Ennemy.PatrolIndex` (`self.EnnemyRef`)) 1) _ennemyref_3))
        (bind _output_get_6 (set `/Game/Blueprints/Characters/BP_Ennemy.GuardLocation` (`|GetArrayItem` (`/Game/Blueprints/Characters/BP_Ennemy.PatrolItinirary` _ennemyref_3) _output_get_5) (`self.EnnemyRef`)))
        (`BTFunctionLibrary.SetBlackboardValueAsVector` (make `BlackboardKeySelector` _ "GuardLocation" "/Script/AIModule.BlackboardKeyType_Vector") _output_get_6)))
    (else
      (`self.PatrolDirection`)))
  (`self.FinishExecute` true))

(fn `PatrolDirection`
  (if (`/Game/Blueprints/Characters/BP_Ennemy.PatrolReverse` (`self.EnnemyRef`))
    (bind _output_get (set `/Game/Blueprints/Characters/BP_Ennemy.PatrolIndex` (- (`/Game/Blueprints/Characters/BP_Ennemy.PatrolIndex` (`self.EnnemyRef`)) 1) (`self.EnnemyRef`)))
    (if (== _output_get -1)
      (set `/Game/Blueprints/Characters/BP_Ennemy.PatrolReverse` false (`self.EnnemyRef`)))
    (bind _output_get_2 (set `/Game/Blueprints/Characters/BP_Ennemy.GuardLocation` (`|GetArrayItem` (`/Game/Blueprints/Characters/BP_Ennemy.PatrolItinirary` (`self.EnnemyRef`)) _output_get) (`self.EnnemyRef`)))
    (`BTFunctionLibrary.SetBlackboardValueAsVector` (make `BlackboardKeySelector` _ "GuardLocation" "/Script/AIModule.BlackboardKeyType_Vector") _output_get_2)
    (else
      (bind _output_get_3 (set `/Game/Blueprints/Characters/BP_Ennemy.PatrolIndex` (+ (`/Game/Blueprints/Characters/BP_Ennemy.PatrolIndex` (`self.EnnemyRef`)) 1) (`self.EnnemyRef`)))
      (if (== _output_get_3 (`KismetArrayLibrary.Array_Length` (`/Game/Blueprints/Characters/BP_Ennemy.PatrolItinirary` (`self.EnnemyRef`))))
        (set `/Game/Blueprints/Characters/BP_Ennemy.PatrolReverse` true (`self.EnnemyRef`)))
      (bind _output_get_4 (set `/Game/Blueprints/Characters/BP_Ennemy.GuardLocation` (`|GetArrayItem` (`/Game/Blueprints/Characters/BP_Ennemy.PatrolItinirary` (`self.EnnemyRef`)) _output_get_3) (`self.EnnemyRef`)))
      (`BTFunctionLibrary.SetBlackboardValueAsVector` (make `BlackboardKeySelector` _ "GuardLocation" "/Script/AIModule.BlackboardKeyType_Vector") _output_get_4))))