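; Behavior tree task that feeds the next patrol point to an AI run by BP_AIC_Rage_Controller.
; On execute it casts the owning controller and writes the location of the current Patrol point actor into the GuardLocation blackboard key.
; It then increments its own PatrolIndex, with no wrap or bounds check, and finishes successfully.
; A failed cast never calls FinishExecute, and a debug print is left disconnected.
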(event `self.ReceiveExecuteAI`
  (params (OwnerController :type "AIController Object Reference") (ControlledPawn :type "Pawn Object Reference"))
  (bind _asaic_rage_controller (cast `/Game/Blueprints/AI/BP_AIC_Rage_Controller` OwnerController))
  (`BlackboardComponent.SetValueAsVector` (`/Game/Blueprints/AI/BP_AIC_Rage_Controller.Blackboard1` _asaic_rage_controller) "GuardLocation" (`Actor.K2_GetActorLocation` (`|GetArrayItem` (`/Game/Blueprints/AI/BP_Patrol.PatrolPoints` (`/Game/Blueprints/AI/BP_AIC_Rage_Controller.Patrol` _asaic_rage_controller)) (`self.PatrolIndex`))))
  (set `self.PatrolIndex` (+ (`self.PatrolIndex`) 1))
  (`self.FinishExecute` true))