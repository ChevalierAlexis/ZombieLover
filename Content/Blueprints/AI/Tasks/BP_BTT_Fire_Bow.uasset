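; Behavior tree task that makes a bowman AI fire an arrow projectile at the nearest enemy.
; It finds the closest BP_Ennemy to the pawn's flipbook and stores it as the bowman's Target.
; It spawns BP_Projectile slightly above the sprite, with speed scaled by distance to that enemy and Velocity read from the Blackboard.
; The task then finishes successfully; a look-at rotation node is left unconnected.
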(event `self.ReceiveExecuteAI`
  (params (OwnerController :type "AIController Object Reference") (ControlledPawn :type "Pawn Object Reference"))
  (bind _returnvalue (`SceneComponent.K2_GetComponentLocation` (`Actor.GetComponentByClass` ControlledPawn "/Script/Paper2D.PaperFlipbookComponent")))
  (bind _asbp_bowman (cast `/Game/Blueprints/Characters/BP_Bowman` ControlledPawn))
  (bind _outactors (`GameplayStatics.GetAllActorsOfClass` "/Game/Blueprints/Characters/BP_Ennemy.BP_Ennemy_C"))
  (bind (_distance _returnvalue_2) (`GameplayStatics.FindNearestActor` _returnvalue _outactors))
  (set `/Game/Blueprints/Characters/BP_Bowman.Target` _returnvalue_2 _asbp_bowman)
  (`|SpawnActorFromClass` "/Game/Blueprints/Objects/BP_Projectile.BP_Projectile_C" (`KismetMathLibrary.MakeTransform` (+ _returnvalue (0.0 0.0 50.0))) "Undefined" "MultiplyWithRoot" null (* _distance 1.5) (`BTFunctionLibrary.GetBlackboardValueAsVector` (make `BlackboardKeySelector` _ "Velocity" "/Script/AIModule.BlackboardKeyType_Vector")) ControlledPawn)
  (`self.FinishExecute` true))