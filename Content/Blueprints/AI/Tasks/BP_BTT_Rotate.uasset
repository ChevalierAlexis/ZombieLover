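; Behavior tree task that gives an enemy pawn a yaw value relative to its blackboard Target location.
; On execute it takes the yaw of the vector from the Target to the pawn, so facing away from the Target, and writes it to RotateValue on BP_Ennemy.
; It finishes immediately with success and does not rotate the pawn itself.
; An unconnected branch on that yaw never runs.
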(event `self.ReceiveExecuteAI`
  (params (OwnerController :type "AIController Object Reference") (ControlledPawn :type "Pawn Object Reference"))
  (bind (_returnvalue_roll _returnvalue_pitch _returnvalue_yaw) (`KismetMathLibrary.BreakRotator` (`KismetMathLibrary.Conv_VectorToRotator` (- (`Actor.K2_GetActorLocation` ControlledPawn) (`BTFunctionLibrary.GetBlackboardValueAsVector` (`self.Target`))))))
  (set `self.Owner Controller` OwnerController)
  (set `self.Controlled Pawn` ControlledPawn)
  (bind _asbp_ennemy (cast `/Game/Blueprints/Characters/BP_Ennemy` (`self.Controlled Pawn`)))
  (set `/Game/Blueprints/Characters/BP_Ennemy.RotateValue` _returnvalue_yaw _asbp_ennemy)
  (`self.FinishExecute` true))