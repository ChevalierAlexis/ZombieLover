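; Behavior tree task that picks the nearest target for an AI enemy, branching on its controller type.
; For a Rage controller, it writes the nearest EnnemyTarget-class actor to the Player blackboard key and always succeeds.
; For a Bowman controller, it writes the nearest BP_Character_Base within Range to Player and that actor's location to GuardLocation, or fails if none is in range.
; Other controller types never reach FinishExecute.
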(event `self.ReceiveExecuteAI`
  (params (OwnerController :type "AIController Object Reference") (ControlledPawn :type "Pawn Object Reference"))
  (bind _asaic_rage_controller (cast `/Game/Blueprints/AI/BP_AIC_Rage_Controller` OwnerController)
    (:`then`
      (bind _outactors (`GameplayStatics.GetAllActorsOfClass` (`self.EnnemyTarget`)))
      (`BlackboardComponent.SetValueAsObject` (`/Game/Blueprints/AI/BP_AIC_Rage_Controller.Blackboard1` _asaic_rage_controller) "Player" (`.ReturnValue` (`GameplayStatics.FindNearestActor` (`Actor.K2_GetActorLocation` ControlledPawn) _outactors)))
      (`self.FinishExecute` true))
    (:`CastFailed`
      (bind _asaic_bowman_controller (cast `/Game/Blueprints/AI/BP_AIC_Bowman_Controller` OwnerController))
      (bind _outactors_2 (`GameplayStatics.GetAllActorsOfClass` "/Game/Blueprints/Characters/BP_Character_Base.BP_Character_Base_C"))
      (bind (_distance _returnvalue) (`GameplayStatics.FindNearestActor` (`Actor.K2_GetActorLocation` ControlledPawn) _outactors_2))
      (if (>= (`/Game/Blueprints/AI/BP_AIC_Bowman_Controller.Range` _asaic_bowman_controller) _distance)
        (bind _blackboard1 (`/Game/Blueprints/AI/BP_AIC_Bowman_Controller.Blackboard1` _asaic_bowman_controller))
        (`BlackboardComponent.SetValueAsObject` _blackboard1 "Player" _returnvalue)
        (`BlackboardComponent.SetValueAsVector` _blackboard1 "GuardLocation" (`Actor.K2_GetActorLocation` _returnvalue))
        (`self.FinishExecute` true)
        (else
          (`self.FinishExecute` false))))))