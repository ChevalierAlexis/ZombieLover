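; Behavior Tree attack task that either kills the blackboard target or triggers an enemy's attack animation.
; For a BP_Character_Base pawn, it plays the zombie-eat sound from DT_Sound_List, passes the target to BP_Kill_AC, clears Player and HasLineOfSight, then finishes.
; Other BP_Ennemy pawns just set IsAttacking on their PaperZD anim instance and finish.
; A Death event jumps straight into the kill-and-reset sequence, skipping the sound.
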(event `Death`
  (`/Game/Blueprints/Characters/Components/BP_Kill_AC.KillActor` (`Actor.GetComponentByClass` (stale `self.ReceiveExecuteAI` ControlledPawn) "/Game/Blueprints/Characters/Components/BP_Kill_AC.BP_Kill_AC_C") (`BTFunctionLibrary.GetBlackboardValueAsActor` (`self.Target`)) :!label _label)
  (bind _returnvalue (`Actor.GetComponentByClass` (stale `self.ReceiveExecuteAI` OwnerController) "/Script/AIModule.BlackboardComponent"))
  (`BlackboardComponent.SetValueAsObject` _returnvalue "Player" null)
  (`BlackboardComponent.SetValueAsBool` _returnvalue "HasLineOfSight" false)
  (`self.FinishExecute` true))

(event `self.ReceiveExecuteAI`
  (params (OwnerController :type "AIController Object Reference") (ControlledPawn :type "Pawn Object Reference"))
  (cast `/Game/Blueprints/Characters/BP_Character_Base` ControlledPawn
    (:`then`
      (bind _returnvalue (`|GetDataTableRow` "/Game/Sound/DT_Sound_List.DT_Sound_List" "A_Zombie_Eat")
        (:`then`
          (`GameplayStatics.PlaySound2D` (break `/Game/Blueprints/Structures/SSound` _returnvalue) 1.0 1.0 0.0 null null)
          (goto _label))))
    (:`CastFailed`
      (bind _asbp_ennemy (cast `/Game/Blueprints/Characters/BP_Ennemy` ControlledPawn))
      (bind _asabp_pzd_ennemies (cast `/Game/Animation/Ennemies/ABP_PZD_Ennemies` (`PaperZDAnimationComponent.AnimInstance` (`/Game/Blueprints/Characters/BP_Ennemy.PaperZDAnimation` _asbp_ennemy))))
      (set `/Game/Animation/Ennemies/ABP_PZD_Ennemies.IsAttacking` true _asabp_pzd_ennemies)
      (`self.FinishExecute` true))))