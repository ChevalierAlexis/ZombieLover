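; BP_BTT_GiveUp is a behavior tree task for enemy AI, apparently an unfinished give-up step.
; On execute it casts the owner to BP_AIC_Enemy_Controller and checks the HasLineOfSight blackboard key, but the branch leads to no action.
; Two nodes that set HasWaited to true or false are disconnected, and the task never calls Finish Execute.
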(event `self.ReceiveExecuteAI`
  (params (OwnerController :type "AIController Object Reference") (ControlledPawn :type "Pawn Object Reference"))
  (bind _asaic_enemy_controller (cast `/Game/Blueprints/AI/BP_AIC_Enemy_Controller` OwnerController))
  (bind _blackboard1 (`/Game/Blueprints/AI/BP_AIC_Enemy_Controller.Blackboard1` _asaic_enemy_controller))
  (set `self.Blackboard 1` _blackboard1)
  (if (`BlackboardComponent.GetValueAsBool` _blackboard1 "HasLineOfSight")
    _))