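; Behavior tree task that aims an AI pawn's projectile by finding a launch velocity that lands near the blackboard GuardLocation.
; It repeatedly simulates a debug-drawn shot from above the flipbook, nudging X and Y velocity in fixed steps toward that point.
; Within tolerance it writes Velocity to the blackboard and succeeds.
; The loop has no iteration cap and stalls unfinished if Y matches exactly; the fetched EnnemyTarget is unused.
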(event `self.ReceiveExecuteAI`
  (params (OwnerController :type "AIController Object Reference") (ControlledPawn :type "Pawn Object Reference"))
  (bind (_hitlocation_x _hitlocation_y) (`KismetMathLibrary.BreakVector` (`self.HitLocation`)))
  (bind _hitlocation_x_2 (`KismetMathLibrary.BreakVector` (`self.HitLocation`)))
  (bind (_hitlocation_x_3 _hitlocation_y_2) (`KismetMathLibrary.BreakVector` (`self.HitLocation`)))
  (bind _hitlocation_x_4 (`KismetMathLibrary.BreakVector` (`self.HitLocation`)))
  (bind (_returnvalue_x _returnvalue_y) (`KismetMathLibrary.BreakVector` (`BlackboardComponent.GetValueAsVector` (`Actor.GetComponentByClass` (`self.Owner Controller`) "/Script/AIModule.BlackboardComponent") "GuardLocation")))
  (bind _returnvalue_x_2 (`KismetMathLibrary.BreakVector` (`BlackboardComponent.GetValueAsVector` (`Actor.GetComponentByClass` (`self.Owner Controller`) "/Script/AIModule.BlackboardComponent") "GuardLocation")))
  (bind (_returnvalue_x_3 _returnvalue_y_2) (`KismetMathLibrary.BreakVector` (`BlackboardComponent.GetValueAsVector` (`Actor.GetComponentByClass` (`self.Owner Controller`) "/Script/AIModule.BlackboardComponent") "GuardLocation")))
  (bind _returnvalue_x_4 (`KismetMathLibrary.BreakVector` (`BlackboardComponent.GetValueAsVector` (`Actor.GetComponentByClass` (`self.Owner Controller`) "/Script/AIModule.BlackboardComponent") "GuardLocation")))
  ;[1 1 1] Acquisition de l'ennemi
  (set `self.Owner Controller` OwnerController)
  (set `self.Target` (`BTFunctionLibrary.GetBlackboardValueAsActor` (`self.EnnemyTarget`)))
  ;[1 1 1] Tant que l'estimation n'est pas sur la cible, relancer une simulation
  (`KismetSystemLibrary.PrintString` "Target")
  (if (== (`self.HitLocation`) (`BlackboardComponent.GetValueAsVector` (`Actor.GetComponentByClass` (`self.Owner Controller`) "/Script/AIModule.BlackboardComponent") "GuardLocation") :`ErrorTolerance` 75.0) :!label _label
    (`BTFunctionLibrary.SetBlackboardValueAsVector` (make `BlackboardKeySelector` _ "Velocity" "/Script/AIModule.BlackboardKeyType_Vector") (`self.Velocity`))
    (`KismetSystemLibrary.PrintString` "gotcha bitch")
    (`self.FinishExecute` true)
    (else
      ;[1 1 1] Simule le tir d'estimation
      (bind _predictresult (`GameplayStatics.Blueprint_PredictProjectilePath_Advanced` (make `PredictProjectilePathParams` (+ (`SceneComponent.K2_GetComponentLocation` (`Actor.GetComponentByClass` ControlledPawn "/Script/Paper2D.PaperFlipbookComponent")) (0.0 0.0 50.0)) (`self.Velocity`) true 22.0 3.0 true "ECC_WorldStatic" _ (`|MakeArray` ControlledPawn :!type "Actor Object Reference") 100.0 0.0 "ForDuration" 1.0 true)))
      (set `self.HitLocation` (`.Location` (`GameplayStatics.BreakHitResult` (`.HitResult` (break `PredictProjectilePathResult` _predictresult)))))
      (`KismetSystemLibrary.PrintString` "Iteration")
      ;[1 1 1] Ajuste la vélocité des tirs selon si le tir trop proche ou trop loin
      (if (< _returnvalue_x_4 _hitlocation_x_2)
        (set `self.Velocity` (- (`self.Velocity`) (50.0 0.0 0.0)))
        (elif (> _returnvalue_x_2 _hitlocation_x_4)
          (set `self.Velocity` (+ (`self.Velocity`) (50.0 0.0 0.0)))))
      (if (< _returnvalue_y _hitlocation_y)
        (set `self.Velocity` (- (`self.Velocity`) (0.0 50.0 0.0)))
        (goto _label)
        (elif (> _returnvalue_y_2 _hitlocation_y_2)
          (set `self.Velocity` (+ (`self.Velocity`) (0.0 50.0 0.0)))
          (goto _label))))))