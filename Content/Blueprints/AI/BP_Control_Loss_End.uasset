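; Trigger volume that ends a control-loss section by handing the first overlapping BP_Character_Top to the Zombie Player Controller.
; It unpossesses the character's current controller, removes its "Booyah" tag and has the zombie controller possess it.
; If the character has a BPC_Kill component, it destroys it, prints a debug result and binds the controller's OnSeparation event.
; The construction script sizes the trigger box from BoxSize.
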(event `self.Box.OnComponentBeginOverlap`
  (params (OverlappedComponent :type "PrimitiveComponent Object Reference") (OtherActor :type "Actor Object Reference") (OtherComp :type "PrimitiveComponent Object Reference") (OtherBodyIndex :type Integer) (bFromSweep :type Boolean) (SweepResult :type "HitResult Structure (by ref)"))
  (bind _character_top (`self.Character_Top`))
  (bind _returnvalue (`self.GetComponentByClass` _character_top "/Game/Blueprints/Characters/Components/BPC_Kill.BPC_Kill_C"))
  (bind _asbp_character_top (cast `/Game/Blueprints/Characters/BP_Character_Top` OtherActor))
  (set `self.Character_Top` _asbp_character_top)
  (`/Engine/EditorBlueprintResources/StandardMacros.DoOnce` false
    (:`Completed`
      (`Controller.UnPossess` (`Pawn.GetController` (`self.Character_Top`)))
      (`KismetArrayLibrary.Array_RemoveItem` (`Actor.Tags` (`self.Character_Top`)) "Booyah")
      (`Controller.Possess` (`/Game/Blueprints/Library/BPFL_Fonction_Library.GetZombiePlayerController`) _character_top)
      (`/Engine/EditorBlueprintResources/StandardMacros.IsValid` _returnvalue
        (:`Is Valid`
          (`ActorComponent.K2_DestroyComponent` _returnvalue)
          (`/Engine/EditorBlueprintResources/StandardMacros.IsValid` (`self.GetComponentByClass` (`self.Character_Top`) "/Game/Blueprints/Characters/Components/BPC_Kill.BPC_Kill_C")
            (:`Is Valid`
              (`KismetSystemLibrary.PrintString` "Fail$"))
            (:`Is Not Valid`
              (`KismetSystemLibrary.PrintString` "Success")))
          (add `/Game/Blueprints/Controllers/BP_Player_Controller.OnSeparation` (`/Game/Blueprints/Library/BPFL_Fonction_Library.GetZombiePlayerController`) (`|CreateDelegate` (`/Game/Blueprints/Library/BPFL_Fonction_Library.GetZombiePlayerController`) :!event `OnSeparationEvent`)))))))

(fn `UserConstructionScript`
  (`BoxComponent.SetBoxExtent` (`self.Box`) (`self.BoxSize`) true))