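; AI controller for enemies that sets up their guard or patrol mode.
; On BeginPlay it writes the IsGuarding blackboard key as the inverse of the IsPatroling flag.
; It then checks the first PatrolItinirary point against the zero vector, printing French warnings when patrol lacks a route or a route is set with patrol disabled.
; Tick and the construction script hold no logic.
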(event `self.ReceiveBeginPlay`
  (`BlackboardComponent.SetValueAsBool` (`self.Blackboard`) (`self.IsGuarding`) (not (`self.IsPatroling`)))
  (if (`self.IsPatroling`)
    (if (== (`|GetArrayItem` (`self.PatrolItinirary`)) (0.0 0.0 0.0))
      (`KismetSystemLibrary.PrintString` "Pas d'itinéraire défini dans \"PatrolItinirary\""))
    (elif (!= (`|GetArrayItem` (`self.PatrolItinirary`)) (0.0 0.0 0.0))
      (`KismetSystemLibrary.PrintString` "Un itinéraire est défini mais le mode patrouille n'est pas activé. Pour ce faire, mettez \"IsPatroling\" sur True."))))

(fn `UserConstructionScript`)