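; AI controller for the Bowman that starts its behavior tree on BeginPlay and feeds it perception results.
; Target perception updates write a sensed BP_Character_Base to the Player blackboard key and sensing success to HasLineOfSight, while other actors clear Player.
; General perception updates rebuild a ValidPlayers array, but its nearest-actor lookup is unused.
; Tick reads HasLineOfSight without acting on it.
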(event `self.ReceiveBeginPlay`
  (`self.RunBehaviorTree` "/Game/Blueprints/AI/BT_Bowman_Behaviour_Tree.BT_Bowman_Behaviour_Tree"))

(event `self.ReceiveTick`
  (params (DeltaSeconds :type "Float (single-precision)"))
  (if (`BlackboardComponent.GetValueAsBool` (`self.Blackboard1`) "HasLineOfSight")
    _))

(event `self.AIPerception.OnTargetPerceptionUpdated`
  (params (Actor :type "Actor Object Reference") (Stimulus :type "AIStimulus Structure"))
  (cast `/Game/Blueprints/Characters/BP_Character_Base` Actor
    (:`then`
      (`BlackboardComponent.SetValueAsObject` (`self.Blackboard1`) "Player" Actor)
      (`BlackboardComponent.SetValueAsBool` (`self.Blackboard1`) "HasLineOfSight" (`.bSuccessfullySensed` (break `AIStimulus` Stimulus))))
    (:`CastFailed`
      (`BlackboardComponent.SetValueAsObject` (`self.Blackboard1`) "Player" null))))

(event `self.AIPerception.OnPerceptionUpdated`
  (params (UpdatedActors :type "Array of Actor Object Reference (by ref)"))
  (`KismetArrayLibrary.Array_Clear` (`self.ValidPlayers`))
  (for _array_element UpdatedActors
    (bind _asbp_character_base (cast `/Game/Blueprints/Characters/BP_Character_Base` _array_element))
    (`KismetArrayLibrary.Array_Add` (`self.ValidPlayers`) _asbp_character_base)))

(fn `UserConstructionScript`)