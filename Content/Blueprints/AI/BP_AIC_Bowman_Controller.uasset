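; AI controller for the Bowman enemy that runs its behavior tree and feeds player perception into the blackboard.
; Target perception updates set Player and HasLineOfSight for whichever actor triggered them; the nearest-actor check there has no effect.
; General perception updates rebuild the player list, clearing sight if the nearest is invisible or too far above the Bowman.
; While sight holds, Tick writes the nearest listed player's distance.
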(event `self.ReceiveBeginPlay`
  (`self.RunBehaviorTree` "/Game/Blueprints/AI/BT_Bowman_Behaviour_Tree.BT_Bowman_Behaviour_Tree"))

(event `self.AIPerception.OnPerceptionUpdated`
  (params (UpdatedActors :type "Array of Actor Object Reference (by ref)"))
  (bind (_returnvalue_x _returnvalue_y _returnvalue_z) (`KismetMathLibrary.BreakVector` (`self.K2_GetActorLocation` (`self.K2_GetPawn`))))
  (`KismetArrayLibrary.Array_Clear` (`self.ValidPlayers`))
  (for _array_element UpdatedActors
    (bind _asbp_character_base (cast `/Game/Blueprints/Characters/BP_Character_Base` _array_element))
    (`KismetArrayLibrary.Array_Add` (`self.ValidPlayers`) _asbp_character_base))
  (bind _asbp_character_base_2 (cast `/Game/Blueprints/Characters/BP_Character_Base` (`.ReturnValue` (`GameplayStatics.FindNearestActor` (`self.K2_GetActorLocation` (`self.K2_GetPawn`)) (`self.ValidPlayers`)))))
  ;[1 1 1] Si le joueur est caché, vider les variables permettant de le repérer
  (if (`/Game/Blueprints/Characters/BP_Character_Base.IsInvisible` _asbp_character_base_2)
    (`self.ClearBowmanVision`)
    (else
      (bind (_returnvalue_x_2 _returnvalue_y_2 _returnvalue_z_2) (`KismetMathLibrary.BreakVector` (`self.K2_GetActorLocation` _asbp_character_base_2)))
      ;[1 1 1] Cache le joueur si celui-ci est trop haut par rapport à l'ennemi
      (if (not (<= (- _returnvalue_z_2 _returnvalue_z) 50.0))
        (`self.ClearBowmanVision`)))))

(event `self.ReceiveTick`
  (params (DeltaSeconds :type "Float (single-precision)"))
  ;[1 1 1] Met A jour la distance entre l'ennemi et le joueur
  (if (`BlackboardComponent.GetValueAsBool` (`self.Blackboard1`) "HasLineOfSight")
    (`BlackboardComponent.SetValueAsFloat` (`self.Blackboard1`) "Distance" (`GameplayStatics.FindNearestActor` (`self.K2_GetActorLocation` (`self.K2_GetPawn`)) (`self.ValidPlayers`)))))

(event `self.AIPerception.OnTargetPerceptionUpdated`
  (params (Actor :type "Actor Object Reference") (Stimulus :type "AIStimulus Structure"))
  (if (== (`.ReturnValue` (`GameplayStatics.FindNearestActor` (`self.K2_GetActorLocation` (`self.K2_GetPawn`)) (`self.ValidPlayers`))) Actor)
    _
    (else
      _))
  (`BlackboardComponent.SetValueAsObject` (`self.Blackboard1`) "Player" Actor)
  (`BlackboardComponent.SetValueAsBool` (`self.Blackboard1`) "HasLineOfSight" (`.bSuccessfullySensed` (break `AIStimulus` Stimulus))))

(fn `ClearBowmanVision`
  (`BlackboardComponent.SetValueAsBool` (`self.Blackboard1`) "HasLineOfSight" false)
  (`BlackboardComponent.SetValueAsObject` (`self.Blackboard1`) "Player" null))

(fn `UserConstructionScript`)