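; AI controller for enemies that runs the enemy behavior tree and feeds it player sighting data through the blackboard.
; Perception updates collect player characters and write the sensed target and line of sight.
; Vision is cleared when the blackboard player is invisible, with a further check meant for players too high above the enemy.
; Successful or lost sensing rebinds a tick dispatcher, and a SetDistance event writes nearest-player distance.
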(event OnPerceptionUpdated(AIPerception)
  (params (UpdatedActors :type Array%20of%20Actor%20Object%20References))
  (Utilities|Array|Clear (Variables|Default|GetValidPlayers))
  (for _array_element UpdatedActors
    (bind _asbp_character_base (Utilities|Casting|CastToBP_Character_Base _array_element))
    (Utilities|Array|Add (Variables|Default|GetValidPlayers) _asbp_character_base))
  (Utilities|IsValid (Pawn|GetControlledPawn)
    (:Is%20Valid
      (bind _asbp_character_base_2 (Utilities|Casting|CastToBP_Character_Base (AI|Components|Blackboard|GetValueasObject (Variables|Default|GetBlackboard1) (Utilities|Name|MakeLiteralName "Player"))))
      (if (Variables|/Game/Blueprints/Characters/BP_Character_Base.BP_Character_Base_C|GetIsInvisible _asbp_character_base_2)
        (AI|Components|Blackboard|SetValueasBool (Variables|Default|GetBlackboard1) (Utilities|Name|MakeLiteralName "HasLineOfSight") false)
        (AI|Components|Blackboard|SetValueasObject (Variables|Default|GetBlackboard1) (Utilities|Name|MakeLiteralName "Player") 0)
        (else
          ;[1 1 1] Cache le joueur si celui-ci est trop haut par rapport à l'ennemi
          (if (not (<= (- (.z (Transformation|GetActorLocation (stale _asbp_character_base))) (.z (Transformation|GetActorLocation (Pawn|GetControlledPawn)))) 5e+01))
            (CallFunction|ClearVision)))))))

(event OnTargetPerceptionUpdated(AIPerception)
  (params (Actor :type Actor%20Object%20Reference) (Stimulus :type AI%20Stimulus%20Structure))
  (bind _bsuccessfullysensed (Utilities|Struct|BreakAIStimulus Stimulus))
  (Utilities|IsValid (Pawn|GetControlledPawn)
    (:Is%20Valid
      (if (== (.ReturnValue (Actor|FindNearestActor (Transformation|GetActorLocation (Pawn|GetControlledPawn)) (Variables|Default|GetValidPlayers))) Actor)
        _
        (else
          _))
      (AI|Components|Blackboard|SetValueasObject (Variables|Default|GetBlackboard1) (Utilities|Name|MakeLiteralName "Player") Actor)
      (AI|Components|Blackboard|SetValueasBool (Variables|Default|GetBlackboard1) (Utilities|Name|MakeLiteralName "HasLineOfSight") _bsuccessfullysensed)
      (if _bsuccessfullysensed
        (EventDispatchers|BindEventtoOnTick (EventDispatchers|CreateEvent :!event Custom|SetDistance))
        (else
          (EventDispatchers|BindEventtoOnTick (EventDispatchers|CreateEvent :!event Custom|SetDistance)))))))

(event Custom|SetDistance
  (AI|Components|Blackboard|SetValueasFloat (Variables|Default|GetBlackboard1) (Utilities|Name|MakeLiteralName "Distance") (.Distance (Actor|FindNearestActor (Transformation|GetActorLocation (Pawn|GetControlledPawn)) (Variables|Default|GetValidPlayers)))))

(event EventBeginPlay
  (AI|RunBehaviorTree "/Game/Blueprints/AI/BT_Enemy_Behaviour_Tree.BT_Enemy_Behaviour_Tree")
  (bind _asbp_ennemy (Utilities|Casting|CastToBP_Ennemy (Pawn|GetControlledPawn))))

(event EventTick
  (params (DeltaSeconds :type Float%20%28single-precision%29))
  (Default|CallOnTick))

(fn ConstructionScript)

(fn ClearVision
  (AI|Components|Blackboard|SetValueasBool (Variables|Default|GetBlackboard1) (Utilities|Name|MakeLiteralName "HasLineOfSight") false)
  (AI|Components|Blackboard|SetValueasObject (Variables|Default|GetBlackboard1) (Utilities|Name|MakeLiteralName "Player") 0))