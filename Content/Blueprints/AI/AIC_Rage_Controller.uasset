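; AI controller for the Rage enemy that runs its behavior tree and feeds it player sighting data through the blackboard.
; Perception updates set the target player and line of sight, treating invisible characters as lost and ignoring those more than 50 units above the pawn.
; While line of sight holds, Tick writes the 2D distance to the player.
; An unconnected closest-player search is left unused.
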(event `self.ReceiveBeginPlay`
  (`self.RunBehaviorTree` "/Game/Blueprints/AI/BT_Rage_Behaviour_Tree.BT_Rage_Behaviour_Tree"))

(event `self.AIPerception.OnTargetPerceptionUpdated`
  (params (Actor :type "Actor Object Reference") (Stimulus :type "AIStimulus Structure"))
  (bind _blackboard1 (`self.Blackboard1`))
  (bind (_returnvalue_x _returnvalue_y _returnvalue_z) (`KismetMathLibrary.BreakVector` (`self.K2_GetActorLocation` (`self.K2_GetPawn`))))
  (bind _asbp_character_base (cast `/Game/Blueprints/Characters/BP_Character_Base` Actor))
  (if (`/Game/Blueprints/Characters/BP_Character_Base.IsInvisible` _asbp_character_base)
    (`BlackboardComponent.SetValueAsBool` (`self.Blackboard1`) "HasLineOfSight" false)
    (`BlackboardComponent.SetValueAsObject` (`self.Blackboard1`) "Player" null)
    (else
      (bind (_returnvalue_x_2 _returnvalue_y_2 _returnvalue_z_2) (`KismetMathLibrary.BreakVector` (`self.K2_GetActorLocation` _asbp_character_base)))
      (if (<= (- _returnvalue_z_2 _returnvalue_z) 50.0)
        (`BlackboardComponent.SetValueAsObject` _blackboard1 "Player" _asbp_character_base)
        (`BlackboardComponent.SetValueAsBool` _blackboard1 "HasLineOfSight" (`.bSuccessfullySensed` (break `AIStimulus` Stimulus)))
        (else
          (`BlackboardComponent.SetValueAsBool` (`self.Blackboard1`) "HasLineOfSight" false))))))

(event `self.ReceiveTick`
  (params (DeltaSeconds :type "Float (single-precision)"))
  (if (`BlackboardComponent.GetValueAsBool` (`self.Blackboard1`) "HasLineOfSight")
    (bind _asbp_character_base (cast `/Game/Blueprints/Characters/BP_Character_Base` (`BlackboardComponent.GetValueAsObject` (`self.Blackboard1`) "Player")))
    (`BlackboardComponent.SetValueAsFloat` (`self.Blackboard1`) "Distance" (`KismetMathLibrary.Vector_Distance2D` (`self.K2_GetActorLocation` _asbp_character_base) (`self.K2_GetActorLocation` (`self.K2_GetPawn`))))))

(fn `UserConstructionScript`)