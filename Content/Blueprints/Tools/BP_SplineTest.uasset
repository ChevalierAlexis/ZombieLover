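; BP_SplineTest is a test tool actor that lays a repeating mesh with pillars along an editable spline.
; The construction script splits the spline by MeshXLength, adding an X-forward spline mesh per segment and a Pillar static mesh at each segment start.
; Segment tangents are clamped to the mesh length.
; It also prints the root component's child count, and the event graph holds no active logic.
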(fn `UserConstructionScript`
  (bind _spline (`self.Spline`))
  (`KismetSystemLibrary.PrintString` (`KismetStringLibrary.Conv_IntToString` (`KismetArrayLibrary.Array_Length` (`SceneComponent.GetChildrenComponents` (`self.DefaultSceneRoot`) false))))
  (for _index (range (+ (`KismetMathLibrary.FTrunc` (/ (`SplineComponent.GetSplineLength` (`self.Spline`)) (`self.Mesh X Length`))) 1))
    ;[1 1 1] Adding Mesh
    (bind _returnvalue (`AddComponent|NODE_AddSplineMeshComponent-0`))
    (`StaticMeshComponent.SetStaticMesh` _returnvalue (`self.Mesh`))
    (`SplineMeshComponent.SetForwardAxis` _returnvalue "X" true)
    (bind _returnvalue_2 (`KismetMathLibrary.Conv_IntToDouble` _index))
    (bind _returnvalue_3 (* _returnvalue_2 (`self.Mesh X Length`)))
    (bind _returnvalue_4 (* (+ (`KismetMathLibrary.Conv_IntToDouble` _index) 1.0) (`self.Mesh X Length`)))
    (`SplineMeshComponent.SetStartAndEnd` _returnvalue (`SplineComponent.GetLocationAtDistanceAlongSpline` _spline _returnvalue_3 "Local") (`KismetMathLibrary.ClampVectorSize` (`SplineComponent.GetTangentAtDistanceAlongSpline` _spline _returnvalue_3 "Local") 0.0 (`self.Mesh X Length`)) (`SplineComponent.GetLocationAtDistanceAlongSpline` _spline _returnvalue_4 "Local") (`KismetMathLibrary.ClampVectorSize` (`SplineComponent.GetTangentAtDistanceAlongSpline` _spline _returnvalue_4 "Local") 0.0 (`self.Mesh X Length`)) true)
    (bind _returnvalue_5 (`AddComponent|NODE_AddStaticMeshComponent-0` :`RelativeTransform` (`SplineComponent.GetTransformAtDistanceAlongSpline` (`self.Spline`) (* _returnvalue_2 (`self.Mesh X Length`)) "Local" false)))
    (`StaticMeshComponent.SetStaticMesh` _returnvalue_5 (`self.Pillar`))))