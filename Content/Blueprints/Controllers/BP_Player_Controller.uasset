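; Player controller that turns Enhanced Input into character movement, jumping, interaction, separation, camera tilt, pause and respawn.
; Input actions fire event dispatchers, mostly bound on BeginPlay to handlers that drive the controlled character and camera manager UI.
; Rebinding dispatchers switches front movement to ladder climbing and disables jumping while BP_Character_Full grabs an object.
; Jumps honor coyote time and buffering, falling back to separation; temporary keys load prototype levels.
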(event `self.ReceiveBeginPlay`
  (bind _returnvalue (pcsubsystem `EnhancedInputLocalPlayerSubsystem` self))
  ;[1 1 1] Bind Event
  (`|ExecutionSequence`
    (:`then_0`
      (add `self.OnInteraction` (`|CreateDelegate` :!event `OnInteractionEvent`))
      (add `self.OnInteractionStop` (`|CreateDelegate` :!event `OnInteractioStopEvent`))
      (add `self.OnSeparation` (`|CreateDelegate` :!event `OnSeparationEvent`))
      (add `self.OnJump` (`|CreateDelegate` :!event `OnJumpEvent`))
      (add `self.OnStopJump` (`|CreateDelegate` :!event `OnStopJumpEvent`))
      (add `self.OnMoveRight` (`|CreateDelegate` :!event `MoveRightEvent`))
      (add `self.OnMoveFront` (`|CreateDelegate` :!event `MoveFrontEvent`))
      (add `self.OnPopUpInteract` (`|CreateDelegate` :!event `OnPopUpInteractEvent`))
      (add `self.OnCamTiltRight` (`|CreateDelegate` :!event `OnCamTiltRightEvent`))
      (add `self.OnCamTiltReset` (`|CreateDelegate` :!event `OnCamTiltResetEvent`))
      (add `self.OnPause` (`|CreateDelegate` :!event `OnPauseEvent`))
      (add `self.OnInteraction` (`|CreateDelegate` :!event `OnGrabEvent`)))
    (:`then_1`
      ;[1 1 1] Ajoute les contrôles
      (`/Engine/EditorBlueprintResources/StandardMacros.IsValid` _returnvalue
        (:`Is Valid`
          (`EnhancedInputSubsystemInterface.AddMappingContext` _returnvalue "/Game/Inputs/IMC_Mapping_Context.IMC_Mapping_Context" 0 (struct)))))))

(event `Key|U`
  (params (Key :type "Key Structure"))
  ;[1 1 1] prototype (temporaire)
  (:`Pressed`
    (`GameplayStatics.OpenLevelBySoftObjectPtr` "/Game/Levels/L_Proto.L_Proto")))

(event `EnhancedInput|/Game/Inputs/InputActions/IA_Move_Front`
  (params (ActionValue :type "Float (double-precision)") (ElapsedSeconds :type "Float (double-precision)") (TriggeredSeconds :type "Float (double-precision)") (InputAction :type "InputAction Object Reference" :default "/Game/Inputs/InputActions/IA_Move_Front.IA_Move_Front"))
  ;[1 1 1] Enhanced Inputs + event dispatchers
  (:`Triggered`
    (`self.OnMoveFront`)))

(event `OnInteractionEvent`
  ;[1 1 1] Events
  (if (`/Game/Blueprints/Library/BPFL_Fonction_Library.Is Current Player Alive` null)
    (`/Game/Blueprints/Characters/BP_Character_Base.Interact` (`/Game/Blueprints/Library/BPFL_Fonction_Library.CastToPlayerCharacter`))))

(event `OnInteractioStopEvent`
  ;[1 1 1] Events
  (if (`/Game/Blueprints/Library/BPFL_Fonction_Library.Is Current Player Alive` null)
    (`/Game/Blueprints/Characters/BP_Character_Base.StopInteract` (`/Game/Blueprints/Library/BPFL_Fonction_Library.CastToPlayerCharacter`))))

(event `OnSeparationEvent`
  ;[1 1 1] Events
  (if (`/Game/Blueprints/Library/BPFL_Fonction_Library.Is Current Player Alive` null)
    (`/Game/Blueprints/Characters/BP_Character_Base.Separate` (`/Game/Blueprints/Library/BPFL_Fonction_Library.CastToPlayerCharacter`))))

(event `MoveRightEvent`
  (bind _asbp_character_base0 (`/Game/Blueprints/Library/BPFL_Fonction_Library.CastToPlayerCharacter`))
  (bind _asbp_character_base0_2 (`/Game/Blueprints/Library/BPFL_Fonction_Library.CastToPlayerCharacter`))
  (bind _returnvalue (`|GetInputActionValue`))
  ;[1 1 1] Events
  (if (and (`/Game/Blueprints/Library/BPFL_Fonction_Library.Is Current Player Alive` null) (or (not (`self.Ladder`)) (`/Game/Blueprints/Characters/BP_Character_Base.Grounded` (`/Game/Blueprints/Library/BPFL_Fonction_Library.CastToPlayerCharacter`))))
    (if (> _returnvalue 0.0)
      (set `/Game/Blueprints/Characters/BP_Character_Base.IsFacingRight` true _asbp_character_base0_2)
      (bind _asbp_character_full (cast `/Game/Blueprints/Characters/BP_Character_Full` _asbp_character_base0_2)
        (:`then`
          (`/Engine/EditorBlueprintResources/StandardMacros.IsValid` (`/Game/Blueprints/Characters/BP_Character_Full.GrabbedObject` _asbp_character_full)
            (:`Is Valid`
              _)
            (:`Is Not Valid`
              (`SceneComponent.K2_SetRelativeRotation` :`self` (`PaperCharacter.Sprite` _asbp_character_base0_2) :!label _label))))
        (:`CastFailed`
          (goto _label)))
      (`Pawn.AddMovementInput` (`/Game/Blueprints/Library/BPFL_Fonction_Library.CastToPlayerCharacter`) (1.0 0.0 0.0) (`|GetInputActionValue`) false :!label _label_2)
      (elif (< _returnvalue 0.0)
        (set `/Game/Blueprints/Characters/BP_Character_Base.IsFacingRight` false _asbp_character_base0)
        (bind _asbp_character_full_2 (cast `/Game/Blueprints/Characters/BP_Character_Full` _asbp_character_base0)
          (:`then`
            (`/Engine/EditorBlueprintResources/StandardMacros.IsValid` (`/Game/Blueprints/Characters/BP_Character_Full.GrabbedObject` _asbp_character_full_2)
              (:`Is Valid`
                (goto _label_2))
              (:`Is Not Valid`
                _)))
          (:`CastFailed`
            _))
        (`SceneComponent.K2_SetRelativeRotation` (`PaperCharacter.Sprite` _asbp_character_base0) (struct :`Yaw` 180.0) false false)
        (goto _label_2)))))

(event `EnhancedInput|/Game/Inputs/InputActions/IA_Move_Right`
  (params (ActionValue :type "Float (double-precision)") (ElapsedSeconds :type "Float (double-precision)") (TriggeredSeconds :type "Float (double-precision)") (InputAction :type "InputAction Object Reference" :default "/Game/Inputs/InputActions/IA_Move_Right.IA_Move_Right"))
  ;[1 1 1] Enhanced Inputs + event dispatchers
  (:`Triggered`
    (`self.OnMoveRight`)))

(event `Key|I`
  (params (Key :type "Key Structure"))
  ;[1 1 1] prototype (temporaire)
  (:`Pressed`
    (`GameplayStatics.OpenLevelBySoftObjectPtr` "/Game/Levels/L_Diorama.L_Diorama")))

(event `OnPauseEvent`
  ;[1 1 1] Events
  (bind (_asbp_camera_manager _pawntarget _checkpoint _uideathref _uicontrol _uipause) (`/Game/Blueprints/Library/BPFL_Fonction_Library.GetCameraManager`))
  (if (`/Game/Blueprints/UI/WBP_UI_Pause.IsOnMainMenu` _uipause)
    (`/Game/Blueprints/CameraManager/BP_Camera_Manager.PopPauseMenu` _asbp_camera_manager)
    (else
      (`/Game/Blueprints/UI/WBP_UI_Pause.Echap` _uipause))))

(event `EnhancedInput|/Game/Inputs/InputActions/IA_Interaction`
  (params (ActionValue :type Boolean) (ElapsedSeconds :type "Float (double-precision)") (TriggeredSeconds :type "Float (double-precision)") (InputAction :type "InputAction Object Reference" :default "/Game/Inputs/InputActions/IA_Interaction.IA_Interaction"))
  ;[1 1 1] Enhanced Inputs + event dispatchers
  (:`Started`
    (`self.OnInteraction`))
  (:`Completed`
    (`self.OnInteractionStop`)))

(event `Key|O`
  (params (Key :type "Key Structure"))
  ;[1 1 1] prototype (temporaire)
  (:`Pressed`
    (`GameplayStatics.OpenLevelBySoftObjectPtr` "/Game/Levels/L_Diorama2.L_Diorama2")))

(event `Key|P`
  (params (Key :type "Key Structure"))
  ;[1 1 1] prototype (temporaire)
  (:`Pressed`
    (`GameplayStatics.OpenLevelBySoftObjectPtr` "/Game/Levels/L_Diorama01.L_Diorama01")))

(event `MoveFrontEvent`
  (bind _asbp_character_base0 (`/Game/Blueprints/Library/BPFL_Fonction_Library.CastToPlayerCharacter`))
  (bind _asbp_character_base0_2 (`/Game/Blueprints/Library/BPFL_Fonction_Library.CastToPlayerCharacter`))
  (bind _returnvalue (`|GetInputActionValue`))
  ;[1 1 1] Events
  (if (`/Game/Blueprints/Library/BPFL_Fonction_Library.Is Current Player Alive` null)
    (if (> _returnvalue 0.0)
      (set `/Game/Blueprints/Characters/BP_Character_Base.IsFacingFront` true _asbp_character_base0)
      (set `/Game/Blueprints/Characters/BP_Character_Base.IsMovingFront` true _asbp_character_base0 :!label _label_3)
      (`Pawn.AddMovementInput` _asbp_character_base0 (0.0 1.0 0.0) (`|GetInputActionValue`) false)
      (elif (< _returnvalue 0.0)
        (set `/Game/Blueprints/Characters/BP_Character_Base.IsFacingFront` false _asbp_character_base0_2)
        (goto _label_3)
        (else
          (set `/Game/Blueprints/Characters/BP_Character_Base.IsMovingFront` false _asbp_character_base0_2))))))

(event `EnhancedInput|/Game/Inputs/InputActions/IA_Separation`
  (params (ActionValue :type Boolean) (ElapsedSeconds :type "Float (double-precision)") (TriggeredSeconds :type "Float (double-precision)") (InputAction :type "InputAction Object Reference" :default "/Game/Inputs/InputActions/IA_Separation.IA_Separation"))
  ;[1 1 1] Enhanced Inputs + event dispatchers
  (:`Triggered`
    (`self.OnSeparation`)))

(event `OnJumpEvent`
  (bind _asbp_character_base0 (`/Game/Blueprints/Library/BPFL_Fonction_Library.CastToPlayerCharacter`))
  ;[1 1 1] Events
  (if (`/Game/Blueprints/Library/BPFL_Fonction_Library.Is Current Player Alive` null)
    (if (`NavMovementComponent.IsMovingOnGround` (`Character.CharacterMovement` _asbp_character_base0))
      (`/Game/Blueprints/Characters/BP_Character_Base.JumpSqueeze` _asbp_character_base0 :!label _label_4)
      (`Character.Jump` _asbp_character_base0)
      (elif (> (`KismetSystemLibrary.K2_GetTimerRemainingTimeHandle` (`/Game/Blueprints/Characters/BP_Character_Base.CoyoteTime` _asbp_character_base0)) 0.0)
        (goto _label_4)
        (else
          (`/Game/Blueprints/Characters/BP_Character_Base.BufferJump` _asbp_character_base0)
          (if (not (`/Game/Blueprints/Characters/BP_Character_Base.JumpBuffered` _asbp_character_base0))
            (bind _asbp_character_full (cast `/Game/Blueprints/Characters/BP_Character_Full` (`self.K2_GetPawn`)))
            (`/Game/Blueprints/Characters/BP_Character_Base.Separate` _asbp_character_full)))))))

(event `EnhancedInput|/Game/Inputs/InputActions/IA_Jump`
  (params (ActionValue :type Boolean) (ElapsedSeconds :type "Float (double-precision)") (TriggeredSeconds :type "Float (double-precision)") (InputAction :type "InputAction Object Reference" :default "/Game/Inputs/InputActions/IA_Jump.IA_Jump"))
  ;[1 1 1] Enhanced Inputs + event dispatchers
  (:`Triggered`
    (`self.OnJump`)))

(event `OnStopJumpEvent`
  ;[1 1 1] Events
  (`Character.StopJumping` (`/Game/Blueprints/Library/BPFL_Fonction_Library.CastToPlayerCharacter`)))

(event `EnhancedInput|/Game/Inputs/InputActions/IA_Jump_Stop`
  (params (ActionValue :type Boolean) (ElapsedSeconds :type "Float (double-precision)") (TriggeredSeconds :type "Float (double-precision)") (InputAction :type "InputAction Object Reference" :default "/Game/Inputs/InputActions/IA_Jump_Stop.IA_Jump_Stop"))
  ;[1 1 1] Enhanced Inputs + event dispatchers
  (:`Triggered`
    (`self.OnStopJump`)))

(event `EnhancedInput|/Game/Inputs/InputActions/IA_PopUpInteract`
  (params (ActionValue :type Boolean) (ElapsedSeconds :type "Float (double-precision)") (TriggeredSeconds :type "Float (double-precision)") (InputAction :type "InputAction Object Reference" :default "/Game/Inputs/InputActions/IA_PopUpInteract.IA_PopUpInteract"))
  ;[1 1 1] Enhanced Inputs + event dispatchers
  (:`Triggered`
    (`self.OnPopUpInteract`)))

(event `EnhancedInput|/Game/Inputs/InputActions/IA_Tilt_Cam_Right`
  (params (ActionValue :type "Float (double-precision)") (ElapsedSeconds :type "Float (double-precision)") (TriggeredSeconds :type "Float (double-precision)") (InputAction :type "InputAction Object Reference" :default "/Game/Inputs/InputActions/IA_Tilt_Cam_Right.IA_Tilt_Cam_Right"))
  ;[1 1 1] Enhanced Inputs + event dispatchers
  (:`Triggered`
    (`self.OnCamTiltRight`)))

(event `OnPopUpInteractEvent`
  ;[1 1 1] Events
  (bind (_asbp_camera_manager _pawntarget _checkpoint _uideathref) (`/Game/Blueprints/Library/BPFL_Fonction_Library.GetCameraManager`))
  (if (`Widget.IsVisible` _uideathref)
    (`/Game/Blueprints/Characters/BP_Character_Base.Respawn` (`/Game/Blueprints/Library/BPFL_Fonction_Library.CastToPlayerCharacter`))
    (`/Game/Blueprints/CameraManager/BP_Camera_Manager.PopDeathUi` _asbp_camera_manager false)))

(event `EnhancedInput|/Game/Inputs/InputActions/IA_Tilt_Cam_Reset`
  (params (ActionValue :type Boolean) (ElapsedSeconds :type "Float (double-precision)") (TriggeredSeconds :type "Float (double-precision)") (InputAction :type "InputAction Object Reference" :default "/Game/Inputs/InputActions/IA_Tilt_Cam_Reset.IA_Tilt_Cam_Reset"))
  ;[1 1 1] Enhanced Inputs + event dispatchers
  (:`Triggered`
    (`self.OnCamTiltReset`)))

(event `EnhancedInput|/Game/Inputs/InputActions/IA_Merge`
  (params (ActionValue :type Boolean) (ElapsedSeconds :type "Float (double-precision)") (TriggeredSeconds :type "Float (double-precision)") (InputAction :type "InputAction Object Reference" :default "/Game/Inputs/InputActions/IA_Merge.IA_Merge"))
  ;[1 1 1] Enhanced Inputs + event dispatchers
  (:`Triggered`
    (`self.OnMerge`)))

(event `ClimbingEvent`
  (bind _asbp_character_base0 (`/Game/Blueprints/Library/BPFL_Fonction_Library.CastToPlayerCharacter`))
  (bind _returnvalue (`|GetInputActionValue`))
  ;[1 1 1] Climb
  (if (`/Game/Blueprints/Library/BPFL_Fonction_Library.Is Current Player Alive` null)
    (if (> _returnvalue 0.0)
      (if (`/Game/Blueprints/Characters/BP_Character_Base.Grounded` _asbp_character_base0)
        (`self.MoveFrontEvent`)
        (else
          (`Pawn.AddMovementInput` _asbp_character_base0 (0.0 0.0 -1.0) 1.0 false)))
      (else
        (`Pawn.AddMovementInput` _asbp_character_base0 (0.0 -0.1 1.0) (* _returnvalue -1.0) false)))))

(event `OnCamTiltRightEvent`
  ;[1 1 1] Events
  (`/Game/Blueprints/Characters/BP_Character_Base.TiltCam` (`/Game/Blueprints/Library/BPFL_Fonction_Library.CastToPlayerCharacter`) (`|GetInputActionValue`))
  (if (not (`self.IsAnimPlayed`))
    (set `self.IsAnimPlayed` true)
    (bind (_asbp_camera_manager _pawntarget _checkpoint _uideathref _uicontrol) (`/Game/Blueprints/Library/BPFL_Fonction_Library.GetCameraManager`))
    (`/Engine/EditorBlueprintResources/StandardMacros.IsValid` _uicontrol
      (:`Is Valid`
        (`/Game/Blueprints/UI/WBP_UIControls.PlayAnimationButtonResetCam` _uicontrol "Forward")))))

(event `EnhancedInput|/Game/Inputs/InputActions/IA_Pause`
  (params (ActionValue :type Boolean) (ElapsedSeconds :type "Float (double-precision)") (TriggeredSeconds :type "Float (double-precision)") (InputAction :type "InputAction Object Reference" :default "/Game/Inputs/InputActions/IA_Pause.IA_Pause"))
  ;[1 1 1] Enhanced Inputs + event dispatchers
  (:`Triggered`
    (`self.OnPause`)))

(event `OnCamTiltResetEvent`
  ;[1 1 1] Events
  (`/Game/Blueprints/Characters/BP_Character_Base.ResetCamTilt` (`/Game/Blueprints/Library/BPFL_Fonction_Library.CastToPlayerCharacter`))
  (if (`self.IsAnimPlayed`)
    (set `self.IsAnimPlayed` false)
    (bind (_asbp_camera_manager _pawntarget _checkpoint _uideathref _uicontrol) (`/Game/Blueprints/Library/BPFL_Fonction_Library.GetCameraManager`))
    (`/Engine/EditorBlueprintResources/StandardMacros.IsValid` _uicontrol
      (:`Is Valid`
        (`/Game/Blueprints/UI/WBP_UIControls.PlayAnimationButtonResetCam` _uicontrol "Reverse")))))

(event `SetToClimbingMode`
  (params (Ladder :type Boolean))
  ;[1 1 1] Climb
  (clear `self.OnMoveFront`)
  (add `self.OnMoveFront` (`|CreateDelegate` :!event `ClimbingEvent`))
  (`CharacterMovementComponent.SetMovementMode` (`Character.CharacterMovement` (`/Game/Blueprints/Library/BPFL_Fonction_Library.CastToPlayerCharacter`)) "MOVE_Flying" 0)
  (set `self.Ladder` Ladder))

(event `SetToWalkingMode`
  ;[1 1 1] Climb
  (clear `self.OnMoveFront`)
  (add `self.OnMoveFront` (`|CreateDelegate` :!event `MoveFrontEvent`))
  (`CharacterMovementComponent.SetMovementMode` (`Character.CharacterMovement` (`/Game/Blueprints/Library/BPFL_Fonction_Library.CastToPlayerCharacter`)) "MOVE_Walking" 0)
  (set `self.Ladder` false))

(event `OnGrabEvent`
  ;[1 1 1] Grab
  (bind _asbp_character_full (cast `/Game/Blueprints/Characters/BP_Character_Full` (`self.K2_GetPawn`)))
  (bind _grabbedobject (`/Game/Blueprints/Characters/BP_Character_Full.GrabbedObject` _asbp_character_full))
  (`/Engine/EditorBlueprintResources/StandardMacros.IsValid` _grabbedobject
    (:`Is Valid`
      (`|ExecutionSequence`
        (:`then_0`
          (add `self.OnJump` (`|CreateDelegate` :!event `OnJumpEvent`))
          (bind _characterspeed (`/Game/Blueprints/Characters/BP_Character_Base.CharacterSpeed` _asbp_character_full))
          (bind _charactermovement (`Character.CharacterMovement` _asbp_character_full))
          (set `CharacterMovementComponent.MaxWalkSpeed` _characterspeed _charactermovement))
        (:`then_1`
          ;;[1 1 1] Enlever grabbed object à la fin si on veut l'utiliser avant
          (set `/Game/Blueprints/Objects/GrabbableObjects/BP_Grabbable_Object.CharaRef` null _grabbedobject)
          (set `/Game/Blueprints/Characters/BP_Character_Full.GrabbedObject` null _asbp_character_full))))
    (:`Is Not Valid`
      (bind _returnvalue (`SceneComponent.K2_GetComponentLocation` (`PaperCharacter.Sprite` _asbp_character_full)))
      (bind (_returnvalue_2 _distance) (`/Game/Blueprints/Library/BPFL_Fonction_Library.FindNearestActorOfClass` "/Game/Blueprints/Objects/GrabbableObjects/BP_Grabbable_Object.BP_Grabbable_Object_C" _returnvalue))
      (if (<= _distance 50.0)
        (bind _asbp_grabbable_object (cast `/Game/Blueprints/Objects/GrabbableObjects/BP_Grabbable_Object` _returnvalue_2))
        (bind _returnvalue_3 (`SceneComponent.K2_GetComponentLocation` (`/Game/Blueprints/Objects/GrabbableObjects/BP_Grabbable_Object.TopOfMesh` _asbp_grabbable_object)))
        (if (and (> (.z _returnvalue_3) (.z _returnvalue)) (`NavMovementComponent.IsMovingOnGround` (`Character.CharacterMovement` _asbp_character_full)) (`/Game/Blueprints/Library/BPFL_Fonction_Library.Is Current Player Alive` null))
          (bind _output_get (set `/Game/Blueprints/Characters/BP_Character_Full.GrabbedObject` _asbp_grabbable_object _asbp_character_full))
          (set `/Game/Blueprints/Objects/GrabbableObjects/BP_Grabbable_Object.CharaRef` _asbp_character_full _output_get)
          (remove `self.OnJump` (`|CreateDelegate` :!event `OnJumpEvent`))
          (set `CharacterMovementComponent.MaxWalkSpeed` (* _characterspeed 0.7) _charactermovement)
          (`/Game/Blueprints/Objects/GrabbableObjects/BP_Grabbable_Object.SnapCharacter` _output_get (`/Game/Blueprints/Library/BPFL_Fonction_Library.GetRelativeCardinalPoint` _returnvalue_3 _returnvalue)))))))

(event `Interract`)

(fn `UserConstructionScript`)