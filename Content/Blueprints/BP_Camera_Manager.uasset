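; Player camera manager that overrides BlueprintUpdateCamera to follow a pawn's camera while locking its world Y position.
; It copies X, Z, rotation and FOV from PawnTarget's camera component.
; Y is clamped with identical bounds, pinning it to the spring arm length plus a fixed offset.
; An invalid PawnTarget returns false with zeroed outputs; this file never assigns that variable.
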(fn `BlueprintUpdateCamera`
  (params (CameraTarget :type "Actor Object Reference"))
  (returns (NewCameraLocation :type "Vector Structure") (NewCameraRotation :type "Rotator Structure") (NewCameraFOV :type "Float (single-precision)") (ReturnValue :type Boolean))
  (bind _pawntarget (`self.PawnTarget`))
  (bind _camera (`/Game/Blueprints/Character/BP_Character_Base.Camera` _pawntarget))
  (bind (_returnvalue_location _returnvalue_rotation) (`KismetMathLibrary.BreakTransform` (`SceneComponent.K2_GetComponentToWorld` _camera)))
  (bind _returnvalue (+ (`SpringArmComponent.TargetArmLength` (`/Game/Blueprints/Character/BP_Character_Base.SpringArm` _pawntarget)) 1000.0))
  (`/Engine/EditorBlueprintResources/StandardMacros.IsValid` _pawntarget
    (:`Is Valid`
      (return (`KismetMathLibrary.MakeVector` (.x _returnvalue_location) (`KismetMathLibrary.FClamp` (.y _returnvalue_location) _returnvalue _returnvalue) (.z _returnvalue_location)) _returnvalue_rotation (`CameraComponent.FieldOfView` _camera) true))
    (:`Is Not Valid`
      (return (0.0 0.0 0.0) (struct) 0.0 false))))

(fn `UserConstructionScript`)