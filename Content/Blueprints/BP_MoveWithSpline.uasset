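; BP_MoveWithSpline is a Blueprint that moves its static mesh along its spline in a continuous loop.
; Each Tick advances a normalized Time by DeltaSeconds divided by Speed, so Speed acts as lap duration, and resets it at 1.
; The mesh takes the spline's local location at that time, without constant velocity, and follows only its yaw, offset by -90 degrees.
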(event `self.ReceiveTick`
  (params (DeltaSeconds :type "Float (single-precision)"))
  (bind _spline (`self.Spline`))
  (bind _staticmesh (`self.StaticMesh`))
  (bind (_returnvalue_roll _returnvalue_pitch _returnvalue_yaw) (`KismetMathLibrary.BreakRotator` (`SplineComponent.GetRotationAtTime` _spline (`self.Time`) "Local" false)))
  (if (>= (`self.Time`) 1.0)
    (set `self.Time` 0.0)
    (else
      (set `self.Time` (+ (/ DeltaSeconds (`self.Speed`)) (`self.Time`)))))
  (`SceneComponent.K2_SetRelativeLocation` _staticmesh (`SplineComponent.GetLocationAtTime` _spline (`self.Time`) "Local" false) false false)
  (`SceneComponent.K2_SetRelativeRotation` _staticmesh (`KismetMathLibrary.MakeRotator` 0.0 0.0 (- _returnvalue_yaw 90.0)) false false))

(fn `UserConstructionScript`)