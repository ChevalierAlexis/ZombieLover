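; Player controller for a sprite character that can split into top and bottom halves and merge back.
; Enhanced Input actions fire event dispatchers, with handlers bound at BeginPlay driving movement, interaction, camera tilt and respawn.
; Jumping supports coyote time and buffering, separating the full character when an airborne jump isn't buffered.
; Also holds climbing, object-grab and manual-merge handlers, adds the controls UI, and has temporary level-switch keys.
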(event `self.ReceiveBeginPlay`
  (bind _returnvalue (pcsubsystem `EnhancedInputLocalPlayerSubsystem` self))
  ;[1 1 1] Bind Event
  (`|ExecutionSequence`
    (:`then_0`
      (add `self.OnInteraction` (`|CreateDelegate` :!event `OnInteractionEvent`))
      (add `self.OnInteractionStop` (`|CreateDelegate` :!event `OnInteractioStopEvent`))
      (add `self.OnSeparation` (`|CreateDelegate` :!event `OnSeparationEvent`))
      (add `self.OnJump` (`|CreateDelegate` :!event `OnJumpEvent`))
      (add `self.OnStopJump` (`|CreateDelegate` :!event `OnStopJumpEvent`))
      (add `self.OnMoveRight` (`|CreateDelegate` :!event `MoveRightEvent`))
      (add `self.OnMoveFront` (`|CreateDelegate` :!event `MoveFrontEvent`))
      (add `self.OnPopUpInteract` (`|CreateDelegate` :!event `OnPopUpInteractEvent`))
      (add `self.OnCamTiltRight` (`|CreateDelegate` :!event `OnCamTiltRightEvent`))
      (add `self.OnCamTiltReset` (`|CreateDelegate` :!event `OnCamTiltResetEvent`)))
    (:`then_1`
      ;[1 1 1] Ajoute les contrôles
      (`/Engine/EditorBlueprintResources/StandardMacros.IsValid` _returnvalue
        (:`Is Valid`
          (`EnhancedInputSubsystemInterface.AddMappingContext` _returnvalue "/Game/Inputs/IMC_Mapping_Context.IMC_Mapping_Context" 0 (struct))
          ;[1 1 1] Ajoute l'UI
          (bind _returnvalue_2 (`|CreateWidget` "/Game/Blueprints/UI/W_UIControls.W_UIControls_C" self))
          (`UserWidget.AddToViewport` _returnvalue_2 0))))))

(event `OnInteractionEvent`
  ;[1 1 1] Events
  (`/Game/Blueprints/Characters/BP_Character_Base.Interact` (`/Game/Blueprints/Library/BPFL_Fonction_Library.CastToPlayerCharacter`)))

(event `OnSeparationEvent`
  ;[1 1 1] Events
  (`/Game/Blueprints/Characters/BP_Character_Base.Separate` (`/Game/Blueprints/Library/BPFL_Fonction_Library.CastToPlayerCharacter`)))

(event `Key|U`
  (params (Key :type "Key Structure"))
  ;[1 1 1] prototype (temporaire)
  (:`Pressed`
    (`GameplayStatics.OpenLevelBySoftObjectPtr` "/Game/Levels/L_Proto.L_Proto")))

(event `EnhancedInput|/Game/Inputs/InputActions/IA_Move_Front`
  (params (ActionValue :type "Float (double-precision)") (ElapsedSeconds :type "Float (double-precision)") (TriggeredSeconds :type "Float (double-precision)") (InputAction :type "InputAction Object Reference" :default "/Game/Inputs/InputActions/IA_Move_Front.IA_Move_Front"))
  ;[1 1 1] Enhanced Inputs + event dispatchers
  (:`Triggered`
    (`self.OnMoveFront`)))

(event `MoveRightEvent`
  (bind _asbp_character_base0 (`/Game/Blueprints/Library/BPFL_Fonction_Library.CastToPlayerCharacter`))
  (bind _asbp_character_base0_2 (`/Game/Blueprints/Library/BPFL_Fonction_Library.CastToPlayerCharacter`))
  (bind _returnvalue (`|GetInputActionValue`))
  ;[1 1 1] Events
  (if (> _returnvalue 0.0)
    (set `/Game/Blueprints/Characters/BP_Character_Base.IsFacingRight` true _asbp_character_base0_2)
    (bind _asbp_character_full (cast `/Game/Blueprints/Characters/BP_Character_Full` _asbp_character_base0_2)
      (:`then`
        (if (not (`/Game/Blueprints/Characters/BP_Character_Full.Grab` _asbp_character_full))
          (`SceneComponent.K2_SetRelativeRotation` :`self` (`PaperCharacter.Sprite` _asbp_character_base0_2) :!label _label)))
      (:`CastFailed`
        (goto _label)))
    (`Pawn.AddMovementInput` (`/Game/Blueprints/Library/BPFL_Fonction_Library.CastToPlayerCharacter`) (1.0 0.0 0.0) (`|GetInputActionValue`) false :!label _label_2)
    (elif (< _returnvalue 0.0)
      (set `/Game/Blueprints/Characters/BP_Character_Base.IsFacingRight` false _asbp_character_base0)
      (bind _asbp_character_full_2 (cast `/Game/Blueprints/Characters/BP_Character_Full` _asbp_character_base0)
        (:`then`
          (if (`/Game/Blueprints/Characters/BP_Character_Full.Grab` _asbp_character_full_2)
            (goto _label_2)
            (else
              _)))
        (:`CastFailed`
          _))
      (`SceneComponent.K2_SetRelativeRotation` (`PaperCharacter.Sprite` _asbp_character_base0) (struct :`Yaw` 180.0) false false)
      (goto _label_2))))

(event `EnhancedInput|/Game/Inputs/InputActions/IA_Move_Right`
  (params (ActionValue :type "Float (double-precision)") (ElapsedSeconds :type "Float (double-precision)") (TriggeredSeconds :type "Float (double-precision)") (InputAction :type "InputAction Object Reference" :default "/Game/Inputs/InputActions/IA_Move_Right.IA_Move_Right"))
  ;[1 1 1] Enhanced Inputs + event dispatchers
  (:`Triggered`
    (`self.OnMoveRight`)))

(event `Key|I`
  (params (Key :type "Key Structure"))
  ;[1 1 1] prototype (temporaire)
  (:`Pressed`
    (`GameplayStatics.OpenLevelBySoftObjectPtr` "/Game/Levels/L_Diorama.L_Diorama")))

(event `OnInteractioStopEvent`
  ;[1 1 1] Events
)

(event `EnhancedInput|/Game/Inputs/InputActions/IA_Interaction`
  (params (ActionValue :type Boolean) (ElapsedSeconds :type "Float (double-precision)") (TriggeredSeconds :type "Float (double-precision)") (InputAction :type "InputAction Object Reference" :default "/Game/Inputs/InputActions/IA_Interaction.IA_Interaction"))
  ;[1 1 1] Enhanced Inputs + event dispatchers
  (:`Started`
    (`self.OnInteraction`))
  (:`Completed`
    (`self.OnInteractionStop`)))

(event `Key|O`
  (params (Key :type "Key Structure"))
  ;[1 1 1] prototype (temporaire)
  (:`Pressed`
    (`GameplayStatics.OpenLevelBySoftObjectPtr` "/Game/Levels/L_Diorama2.L_Diorama2")))

(event `Key|P`
  (params (Key :type "Key Structure"))
  ;[1 1 1] prototype (temporaire)
  (:`Pressed`
    (`GameplayStatics.OpenLevelBySoftObjectPtr` "/Game/Levels/L_Diorama01.L_Diorama01")))

(event `OnJumpEvent`
  (bind _asbp_character_base0 (`/Game/Blueprints/Library/BPFL_Fonction_Library.CastToPlayerCharacter`))
  ;[1 1 1] Events
  (if (`NavMovementComponent.IsMovingOnGround` (`Character.CharacterMovement` _asbp_character_base0))
    (`/Game/Blueprints/Characters/BP_Character_Base.JumpSqueeze` _asbp_character_base0 :!label _label_3)
    (`Character.Jump` _asbp_character_base0)
    (elif (> (`KismetSystemLibrary.K2_GetTimerRemainingTimeHandle` (`/Game/Blueprints/Characters/BP_Character_Base.CoyoteTime` _asbp_character_base0)) 0.0)
      (goto _label_3)
      (else
        (`/Game/Blueprints/Characters/BP_Character_Base.BufferJump` _asbp_character_base0)
        (if (not (`/Game/Blueprints/Characters/BP_Character_Base.JumpBuffered` _asbp_character_base0))
          (bind _asbp_character_full (cast `/Game/Blueprints/Characters/BP_Character_Full` (`self.K2_GetPawn`)))
          (`/Game/Blueprints/Characters/BP_Character_Base.Separate` _asbp_character_full))))))

(event `MoveFrontEvent`
  (bind _asbp_character_base0 (`/Game/Blueprints/Library/BPFL_Fonction_Library.CastToPlayerCharacter`))
  (bind _asbp_character_base0_2 (`/Game/Blueprints/Library/BPFL_Fonction_Library.CastToPlayerCharacter`))
  (bind _returnvalue (`|GetInputActionValue`))
  ;[1 1 1] Events
  (if (> _returnvalue 0.0)
    (set `/Game/Blueprints/Characters/BP_Character_Base.IsFacingFront` true _asbp_character_base0)
    (set `/Game/Blueprints/Characters/BP_Character_Base.IsMovingFront` true _asbp_character_base0 :!label _label_4)
    (`Pawn.AddMovementInput` _asbp_character_base0 (0.0 1.0 0.0) (`|GetInputActionValue`) false)
    (elif (< _returnvalue 0.0)
      (set `/Game/Blueprints/Characters/BP_Character_Base.IsFacingFront` false _asbp_character_base0_2)
      (goto _label_4)
      (else
        (set `/Game/Blueprints/Characters/BP_Character_Base.IsMovingFront` false _asbp_character_base0_2)))))

(event `EnhancedInput|/Game/Inputs/InputActions/IA_Separation`
  (params (ActionValue :type Boolean) (ElapsedSeconds :type "Float (double-precision)") (TriggeredSeconds :type "Float (double-precision)") (InputAction :type "InputAction Object Reference" :default "/Game/Inputs/InputActions/IA_Separation.IA_Separation"))
  ;[1 1 1] Enhanced Inputs + event dispatchers
  (:`Triggered`
    (`self.OnSeparation`)))

(event `EnhancedInput|/Game/Inputs/InputActions/IA_Jump`
  (params (ActionValue :type Boolean) (ElapsedSeconds :type "Float (double-precision)") (TriggeredSeconds :type "Float (double-precision)") (InputAction :type "InputAction Object Reference" :default "/Game/Inputs/InputActions/IA_Jump.IA_Jump"))
  ;[1 1 1] Enhanced Inputs + event dispatchers
  (:`Triggered`
    (`self.OnJump`)))

(event `EnhancedInput|/Game/Inputs/InputActions/IA_Jump_Stop`
  (params (ActionValue :type Boolean) (ElapsedSeconds :type "Float (double-precision)") (TriggeredSeconds :type "Float (double-precision)") (InputAction :type "InputAction Object Reference" :default "/Game/Inputs/InputActions/IA_Jump_Stop.IA_Jump_Stop"))
  ;[1 1 1] Enhanced Inputs + event dispatchers
  (:`Triggered`
    (`self.OnStopJump`)))

(event `EnhancedInput|/Game/Inputs/InputActions/IA_PopUpInteract`
  (params (ActionValue :type Boolean) (ElapsedSeconds :type "Float (double-precision)") (TriggeredSeconds :type "Float (double-precision)") (InputAction :type "InputAction Object Reference" :default "/Game/Inputs/InputActions/IA_PopUpInteract.IA_PopUpInteract"))
  ;[1 1 1] Enhanced Inputs + event dispatchers
  (:`Triggered`
    (`self.OnPopUpInteract`)))

(event `EnhancedInput|/Game/Inputs/InputActions/IA_Tilt_Cam_Right`
  (params (ActionValue :type "Float (double-precision)") (ElapsedSeconds :type "Float (double-precision)") (TriggeredSeconds :type "Float (double-precision)") (InputAction :type "InputAction Object Reference" :default "/Game/Inputs/InputActions/IA_Tilt_Cam_Right.IA_Tilt_Cam_Right"))
  ;[1 1 1] Enhanced Inputs + event dispatchers
  (:`Triggered`
    (`self.OnCamTiltRight`)))

(event `OnStopJumpEvent`
  ;[1 1 1] Events
  (`Character.StopJumping` (`/Game/Blueprints/Library/BPFL_Fonction_Library.CastToPlayerCharacter`)))

(event `Grounded Climbing`
  (bind _returnvalue (`GameplayStatics.GetPlayerCharacter` 0))
  ;[1 1 1] Events
  (if (`/Game/Blueprints/Characters/BP_Character_Base.Grounded` (`/Game/Blueprints/Library/BPFL_Fonction_Library.CastToPlayerCharacter`))
    (bind _result (`/Engine/EditorBlueprintResources/StandardMacros.NegateFloat` (`|GetInputActionValue`))
      (:`  `
        (if (<= _result 0.0)
          (`Pawn.AddMovementInput` _returnvalue (* (`self.GetActorUpVector` _returnvalue) (0.0 0.0 0.25)) _result false)
          (else
            (`Pawn.AddMovementInput` (`/Game/Blueprints/Library/BPFL_Fonction_Library.CastToPlayerCharacter`) (0.0 1.0 0.0) (`|GetInputActionValue`) false)))))
    (else
      (remove `self.OnMoveFront` (`|CreateDelegate` :!event `Grounded Climbing`))
      (add `self.OnMoveFront` (`|CreateDelegate` :!event `ClimbingEvent`))
      (if (`self.Ladder`)
        (clear `self.OnMoveRight`)))))

(event `EnhancedInput|/Game/Inputs/InputActions/IA_Tilt_Cam_Reset`
  (params (ActionValue :type Boolean) (ElapsedSeconds :type "Float (double-precision)") (TriggeredSeconds :type "Float (double-precision)") (InputAction :type "InputAction Object Reference" :default "/Game/Inputs/InputActions/IA_Tilt_Cam_Reset.IA_Tilt_Cam_Reset"))
  ;[1 1 1] Enhanced Inputs + event dispatchers
  (:`Triggered`
    (`self.OnCamTiltReset`)))

(event `EnhancedInput|/Game/Inputs/InputActions/IA_Merge`
  (params (ActionValue :type Boolean) (ElapsedSeconds :type "Float (double-precision)") (TriggeredSeconds :type "Float (double-precision)") (InputAction :type "InputAction Object Reference" :default "/Game/Inputs/InputActions/IA_Merge.IA_Merge"))
  ;[1 1 1] Enhanced Inputs + event dispatchers
  (:`Triggered`
    (`self.OnMerge`)))

(event `ClimbingEvent`
  (bind _returnvalue (`GameplayStatics.GetPlayerCharacter` 0))
  ;[1 1 1] Events
  (if (`/Game/Blueprints/Characters/BP_Character_Base.Grounded` (`/Game/Blueprints/Library/BPFL_Fonction_Library.CastToPlayerCharacter`))
    (add `self.OnMoveRight` (`|CreateDelegate` :!event `MoveRightEvent`))
    (add `self.OnMoveFront` (`|CreateDelegate` :!event `Grounded Climbing`))
    (else
      (bind _result (`/Engine/EditorBlueprintResources/StandardMacros.NegateFloat` (`|GetInputActionValue`))
        (:`  `
          (`Pawn.AddMovementInput` _returnvalue (* (`self.GetActorUpVector` _returnvalue) (0.0 0.0 0.5)) _result false)
          (if (> _result 0.0)
            (`Pawn.AddMovementInput` _returnvalue (0.0 -1.0 0.0) _result false)))))))

(event `MoveRightGrabbedObject`
  ;[1 1 1] Events
)

(event `OnPopUpInteractEvent`
  ;[1 1 1] Events
  (bind _asbp_camera_manager (`/Game/Blueprints/Library/BPFL_Fonction_Library.GetCameraManager`))
  (`/Game/Blueprints/Characters/BP_Character_Base.Respawn` (`/Game/Blueprints/Library/BPFL_Fonction_Library.CastToPlayerCharacter`))
  (`/Game/Blueprints/BP_Camera_Manager.PopDeathUi` _asbp_camera_manager false))

(event `OnCamTiltRightEvent`
  ;[1 1 1] Events
  (`/Game/Blueprints/Characters/BP_Character_Base.TiltCam` (`/Game/Blueprints/Library/BPFL_Fonction_Library.CastToPlayerCharacter`) (`|GetInputActionValue`))
  (if (not (`self.IsAnimPlayed`))
    (set `self.IsAnimPlayed` true)
    (bind (_asbp_camera_manager _pawntarget _uideathref _uicontrol) (`/Game/Blueprints/Library/BPFL_Fonction_Library.GetCameraManager`))
    (`/Game/Blueprints/UI/W_UIControls.PlayAnimationButtonResetCam` _uicontrol "Forward")))

(event `OnGrabEvent`
  (`KismetSystemLibrary.PrintString` "Grab")
  (bind _asbp_character_full (cast `/Game/Blueprints/Characters/BP_Character_Full` (`self.K2_GetPawn`)))
  ;[1 1 1] Events
  (if (`/Game/Blueprints/Characters/BP_Character_Full.Grab` _asbp_character_full)
    (bind _asbp_character_full_2 (cast `/Game/Blueprints/Characters/BP_Character_Full` (`self.K2_GetPawn`)))
    (set `/Game/Blueprints/Characters/BP_Character_Full.Grab` false _asbp_character_full_2)
    (bind _grabbableobjectmesh (`/Game/Blueprints/Objects/GrabbableObjects/BP_Grabbable_Object.GrabbableObjectMesh` (`/Game/Blueprints/Characters/BP_Character_Full.GrabbedObject` _asbp_character_full_2)))
    (`SceneComponent.K2_DetachFromComponent` _grabbableobjectmesh "KeepRelative" "KeepRelative" "KeepRelative" true)
    (`PrimitiveComponent.SetSimulatePhysics` _grabbableobjectmesh true)
    (`PrimitiveComponent.SetCollisionObjectType` _grabbableobjectmesh "ECC_WorldDynamic")
    (`PrimitiveComponent.SetCollisionResponseToChannel` (`Character.CapsuleComponent` _asbp_character_full_2) "ECC_PhysicsBody" "ECR_Block")
    (else
      (`PrimitiveComponent.SetCollisionResponseToChannel` (`Character.CapsuleComponent` _asbp_character_full) "ECC_PhysicsBody" "ECR_Ignore")
      (set `/Game/Blueprints/Characters/BP_Character_Full.Grab` true _asbp_character_full)
      (bind _grabbedobject (`/Game/Blueprints/Characters/BP_Character_Full.GrabbedObject` _asbp_character_full))
      (bind _grabbableobjectmesh_2 (`/Game/Blueprints/Objects/GrabbableObjects/BP_Grabbable_Object.GrabbableObjectMesh` _grabbedobject))
      (`PrimitiveComponent.SetCollisionObjectType` _grabbableobjectmesh_2 "ECC_PhysicsBody")
      (`PrimitiveComponent.SetSimulatePhysics` _grabbableobjectmesh_2 false)
      (`self.K2_AttachToComponent` _grabbedobject (`PaperCharacter.Sprite` (`/Game/Blueprints/Library/BPFL_Fonction_Library.CastToPlayerCharacter`)) "None" "KeepWorld" "KeepWorld" "KeepWorld" true))))

(event `OnCamTiltResetEvent`
  ;[1 1 1] Events
  (`/Game/Blueprints/Characters/BP_Character_Base.ResetCamTilt` (`/Game/Blueprints/Library/BPFL_Fonction_Library.CastToPlayerCharacter`))
  (if (`self.IsAnimPlayed`)
    (set `self.IsAnimPlayed` false)
    (bind (_asbp_camera_manager _pawntarget _uideathref _uicontrol) (`/Game/Blueprints/Library/BPFL_Fonction_Library.GetCameraManager`))
    (`/Game/Blueprints/UI/W_UIControls.PlayAnimationButtonResetCam` _uicontrol "Reverse")))

(event `ManualMerge`
  (bind _returnvalue (`self.K2_GetPawn`))
  (bind _asbp_character_bottom (cast `/Game/Blueprints/Characters/BP_Character_Bottom` _returnvalue)
    (:`then`
      (bind _outactors (`GameplayStatics.GetAllActorsOfClass` "/Game/Blueprints/Characters/BP_Character_Top.BP_Character_Top_C"))
      (if (> (`KismetArrayLibrary.Array_Length` _outactors) 1)
        (`KismetSystemLibrary.PrintString` "Plusieurs \"BP_Character_Top\" détectés !"))
      (`/Game/Blueprints/Characters/BP_Character_Bottom.MergeCharacter` _asbp_character_bottom (`|GetArrayItem` _outactors) false))
    (:`CastFailed`
      (bind _asbp_character_top (cast `/Game/Blueprints/Characters/BP_Character_Top` _returnvalue))
      (bind _outactors_2 (`GameplayStatics.GetAllActorsOfClass` "/Game/Blueprints/Characters/BP_Character_Bottom.BP_Character_Bottom_C"))
      (if (> (`KismetArrayLibrary.Array_Length` _outactors_2) 1)
        (`KismetSystemLibrary.PrintString` "Plusieurs \"BP_Character_Bottom\" détectés !"))
      (bind _asbp_character_bottom_2 (cast `/Game/Blueprints/Characters/BP_Character_Bottom` (`|GetArrayItem` _outactors_2)))
      (`/Game/Blueprints/Characters/BP_Character_Bottom.MergeCharacter` _asbp_character_bottom_2 _asbp_character_top false))))

(event `Interract`)

(fn `UserConstructionScript`)