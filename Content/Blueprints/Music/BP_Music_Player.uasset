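; Music player actor that drives a MetaSound audio component to play and switch between indexed music tracks.
; BeginPlay fires the "On Play" trigger and watches the MetaSound's "FadeOut" output, whose callback fires "NewTrigger" back into it.
; ChangeMusic skips requests matching the stored FormerIndex; otherwise it sets the "Index" parameter, fires "ChangeMusic" and stores the new index.
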(event `self.ReceiveBeginPlay`
  (`AudioParameterControllerInterface.SetTriggerParameter` (`self.Audio`) "On Play")
  (`MetaSoundOutputSubsystem.WatchOutput` (subsystem `MetaSoundOutputSubsystem`) (`self.Audio`) "FadeOut" (delegate `FadedOut`) "None" "None"))

(event `self.ReceiveTick`
  (params (DeltaSeconds :type "Float (single-precision)")))

(event `FadedOut`
  (params (OutputName :type Name) (Output :type "MetaSoundOutput Structure (by ref)"))
  (`KismetSystemLibrary.PrintString` "General Kenobi")
  (`AudioParameterControllerInterface.SetTriggerParameter` (`self.Audio`) "NewTrigger"))

(fn `ChangeMusic`
  (params (Index :type Integer))
  (bind _audio (`self.Audio`))
  (`KismetSystemLibrary.PrintString` (`KismetStringLibrary.Conv_IntToString` Index))
  (bind _isdifferent (`self.IsDifferentMusic` Index))
  (if _isdifferent
    (`AudioParameterControllerInterface.SetIntParameter` _audio "Index" Index)
    (`AudioParameterControllerInterface.SetTriggerParameter` _audio "ChangeMusic")
    (set `self.FormerIndex` Index)))

(fn `IsDifferentMusic`
  (params (Index :type Integer))
  (returns (IsDifferent :type Boolean))
  (return (!= Index (`self.FormerIndex`))))

(fn `UserConstructionScript`)