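; BP_Ladder is a ladder object with an editable height that rebuilds its shape in the Construction Script.
; Height places LadderTop, whose Z then drives the offset and scale of both side rail meshes.
; Crossbar rungs are regenerated as mesh instances at fixed intervals, and the loop also resizes InteractionRange to the ladder's height.
; Activation only forwards to the parent class.
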(fn `Activation`
  (params (PlayerWhoActivated :type "/Game/Blueprints/Characters/BP_Character_Base Object Reference"))
  (`parent.Activation` null))

(fn `AdjustLadderSize`
  (params (Ladder_Mesh :type "SceneComponent Object Reference"))
  (bind _returnvalue (`SceneComponent.GetRelativeTransform` Ladder_Mesh))
  (bind (_relativelocation_x _relativelocation_y _relativelocation_z) (`KismetMathLibrary.BreakVector` (`SceneComponent.RelativeLocation` (`self.Ladder_Top`))))
  (`SceneComponent.K2_SetRelativeTransform` Ladder_Mesh (`KismetMathLibrary.MakeTransform` (`KismetMathLibrary.MakeVector` (.x (.location _returnvalue)) (.y (.location _returnvalue)) (/ _relativelocation_z 1.9)) (.rotation _returnvalue) (`KismetMathLibrary.MakeVector` (.x (.scale _returnvalue)) (.y (.scale _returnvalue)) (/ _relativelocation_z 100.0))) false false))

(fn `UserConstructionScript`
  (bind _interactionrange (`self.InteractionRange`))
  (bind _tempheight (`self.TempHeight`))
  (bind _returnvalue (`SceneComponent.GetRelativeTransform` _interactionrange))
  (bind (_relativelocation_x _relativelocation_y _relativelocation_z) (`KismetMathLibrary.BreakVector` (`SceneComponent.RelativeLocation` (`self.Ladder_Top`))))
  (bind (_relativelocation_x_2 _relativelocation_y_2 _relativelocation_z_2) (`KismetMathLibrary.BreakVector` (`SceneComponent.RelativeLocation` (`self.Ladder_Top`))))
  (`SceneComponent.K2_SetRelativeLocation` (`self.Ladder_Top`) (`KismetMathLibrary.MakeVector` 0.0 0.0 (`self.Height`)) false false)
  (`self.AdjustLadderSize` (`self.Ladder_Mesh_L`))
  (`self.AdjustLadderSize` (`self.Ladder_Mesh_R`))
  (set `self.TempHeight` 0.0)
  (`InstancedStaticMeshComponent.ClearInstances` (`self.Crossbar`))
  (while (< _tempheight _relativelocation_z_2)
    (`InstancedStaticMeshComponent.AddInstance` (`self.Crossbar`) (`KismetMathLibrary.MakeTransform` (`KismetMathLibrary.MakeVector` 0.0 0.0 _tempheight) (struct) (0.075 0.005 0.01)) false)
    (set `self.TempHeight` (+ (`self.TempHeight`) 10.0))
    (`SceneComponent.K2_SetRelativeTransform` _interactionrange (`KismetMathLibrary.MakeTransform` (`KismetMathLibrary.MakeVector` (.x (.location _returnvalue)) (.y (.location _returnvalue)) (/ _relativelocation_z 2.0)) (.rotation _returnvalue) (`KismetMathLibrary.MakeVector` (.x (.scale _returnvalue)) (.y (.scale _returnvalue)) (/ _relativelocation_z 55.0))) false false)))