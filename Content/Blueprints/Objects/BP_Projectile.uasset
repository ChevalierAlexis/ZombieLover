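; BP_Projectile is a flipbook projectile that flies along a timeline-driven arc and kills what it hits.
; On BeginPlay, the Trajectory timeline adds X and Z offsets, scaled by Distance and MaxHeight, to its current location each update.
; Capsule overlap with any actor except the instigator calls KillActor through BPCKill, then destroys the projectile.
; Location debug prints remain, alongside disconnected experiments such as scaling play rate by bowman-to-player distance.
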(event `self.ReceiveBeginPlay`
  (bind (_returnvalue_x _returnvalue_y _returnvalue_z) (`KismetMathLibrary.BreakVector` (`self.K2_GetActorLocation`)))
  (`KismetSystemLibrary.PrintString` (`KismetStringLibrary.Conv_VectorToString` (`self.K2_GetActorLocation`)))
  (bind (_direction _ztrack _xtrack) (`Timeline|Trajectory` :!via `PlayFromStart`)
    (:`Update`
      (`self.K2_SetActorLocation` (`KismetMathLibrary.MakeVector` (+ (* _xtrack (`self.Distance`)) _returnvalue_x) _returnvalue_y (+ (* _ztrack (`self.MaxHeight`)) _returnvalue_z))))))

(event `TrajectoryManager`
  ;[1 1 1] Blblblblblblb
)

(event `self.ReceiveTick`
  (params (DeltaSeconds :type "Float (single-precision)"))
  (`KismetSystemLibrary.PrintString` (`KismetStringLibrary.Conv_VectorToString` (`self.K2_GetActorLocation`))))

(event `self.Capsule.OnComponentBeginOverlap`
  (params (OverlappedComponent :type "PrimitiveComponent Object Reference") (OtherActor :type "Actor Object Reference") (OtherComp :type "PrimitiveComponent Object Reference") (OtherBodyIndex :type Integer) (bFromSweep :type Boolean) (SweepResult :type "HitResult Structure (by ref)"))
  (if (not (== OtherActor (`self.GetInstigator`)))
    (`/Game/Blueprints/Characters/Components/BPC_Kill.KillActor` (`self.BPC_Kill`) OtherActor)
    (`self.K2_DestroyActor`)))

(fn `UserConstructionScript`)