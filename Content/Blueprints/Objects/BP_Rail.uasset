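; Rail actor that draws the player character toward a spline's world Y while railed and this is the controller's ActiveRail.
; Box overlaps by BP_Character_Base toggle the zombie controller's Railed state.
; Tick compares FrontAxisValue with the player's side of the spline, either halving CoefReduc without correction or restoring it and interpolating Y at constant speed.
; The four Move Smooth graphs are identical copies of that interpolation.
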(event `self.ReceiveTick`
  (params (DeltaSeconds :type "Float (single-precision)"))
  (bind _asbp_player_controller (`/Game/Blueprints/Library/BPFL_Fonction_Library.GetZombiePlayerController`))
  (bind _returnvalue (`GameplayStatics.GetPlayerCharacter` 0))
  (bind _returnvalue_2 (`GameplayStatics.GetPlayerCharacter` 0))
  (bind _returnvalue_3 (`GameplayStatics.GetPlayerCharacter` 0))
  (bind _returnvalue_4 (`GameplayStatics.GetPlayerCharacter` 0))
  (bind _returnvalue_5 (`self.K2_GetActorLocation` (`GameplayStatics.GetPlayerCharacter` 0)))
  (bind _returnvalue_6 (`self.K2_GetActorLocation` (`GameplayStatics.GetPlayerCharacter` 0)))
  (bind (_returnvalue_x _returnvalue_y _returnvalue_z) (`KismetMathLibrary.BreakVector` (`self.K2_GetActorLocation` _returnvalue)))
  (bind (_returnvalue_x_2 _returnvalue_y_2 _returnvalue_z_2) (`KismetMathLibrary.BreakVector` (`self.K2_GetActorLocation` _returnvalue_2)))
  (bind (_returnvalue_x_3 _returnvalue_y_3 _returnvalue_z_3) (`KismetMathLibrary.BreakVector` (`self.K2_GetActorLocation` _returnvalue_3)))
  (bind (_returnvalue_x_4 _returnvalue_y_4 _returnvalue_z_4) (`KismetMathLibrary.BreakVector` (`self.K2_GetActorLocation` _returnvalue_4)))
  (bind _frontaxisvalue (`/Game/Blueprints/Controllers/BP_Player_Controller.FrontAxisValue` (`/Game/Blueprints/Library/BPFL_Fonction_Library.GetZombiePlayerController`)))
  (bind (_returnvalue_x_5 _returnvalue_y_5) (`KismetMathLibrary.BreakVector` (`SplineComponent.FindLocationClosestToWorldLocation` (`self.Spline`) _returnvalue_6 "World")))
  (bind (_returnvalue_x_6 _returnvalue_y_6) (`KismetMathLibrary.BreakVector` (`SplineComponent.FindLocationClosestToWorldLocation` (`self.Spline`) _returnvalue_5 "World")))
  (bind (_returnvalue_x_7 _returnvalue_y_7) (`KismetMathLibrary.BreakVector` (`SplineComponent.FindLocationClosestToWorldLocation` (`self.Spline`) (`KismetMathLibrary.MakeVector` _returnvalue_x _returnvalue_y _returnvalue_z) "World")))
  (bind (_returnvalue_x_8 _returnvalue_y_8) (`KismetMathLibrary.BreakVector` (`SplineComponent.FindLocationClosestToWorldLocation` (`self.Spline`) (`KismetMathLibrary.MakeVector` _returnvalue_x_2 _returnvalue_y_2 _returnvalue_z_2) "World")))
  (bind (_returnvalue_x_9 _returnvalue_y_9) (`KismetMathLibrary.BreakVector` (`SplineComponent.FindLocationClosestToWorldLocation` (`self.Spline`) (`KismetMathLibrary.MakeVector` _returnvalue_x_3 _returnvalue_y_3 _returnvalue_z_3) "World")))
  (bind (_returnvalue_x_10 _returnvalue_y_10) (`KismetMathLibrary.BreakVector` (`SplineComponent.FindLocationClosestToWorldLocation` (`self.Spline`) (`KismetMathLibrary.MakeVector` _returnvalue_x_4 _returnvalue_y_4 _returnvalue_z_4) "World")))
  (set `self.Delta Seconds` DeltaSeconds)
  (if (`/Game/Blueprints/Controllers/BP_Player_Controller.Railed` _asbp_player_controller)
    (if (== (`/Game/Blueprints/Controllers/BP_Player_Controller.ActiveRail` _asbp_player_controller) self)
      (if (!= _frontaxisvalue 0.0)
        (if (< _frontaxisvalue 0.0)
          (if (> _returnvalue_y_5 (.y _returnvalue_6))
            (set `/Game/Blueprints/Controllers/BP_Player_Controller.CoefReduc` 0.5 (`/Game/Blueprints/Library/BPFL_Fonction_Library.GetZombiePlayerController`) :!label _label)
            (else
              (set `/Game/Blueprints/Controllers/BP_Player_Controller.CoefReduc` 1.0 (`/Game/Blueprints/Library/BPFL_Fonction_Library.GetZombiePlayerController`))
              (`self.K2_SetActorLocation` _returnvalue_4 (`KismetMathLibrary.VInterpTo_Constant` (`self.K2_GetActorLocation` _returnvalue_4) (`KismetMathLibrary.MakeVector` _returnvalue_x_4 _returnvalue_y_10 _returnvalue_z_4) (`self.Delta Seconds`) 75.0) false false)))
          (elif (> (`/Game/Blueprints/Controllers/BP_Player_Controller.FrontAxisValue` (`/Game/Blueprints/Library/BPFL_Fonction_Library.GetZombiePlayerController`)) 0.0)
            (if (< _returnvalue_y_6 (.y _returnvalue_5))
              (goto _label)
              (else
                (set `/Game/Blueprints/Controllers/BP_Player_Controller.CoefReduc` 1.0 (`/Game/Blueprints/Library/BPFL_Fonction_Library.GetZombiePlayerController`))
                (`self.K2_SetActorLocation` _returnvalue (`KismetMathLibrary.VInterpTo_Constant` (`self.K2_GetActorLocation` _returnvalue) (`KismetMathLibrary.MakeVector` _returnvalue_x _returnvalue_y_7 _returnvalue_z) (`self.Delta Seconds`) 75.0) false false)))
            (else
              (set `/Game/Blueprints/Controllers/BP_Player_Controller.CoefReduc` 1.0 (`/Game/Blueprints/Library/BPFL_Fonction_Library.GetZombiePlayerController`))
              (`self.K2_SetActorLocation` _returnvalue_3 (`KismetMathLibrary.VInterpTo_Constant` (`self.K2_GetActorLocation` _returnvalue_3) (`KismetMathLibrary.MakeVector` _returnvalue_x_3 _returnvalue_y_9 _returnvalue_z_3) (`self.Delta Seconds`) 75.0) false false))))
        (else
          (set `/Game/Blueprints/Controllers/BP_Player_Controller.CoefReduc` 1.0 (`/Game/Blueprints/Library/BPFL_Fonction_Library.GetZombiePlayerController`))
          (`self.K2_SetActorLocation` _returnvalue_2 (`KismetMathLibrary.VInterpTo_Constant` (`self.K2_GetActorLocation` _returnvalue_2) (`KismetMathLibrary.MakeVector` _returnvalue_x_2 _returnvalue_y_8 _returnvalue_z_2) (`self.Delta Seconds`) 75.0) false false))))))

(event `self.Box.OnComponentBeginOverlap`
  (params (OverlappedComponent :type "PrimitiveComponent Object Reference") (OtherActor :type "Actor Object Reference") (OtherComp :type "PrimitiveComponent Object Reference") (OtherBodyIndex :type Integer) (bFromSweep :type Boolean) (SweepResult :type "HitResult Structure (by ref)"))
  (cast `/Game/Blueprints/Characters/BP_Character_Base` OtherActor)
  (`/Game/Blueprints/Controllers/BP_Player_Controller.SetRailed` (`/Game/Blueprints/Library/BPFL_Fonction_Library.GetZombiePlayerController`) true))

(event `self.Box.OnComponentEndOverlap`
  (params (OverlappedComponent :type "PrimitiveComponent Object Reference") (OtherActor :type "Actor Object Reference") (OtherComp :type "PrimitiveComponent Object Reference") (OtherBodyIndex :type Integer))
  (bind _asbp_player_controller (`/Game/Blueprints/Library/BPFL_Fonction_Library.GetZombiePlayerController`))
  (cast `/Game/Blueprints/Characters/BP_Character_Base` OtherActor)
  (set `/Game/Blueprints/Controllers/BP_Player_Controller.CoefReduc` 1.0 _asbp_player_controller)
  (`/Game/Blueprints/Controllers/BP_Player_Controller.SetRailed` _asbp_player_controller false))

(fn `UserConstructionScript`)