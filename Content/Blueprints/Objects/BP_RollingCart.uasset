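; BP_RollingCart is a cart object whose wheels spin when its roule event fires.
; The construction script gathers the four wheel components into a Wheels array.
; The roule event plays the Roulle timeline from the start, and each update adds a relative roll rotation to every wheel, scaled from the timeline's track value.
; The graph rotates only the wheels and does not move the cart itself.
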(event `roule`
  (bind (_direction _newtrack_0) (`Timeline|roulle` :!via `PlayFromStart`)
    (:`Update`
      (for _array_element (`self.Wheels`)
        (`SceneComponent.K2_AddRelativeRotation` _array_element (`KismetMathLibrary.MakeRotator` (* _newtrack_0 15.0)) false false)))))

(fn `UserConstructionScript`
  (bind _wheels (`self.Wheels`))
  (`KismetArrayLibrary.Array_Add` _wheels (`self.Wheel`))
  (`KismetArrayLibrary.Array_Add` _wheels (`self.Wheel1`))
  (`KismetArrayLibrary.Array_Add` _wheels (`self.Wheel2`))
  (`KismetArrayLibrary.Array_Add` _wheels (`self.Wheel3`)))