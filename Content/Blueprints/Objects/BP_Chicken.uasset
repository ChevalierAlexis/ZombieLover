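; BP_Chicken is a flipbook-based chicken object that can carry a key or a decorative object in its beak.
; The construction script snaps an assigned key to the sprite's Beak socket, offsets its capsule, and disables the key and its interaction-range collision.
; Without a valid key, it shows the optional ObjectToAttach flipbook at that socket instead.
; The event graph has no active logic; its delayed rooster-crow chain is disconnected.
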(event `self.ReceiveBeginPlay`)

(fn `UserConstructionScript`
  (bind _keytoattach (`self.KeyToAttach`))
  (bind _objecttoattach (`self.ObjectToAttach`))
  (bind _keytoattach_2 (`self.KeyToAttach`))
  (`/Engine/EditorBlueprintResources/StandardMacros.IsValid` _keytoattach
    (:`Is Valid`
      (`self.K2_AttachToComponent` _keytoattach (`self.Sprite`) "Beak" "SnapToTarget" "SnapToTarget" "SnapToTarget" true)
      (`SceneComponent.K2_SetRelativeLocation` (`/Game/Blueprints/Objects/InputObjects/BP_Key.Capsule` _keytoattach_2) (5.0 1.0 0.0) false false)
      (set `/Game/Blueprints/Objects/InputObjects/BP_Key.Enabled` false _keytoattach_2)
      (`PrimitiveComponent.SetCollisionEnabled` (`/Game/Blueprints/Objects/InputObjects/BP_Interactable.InteractionRange` _keytoattach_2) "NoCollision"))
    (:`Is Not Valid`
      (`/Engine/EditorBlueprintResources/StandardMacros.IsValid` _objecttoattach
        (:`Is Valid`
          (`PaperFlipbookComponent.SetFlipbook` (`self.ToAttach`) _objecttoattach)
          (`SceneComponent.K2_AttachToComponent` (`self.ToAttach`) (`self.Sprite`) "Beak" "SnapToTarget" "SnapToTarget" "SnapToTarget" true))))))