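; BP_Flower00 is a collectible flower that is picked up when a player activates it.
; The construction script takes its Paper2D sprite from FlowerType.
; Activation calls the parent behavior, marks FlowerType as obtained, then hides the actor and disables its collision instead of destroying it.
; On BeginPlay it binds to BPRespawnAC, whose respawn event clears the obtained flag and restores visibility and collision.
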(event `self.ReceiveBeginPlay`
  (add `/Game/Blueprints/Characters/Components/BP_Respawn_AC.Respawn` (`self.BP_Respawn_AC`) (delegate `RespawnEvent`)))

(event `RespawnEvent`
  (set `/Game/Blueprints/Data/BP_DA_Flower.Obtained` false (`self.FlowerType`))
  (`self.SetActorHiddenInGame` false)
  (`self.SetActorEnableCollision` true))

(fn `Activation`
  (params (PlayerWhoActivated :type "/Game/Blueprints/Characters/BP_Character_Base Object Reference"))
  (`parent.Activation` PlayerWhoActivated)
  (set `/Game/Blueprints/Data/BP_DA_Flower.Obtained` true (`self.FlowerType`))
  (`self.SetActorHiddenInGame` true)
  (`self.SetActorEnableCollision` false))

(fn `UserConstructionScript`
  (`PaperSpriteComponent.SetSprite` (`self.PaperSprite`) (`/Game/Blueprints/Data/BP_DA_Flower.Sprite` (`self.FlowerType`))))