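; BP_Box is a grabbable box that shows an A-button prompt (ToucheA) when the player character is nearby.
; It extends a parent Blueprint and sets its BPCDeath component to instant respawn at BeginPlay.
; InteractionRange overlaps with BP_Character_Full toggle the prompt's visibility.
; RemoveA hides the prompt on demand, while MakeVisibleA rechecks current overlaps to show it again.
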(event `self.ReceiveBeginPlay`
  (`parent.ReceiveBeginPlay`)
  (set `/Game/Blueprints/Characters/Components/BPC_Death.DoInstantRespawn` true (`self.BPC_Death`)))

(event `self.ReceiveTick`
  (params (DeltaSeconds :type "Float (single-precision)"))
  (`parent.ReceiveTick` 0.0))

(event `self.InteractionRange.OnComponentBeginOverlap`
  (params (OverlappedComponent :type "PrimitiveComponent Object Reference") (OtherActor :type "Actor Object Reference") (OtherComp :type "PrimitiveComponent Object Reference") (OtherBodyIndex :type Integer) (bFromSweep :type Boolean) (SweepResult :type "HitResult Structure (by ref)"))
  (cast `/Game/Blueprints/Characters/BP_Character_Full` OtherActor)
  (`SceneComponent.SetVisibility` (`self.ToucheA`) true false))

(event `self.InteractionRange.OnComponentEndOverlap`
  (params (OverlappedComponent :type "PrimitiveComponent Object Reference") (OtherActor :type "Actor Object Reference") (OtherComp :type "PrimitiveComponent Object Reference") (OtherBodyIndex :type Integer))
  (cast `/Game/Blueprints/Characters/BP_Character_Full` OtherActor)
  (`SceneComponent.SetVisibility` (`self.ToucheA`) false false))

(event `RemoveA`
  (`SceneComponent.SetVisibility` (`self.ToucheA`) false false))

(event `MakeVisibleA`
  (for _array_element (`PrimitiveComponent.GetOverlappingActors` (`self.InteractionRange`) null)
    (cast `/Game/Blueprints/Characters/BP_Character_Full` _array_element)
    (`SceneComponent.SetVisibility` (`self.ToucheA`) true false)))

(fn `UserConstructionScript`
  (`parent.UserConstructionScript`))