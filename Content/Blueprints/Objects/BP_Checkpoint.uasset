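; Checkpoint actor that records itself as the active respawn point and can teleport a target back to it.
; When a BP_Character_Base overlaps its box, it stores itself as CheckPoint on the camera manager, unless already set.
; TpToCheckPoint moves the target to the flipbook's location, then calls InstantCamUpdate on the linked camera trigger, if valid, to update the camera instantly.
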(event `self.Box.OnComponentBeginOverlap`
  (params (OverlappedComponent :type "PrimitiveComponent Object Reference") (OtherActor :type "Actor Object Reference") (OtherComp :type "PrimitiveComponent Object Reference") (OtherBodyIndex :type Integer) (bFromSweep :type Boolean) (SweepResult :type "HitResult Structure (by ref)"))
  (cast `/Game/Blueprints/Characters/BP_Character_Base` OtherActor)
  (bind (_asbp_camera_manager _pawntarget _uideathref _uicontrol _checkpoint) (`/Game/Blueprints/Library/BPFL_Fonction_Library.GetCameraManager`))
  (if (not (== self _checkpoint))
    (bind _output_get (set `/Game/Blueprints/BP_Camera_Manager.CheckPoint` self _asbp_camera_manager))))

(event `TpToCheckPoint`
  (params (Target :type "Actor Object Reference"))
  (bind _camtriggerref (`self.CamTriggerRef`))
  (`self.K2_SetActorLocation` Target (`SceneComponent.K2_GetComponentLocation` (`self.PaperFlipbook`)) false false)
  (`KismetSystemLibrary.PrintString` (`KismetSystemLibrary.GetDisplayName` _camtriggerref))
  (`/Engine/EditorBlueprintResources/StandardMacros.IsValid` _camtriggerref
    (:`Is Valid`
      (`/Game/Blueprints/Objects/BP_CameraTrigger.InstantCamUpdate` _camtriggerref (`/Game/Blueprints/Library/BPFL_Fonction_Library.CastToPlayerCharacter`)))))

(fn `UserConstructionScript`)