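; BP_TP is a teleporter pad that sends characters of a chosen class (ClassToTp) to a linked Target pad.
; While off cooldown, Tick pulls the nearest matching character toward the plate and teleports it once close enough.
; The receiving pad places it above its plate, spawns a shockwave and launches it onward, with both pads cooling down briefly.
; The construction script tints vortex and sprite by class and toggles plate visibility.
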(event `self.ReceiveTick`
  (params (DeltaSeconds :type "Float (single-precision)"))
  (bind _returnvalue (`SceneComponent.K2_GetComponentLocation` (`self.PlateMesh`)))
  (if (<= (`self.CoolDown`) 0.0)
    (bind (_returnvalue_2 _distance) (`/Game/Blueprints/Library/BPFL_Fonction_Library.FindNearestActorOfClass` (`self.ClassToTp`) _returnvalue))
    (`/Engine/EditorBlueprintResources/StandardMacros.IsValid` _returnvalue_2
      (:`Is Valid`
        (if (and (<= _distance 40.0) (`KismetSystemLibrary.IsValid` (`self.Target`)))
          (bind _asbp_character_base (cast `/Game/Blueprints/Characters/BP_Character_Base` _returnvalue_2))
          (bind _returnvalue_3 (`KismetMathLibrary.GetDirectionUnitVector` (`self.K2_GetActorLocation` _returnvalue_2) _returnvalue))
          (`CharacterMovementComponent.AddForce` (`Character.CharacterMovement` _asbp_character_base) (* _returnvalue_3 400000.0))
          (if (<= _distance 27.0)
            (`self.TP_To` (`self.Target`) _asbp_character_base _returnvalue_3)))))
    (else
      (set `self.CoolDown` (`KismetMathLibrary.FClamp` (- (`self.CoolDown`) DeltaSeconds) 0.0 100.0)))))

(event `StartCoolDown`
  (params (CoolDown :type "Float (double-precision)"))
  (set `self.CoolDown` CoolDown))

(event `TP_To`
  (params (Tp_Target :type "Self Object Reference") (ActorToTp :type "Actor Object Reference") (LaunchDirection :type "Vector Structure"))
  (`/Engine/EditorBlueprintResources/StandardMacros.IsValid` Tp_Target
    (:`Is Valid`
      (`self.StartCoolDown` 0.5)
      (`self.Tp_In` Tp_Target ActorToTp LaunchDirection))))

(event `Tp_In`
  (params (ActorToTp :type "Actor Object Reference") (LaunchDirection :type "Vector Structure"))
  (bind _returnvalue (`self.GetComponentByClass` ActorToTp "/Script/Engine.StaticMeshComponent"))
  (bind (_returnvalue_x _returnvalue_y _returnvalue_z) (`KismetMathLibrary.BreakVector` (`SceneComponent.K2_GetComponentLocation` (`self.PlateMesh`))))
  (bind _returnvalue_2 (* (`KismetMathLibrary.MakeVector` LaunchDirection_X LaunchDirection_Y (/ 200.0 200.0)) 200.0))
  (`self.StartCoolDown` 0.5)
  (`self.K2_SetActorLocation` ActorToTp (`KismetMathLibrary.MakeVector` _returnvalue_x _returnvalue_y (+ _returnvalue_z 5.0)) false true)
  (`NiagaraFunctionLibrary.SpawnSystemAtLocation` "/Game/FX/Zombie/NS_ShockWave.NS_ShockWave" (`SceneComponent.K2_GetComponentLocation` (`self.Sphere`)))
  (bind _ascharacter (cast `Character` ActorToTp)
    (:`then`
      (`Character.LaunchCharacter` _ascharacter _returnvalue_2 false true))
    (:`CastFailed`
      (if (`SceneComponent.IsSimulatingPhysics` _returnvalue "None")
        (`PrimitiveComponent.AddImpulse` _returnvalue (* _returnvalue_2 100.0) "None" false)))))

(fn `UserConstructionScript`
  (bind _classtotp (`self.ClassToTp`))
  (bind _platemesh (`self.PlateMesh`))
  (bind _returnvalue (`KismetMathLibrary.SelectColor` (struct :`R` 1.0 :`G` 1.0 :`B` 1.0 :`A` 1.0) (`KismetMathLibrary.SelectColor` (struct :`R` 0.397272 :`B` 0.703125 :`A` 1.0) (`KismetMathLibrary.SelectColor` (struct :`R` 0.578125 :`B` 0.010615 :`A` 1.0) (struct :`G` 0.259723 :`B` 0.65625 :`A` 1.0) (== _classtotp "/Game/Blueprints/Characters/BP_Character_Top.BP_Character_Top_C")) (== _classtotp "/Game/Blueprints/Characters/BP_Character_Full.BP_Character_Full_C")) (== _classtotp "/Game/Blueprints/Characters/BP_Character_Base.BP_Character_Base_C")))
  (bind _returnvalue_2 (`PrimitiveComponent.CreateDynamicMaterialInstance` (`self.Sphere`) 0 "/Game/Materials/FX/Vortex/M_Vortex.M_Vortex" "None"))
  (bind _output_get (set `self.MaterialSphere` _returnvalue_2))
  (`MaterialInstanceDynamic.SetVectorParameterValue` _output_get "Color" _returnvalue)
  (`PaperSpriteComponent.SetSpriteColor` (`self.PaperSprite`) _returnvalue)
  (if (`self.Plate`)
    (`SceneComponent.SetVisibility` _platemesh true false)
    (else
      (`SceneComponent.SetVisibility` _platemesh false false))))