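; BP_Skulltorches is a skull torch prop whose point light flickers continuously during play.
; A looping timeline lerps the light's intensity toward a random target within a fixed range, then picks a new target from the current intensity each time it finishes.
; BeginPlay also caches the relative transform of LightPosition0, though the graph never uses it.
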(event `self.ReceiveBeginPlay`
  (bind _returnvalue (`KismetMathLibrary.RandomFloatInRange` 400.0 600.0))
  (set `self.baseLightIntensity` 500.0)
  (set `self.targetLightIntensity` _returnvalue)
  (set `self.baseLightTransform` (`SceneComponent.GetRelativeTransform` (`self.LightPosition_0`)))
  ;[1 1 1] Intensity loop
  (bind (_direction _height) (`Timeline|Timeline` :!label _label)
    (:`Update`
      (`LightComponent.SetIntensity` (`self.PointLight`) (`KismetMathLibrary.Lerp` (stale _output_get_2) (stale _output_get) _height)))
    (:`Finished`
      (bind _output_get (set `self.targetLightIntensity` _returnvalue))
      (bind _output_get_2 (set `self.baseLightIntensity` (`LightComponentBase.Intensity` (`self.PointLight`))))
      (goto _label :!via `PlayFromStart`))))

(event `self.ReceiveTick`
  (params (DeltaSeconds :type "Float (single-precision)")))

(fn `UserConstructionScript`)