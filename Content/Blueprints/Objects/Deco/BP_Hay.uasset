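; BP_Hay is a decorative hay object that squashes and puffs particles when a BP_Character_Base moves downward into its box.
; The box overlap checks for negative vertical velocity, then fires a DoOnce that plays the Squeeze timeline to widen and flatten the mesh's scale.
; It also spawns a Niagara hay effect at the box, and a short delayed reset re-arms the DoOnce as a cooldown.
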(event `reset`
  (goto _label :!via `Reset`))

(event `self.Box.OnComponentBeginOverlap`
  (params (OverlappedComponent :type "PrimitiveComponent Object Reference") (OtherActor :type "Actor Object Reference") (OtherComp :type "PrimitiveComponent Object Reference") (OtherBodyIndex :type Integer) (bFromSweep :type Boolean) (SweepResult :type "HitResult Structure (by ref)"))
  (bind _asbp_character_base (cast `/Game/Blueprints/Characters/BP_Character_Base` OtherActor))
  (bind (_returnvalue_x _returnvalue_y _returnvalue_z) (`KismetMathLibrary.BreakVector` (`self.GetVelocity` _asbp_character_base)))
  (if (< _returnvalue_z -0.2)
    (`/Engine/EditorBlueprintResources/StandardMacros.DoOnce` false :!label _label
      (:`Completed`
        (`|ExecutionSequence`
          (:`then_0`
            (`TimelineComponent.SetPlayRate` (`self.Squeeze`) 2.5)
            (bind (_direction _alpha) (`Timeline|Squeeze` :!via `PlayFromStart`)
              (:`Update`
                (`SceneComponent.SetRelativeScale3D` (`self.StaticMesh`) (`KismetMathLibrary.VLerp` (1.0 1.0 1.0) (1.2 1.2 0.8) _alpha)))))
          (:`then_1`
            (`NiagaraFunctionLibrary.SpawnSystemAtLocation` "/Game/FX/NS_HayParticle.NS_HayParticle" (`SceneComponent.K2_GetComponentLocation` (`self.Box`)))
            (`KismetSystemLibrary.Delay` 0.5)
            (`self.reset`)))))))

(fn `UserConstructionScript`)