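; Decorative skull torch that shows a flickering point light and fire effect, and can be switched on or off.
; A looping timeline blends the light intensity toward a random target, then picks a new one from the current value for continuous flicker.
; Activated and Deactivated toggle light and fire visibility through IsOff, which can also start the torch unlit.
; The flicker loop keeps running while hidden.
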(event `self.ReceiveBeginPlay`
  (bind _returnvalue (`KismetMathLibrary.RandomFloatInRange` 30.0 60.0))
  (if (`self.IsOff`)
    (`SceneComponent.SetVisibility` (`self.PointLight`) false false)
    (`SceneComponent.SetVisibility` (`self.NE_Torch_Fire`) false false))
  (set `self.targetLightIntensity` _returnvalue)
  (set `self.baseLightTransform` (`SceneComponent.GetRelativeTransform` (`self.LightPosition_0`)))
  ;[1 1 1] Intensity loop
  (bind (_direction _height) (`Timeline|Timeline` :!label _label)
    (:`Update`
      (`LightComponent.SetIntensity` (`self.PointLight`) (`KismetMathLibrary.Lerp` (stale _output_get_2) (stale _output_get) _height)))
    (:`Finished`
      (bind _output_get (set `self.targetLightIntensity` _returnvalue))
      (bind _output_get_2 (set `self.baseLightIntensity` (`LightComponentBase.Intensity` (`self.PointLight`))))
      (goto _label :!via `PlayFromStart`))))

(event `self.ReceiveTick`
  (params (DeltaSeconds :type "Float (single-precision)")))

(fn `Activated`
  (if (`self.IsOff`)
    (set `self.IsOff` false)
    (`SceneComponent.SetVisibility` (`self.PointLight`) true false)
    (`SceneComponent.SetVisibility` (`self.NE_Torch_Fire`) true false)))

(fn `Deactivated`
  (if (not (`self.IsOff`))
    (set `self.IsOff` true)
    (`SceneComponent.SetVisibility` (`self.PointLight`) false false)
    (`SceneComponent.SetVisibility` (`self.NE_Torch_Fire`) false false)))

(fn `UserConstructionScript`)