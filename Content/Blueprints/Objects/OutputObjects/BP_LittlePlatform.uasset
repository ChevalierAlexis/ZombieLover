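; BP_LittlePlatform is an output object: a platform that rotates on its pivot when activated and swings back when deactivated.
; The Activated and Deactivated functions call events that play or reverse the Bridge timeline.
; The timeline's Rotation track lerps the Pivot's relative pitch from the value cached at BeginPlay to TargetYRotation, holding roll and yaw at zero.
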(event `self.ReceiveBeginPlay`
  (bind (_relativerotation_roll _relativerotation_pitch) (`KismetMathLibrary.BreakRotator` (`SceneComponent.RelativeRotation` (`self.Pivot`))))
  (set `self.OriginalYRotation` _relativerotation_pitch))

(event `Activation`
  (bind (_direction _rotation) (`Timeline|Bridge` :!label _label)
    (:`Update`
      (`SceneComponent.K2_SetRelativeRotation` (`self.Pivot`) (`KismetMathLibrary.MakeRotator` 0.0 (`KismetMathLibrary.Lerp` (`self.OriginalYRotation`) (`self.TargetYRotation`) _rotation)) false false))))

(event `Deactivation`
  (goto _label :!via `Reverse`))

(fn `Activated`
  (`self.Activation`))

(fn `Deactivated`
  (`self.Deactivation`))

(fn `UserConstructionScript`
  (`parent.UserConstructionScript`))