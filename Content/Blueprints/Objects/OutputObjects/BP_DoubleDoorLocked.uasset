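; BP_DoubleDoorLocked is an output-object double door that only passes interaction to its parent when not locked.
; Activation and Deactivation open and close it, playing data-table sounds while timelines lerp both panels' yaw between stored starting and target rotations, opening at double play rate.
; An InteractionRange overlap shows the Lock component while a BP_Character_Base is nearby and the door is locked, hiding it on exit.
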(event `self.ReceiveBeginPlay`
  (bind (_relativerotation_roll _relativerotation_pitch _relativerotation_yaw) (`KismetMathLibrary.BreakRotator` (`SceneComponent.RelativeRotation` (`self.Cube1`))))
  (bind (_relativerotation_roll_2 _relativerotation_pitch_2 _relativerotation_yaw_2) (`KismetMathLibrary.BreakRotator` (`SceneComponent.RelativeRotation` (`self.Cube`))))
  (set `self.Original ZRotation` _relativerotation_yaw_2)
  (set `self.Original ZRotation2` _relativerotation_yaw))

(event `OpenDoor`
  (bind _returnvalue (`|GetDataTableRow` "/Game/Sound/DT_Sound_List.DT_Sound_List" "A_Door_Open")
    (:`then`
      (`GameplayStatics.PlaySound2D` (break `/Game/Blueprints/Structures/SSound` _returnvalue) 1.0 1.0 0.0 null null)
      (`TimelineComponent.SetPlayRate` (`self.DoorOpenTimeline`) 2.0)
      (bind (_direction _height) (`Timeline|DoorOpenTimeline` :!via `PlayFromStart`)
        (:`Update`
          (`SceneComponent.K2_SetRelativeRotation` (`self.Cube`) (`KismetMathLibrary.MakeRotator` 0.0 0.0 (`KismetMathLibrary.Lerp` (`self.Original ZRotation`) (`self.TargetZRotation`) _height)) false false)
          (`SceneComponent.K2_SetRelativeRotation` (`self.Cube1`) (`KismetMathLibrary.MakeRotator` 0.0 0.0 (`KismetMathLibrary.Lerp` (`self.Original ZRotation2`) (`self.TargetZRotation2`) _height)) false false))))))

(event `CloseDoor`
  (bind _returnvalue (`|GetDataTableRow` "/Game/Sound/DT_Sound_List.DT_Sound_List" "A_Door_Close")
    (:`then`
      (`GameplayStatics.PlaySound2D` (break `/Game/Blueprints/Structures/SSound` _returnvalue) 1.0 1.0 0.0 null null)
      (`TimelineComponent.SetPlayRate` (`self.DoorCloseTimeline`) 1.0)
      (bind (_direction _height) (`Timeline|DoorCloseTimeline` :!via `PlayFromStart`)
        (:`Update`
          (`SceneComponent.K2_SetRelativeRotation` (`self.Cube`) (`KismetMathLibrary.MakeRotator` 0.0 0.0 (`KismetMathLibrary.Lerp` (`self.TargetZRotation`) (`self.Original ZRotation`) _height)) false false)
          (`SceneComponent.K2_SetRelativeRotation` (`self.Cube1`) (`KismetMathLibrary.MakeRotator` 0.0 0.0 (`KismetMathLibrary.Lerp` (`self.TargetZRotation2`) (`self.Original ZRotation2`) _height)) false false))))))

(event `self.InteractionRange.OnComponentBeginOverlap`
  (params (OverlappedComponent :type "PrimitiveComponent Object Reference") (OtherActor :type "Actor Object Reference") (OtherComp :type "PrimitiveComponent Object Reference") (OtherBodyIndex :type Integer) (bFromSweep :type Boolean) (SweepResult :type "HitResult Structure (by ref)"))
  (cast `/Game/Blueprints/Characters/BP_Character_Base` OtherActor)
  (if (`self.IsLocked`)
    (`SceneComponent.SetVisibility` (`self.Lock`) true false)
    (else
      (`SceneComponent.SetVisibility` (`self.Lock`) false false))))

(event `self.InteractionRange.OnComponentEndOverlap`
  (params (OverlappedComponent :type "PrimitiveComponent Object Reference") (OtherActor :type "Actor Object Reference") (OtherComp :type "PrimitiveComponent Object Reference") (OtherBodyIndex :type Integer))
  (cast `/Game/Blueprints/Characters/BP_Character_Base` OtherActor)
  (if (`self.IsLocked`)
    (`SceneComponent.SetVisibility` (`self.Lock`) false false)
    (else
      (`SceneComponent.SetVisibility` (`self.Lock`) false false))))

(fn `Activation`
  (params (PlayerWhoActivated :type "/Game/Blueprints/Characters/BP_Character_Base Object Reference"))
  (`self.OpenDoor`))

(fn `Deactivation`
  (params (PlayerWhoActivated :type "/Game/Blueprints/Characters/BP_Character_Base Object Reference") (A :type Boolean))
  (`self.CloseDoor`))

(fn `Interract`
  (if (not (`self.IsLocked`))
    (`parent.Interract`)))

(fn `UserConstructionScript`
  (`parent.UserConstructionScript`))