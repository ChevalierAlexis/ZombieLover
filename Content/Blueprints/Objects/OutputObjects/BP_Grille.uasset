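; BP_Grille is an output object, a grille that slides vertically when activated and returns when deactivated.
; Activated and Deactivated forward to events that play a timeline forward or in reverse.
; The timeline's Height track lerps the Cube's relative Z between its BeginPlay position and TargetZPosition.
; Opening runs at normal rate, while closing uses ClosingTime directly as the play rate.
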(event `self.ReceiveBeginPlay`
  (bind (_relativelocation_x _relativelocation_y _relativelocation_z) (`KismetMathLibrary.BreakVector` (`SceneComponent.RelativeLocation` (`self.Cube`))))
  (set `self.Original ZPosition` _relativelocation_z))

(event `Activation`
  (`TimelineComponent.SetPlayRate` (`self.GrilleOpenTimeline`) 1.0)
  (bind (_direction _height) (`Timeline|GrilleOpenTimeline` :!via `PlayFromStart` :!label _label)
    (:`Update`
      (`SceneComponent.K2_SetRelativeLocation` (`self.Cube`) (`KismetMathLibrary.MakeVector` 0.0 0.0 (`KismetMathLibrary.Lerp` (`self.Original ZPosition`) (`self.TargetZPosition`) _height)) false false))))

(event `Deactivation`
  (`TimelineComponent.SetPlayRate` (`self.GrilleOpenTimeline`) (`self.ClosingTime`))
  (goto _label :!via `Reverse`))

(fn `Activated`
  (`self.Activation`))

(fn `Deactivated`
  (`self.Deactivation`))

(fn `UserConstructionScript`
  (`parent.UserConstructionScript`))