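; BP_Door is an output object that swings open when activated and swings back when deactivated.
; The Activated and Deactivated functions trigger events that play or reverse a timeline, lerping the mesh's yaw from its starting value to a target.
; Each event first plays a 2D sound from DT_Sound_List, moving only if the row is found.
; The construction script applies the configurable static mesh and its first material.
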(event `self.ReceiveBeginPlay`
  (bind (_relativerotation_roll _relativerotation_pitch _relativerotation_yaw) (`KismetMathLibrary.BreakRotator` (`SceneComponent.RelativeRotation` (`self.Cube`))))
  (set `self.Original ZRotation` _relativerotation_yaw))

(event `Activation`
  (bind _returnvalue (`|GetDataTableRow` "/Game/Sound/DT_Sound_List.DT_Sound_List" "A_Door_Open")
    (:`then`
      (`GameplayStatics.PlaySound2D` (break `/Game/Blueprints/Structures/SSound` _returnvalue) 1.0 1.0 0.0 null null)
      (`TimelineComponent.SetPlayRate` (`self.DoorOpenTimeline`) 1.0)
      (bind (_direction _height) (`Timeline|DoorOpenTimeline` :!label _label)
        (:`Update`
          (`SceneComponent.K2_SetRelativeRotation` (`self.Cube`) (`KismetMathLibrary.MakeRotator` 0.0 0.0 (`KismetMathLibrary.Lerp` (`self.Original ZRotation`) (`self.TargetZRotation`) _height)) false false))))))

(event `Deactivation`
  (bind _returnvalue (`|GetDataTableRow` "/Game/Sound/DT_Sound_List.DT_Sound_List" "A_Levier_Activation")
    (:`then`
      (`GameplayStatics.PlaySound2D` (break `/Game/Blueprints/Structures/SSound` _returnvalue) 1.0 1.0 0.0 null null)
      (`TimelineComponent.SetPlayRate` (`self.DoorOpenTimeline`) 1.0)
      (goto _label :!via `Reverse`))))

(fn `Activated`
  (`self.Activation`))

(fn `Deactivated`
  (`self.Deactivation`))

(fn `UserConstructionScript`
  (bind _staticmesh (`self.StaticMesh`))
  (`parent.UserConstructionScript`)
  (`StaticMeshComponent.SetStaticMesh` (`self.Cube`) _staticmesh)
  (`PrimitiveComponent.SetMaterial` (`self.Cube`) 0 (`StaticMesh.GetMaterial` _staticmesh 0)))