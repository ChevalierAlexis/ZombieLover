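; BP_DoorLocked is a door output object that swings open on Activation and closed on Deactivation.
; A timeline lerps the Cube's yaw between its rotation at BeginPlay and a target angle, playing in reverse to close.
; Opening and closing play 2D sounds from a data table, and the timeline only runs if the row is found.
; Interract defers to the parent only when the door is not locked.
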(event `self.ReceiveBeginPlay`
  (bind (_relativerotation_roll _relativerotation_pitch _relativerotation_yaw) (`KismetMathLibrary.BreakRotator` (`SceneComponent.RelativeRotation` (`self.Cube`))))
  (set `self.Original ZRotation` _relativerotation_yaw))

(event `OpenDoor`
  (bind _returnvalue (`|GetDataTableRow` "/Game/Sound/DT_Sound_List.DT_Sound_List" "A_Door_Open")
    (:`then`
      (`GameplayStatics.PlaySound2D` (break `/Game/Blueprints/Structures/SSound` _returnvalue) 1.0 1.0 0.0 null null)
      (`TimelineComponent.SetPlayRate` (`self.DoorOpenTimeline`) 1.0)
      (bind (_direction _height) (`Timeline|DoorOpenTimeline` :!label _label)
        (:`Update`
          (`SceneComponent.K2_SetRelativeRotation` (`self.Cube`) (`KismetMathLibrary.MakeRotator` 0.0 0.0 (`KismetMathLibrary.Lerp` (`self.Original ZRotation`) (`self.TargetZRotation`) _height)) false false))))))

(event `CloseDoor`
  (bind _returnvalue (`|GetDataTableRow` "/Game/Sound/DT_Sound_List.DT_Sound_List" "A_Door_Close")
    (:`then`
      (`GameplayStatics.PlaySound2D` (break `/Game/Blueprints/Structures/SSound` _returnvalue) 1.0 1.0 0.0 null null)
      (`TimelineComponent.SetPlayRate` (`self.DoorOpenTimeline`) 1.0)
      (goto _label :!via `Reverse`))))

(fn `Activation`
  (`self.OpenDoor`))

(fn `Deactivation`
  (`self.CloseDoor`))

(fn `Interract`
  (if (not (`self.IsLocked`))
    (`parent.Interract`)))

(fn `UserConstructionScript`
  (`parent.UserConstructionScript`))