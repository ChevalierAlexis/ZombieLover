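; Catapult output object that swings its arm and launches characters standing in its trigger box when activated.
; Activation plays a timeline that lerps the arm's pitch from its starting value to the target angle, then launches every tracked character with the configured impulse, overriding vertical velocity.
; Deactivation slowly reverses the same timeline, with a flag preventing a launch when the return finishes.
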(event `self.ReceiveBeginPlay`
  (bind (_relativerotation_roll _relativerotation_pitch) (`KismetMathLibrary.BreakRotator` (`SceneComponent.RelativeRotation` (`self.Arm`))))
  (set `self.Origin Y Rotation` _relativerotation_pitch))

(event `Activation`
  (set `self.Launching` true)
  (`TimelineComponent.SetPlayRate` (`self.Launch`) (`self.Speed`))
  (bind (_direction _rotation) (`Timeline|Launch` :!label _label)
    (:`Update`
      (`SceneComponent.K2_SetRelativeRotation` (`self.Arm`) (`KismetMathLibrary.MakeRotator` 0.0 (`KismetMathLibrary.Lerp` (`self.Origin Y Rotation`) (`self.Angle`) _rotation)) false false))
    (:`Finished`
      (if (`self.Launching`)
        (for _array_element (`self.LaunchableTargets`)
          (bind _asbp_character_base (cast `/Game/Blueprints/Characters/BP_Character_Base` _array_element))
          (`Character.LaunchCharacter` _asbp_character_base (`self.Impulse`) false true))))))

(event `Deactivation`
  (set `self.Launching` false)
  (`TimelineComponent.SetPlayRate` (`self.Launch`) 0.1)
  (goto _label :!via `Reverse`))

(event `self.Box.OnComponentBeginOverlap`
  (params (OverlappedComponent :type "PrimitiveComponent Object Reference") (OtherActor :type "Actor Object Reference") (OtherComp :type "PrimitiveComponent Object Reference") (OtherBodyIndex :type Integer) (bFromSweep :type Boolean) (SweepResult :type "HitResult Structure (by ref)"))
  (`KismetArrayLibrary.Array_Add` (`self.LaunchableTargets`) OtherActor))

(event `self.Box.OnComponentEndOverlap`
  (params (OverlappedComponent :type "PrimitiveComponent Object Reference") (OtherActor :type "Actor Object Reference") (OtherComp :type "PrimitiveComponent Object Reference") (OtherBodyIndex :type Integer))
  (`KismetArrayLibrary.Array_RemoveItem` (`self.LaunchableTargets`) OtherActor))

(fn `Activated`
  (`self.Activation`))

(fn `Deactivated`
  (`self.Deactivation`))

(fn `UserConstructionScript`
  (`parent.UserConstructionScript`))