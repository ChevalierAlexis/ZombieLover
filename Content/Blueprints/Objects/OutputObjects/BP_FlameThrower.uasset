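; BP_FlameThrower is a flamethrower output object that sets cramable actors on fire.
; Its logic is inverted: Activated switches off the fire effect, light and eyes, while Deactivated switches them back on.
; While lit, actors entering the capsule get IsOnFire set on their BP_Cramable_AC component, and relighting also ignites actors already overlapping it.
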(event `GetCramed`
  (params (NewParam :type "Actor Object Reference"))
  (bind _returnvalue (`self.GetComponentByClass` NewParam "/Game/Blueprints/Characters/Components/BP_Cramable_AC.BP_Cramable_AC_C"))
  (`/Engine/EditorBlueprintResources/StandardMacros.IsValid` _returnvalue
    (:`Is Valid`
      (set `/Game/Blueprints/Characters/Components/BP_Cramable_AC.IsOnFire` true _returnvalue))))

(event `self.Capsule.OnComponentBeginOverlap`
  (params (OverlappedComponent :type "PrimitiveComponent Object Reference") (OtherActor :type "Actor Object Reference") (OtherComp :type "PrimitiveComponent Object Reference") (OtherBodyIndex :type Integer) (bFromSweep :type Boolean) (SweepResult :type "HitResult Structure (by ref)"))
  (if (`self.OnFire`)
    (`self.GetCramed` OtherActor)))

(fn `Activated`
  (params (Interactable :type "/Game/Blueprints/Objects/InputObjects/BP_Interactable Object Reference"))
  (`parent.Activated` Interactable)
  (`SceneComponent.SetVisibility` (`self.eye1`) false false)
  (`SceneComponent.SetVisibility` (`self.eye0`) false false)
  (`ActorComponent.Deactivate` (`self.Fire`))
  (`SceneComponent.SetVisibility` (`self.PointLight`) false true)
  (set `self.OnFire` false))

(fn `Deactivated`
  (params (Interactable :type "/Game/Blueprints/Objects/InputObjects/BP_Interactable Object Reference"))
  (`parent.Deactivated` Interactable)
  (`SceneComponent.SetVisibility` (`self.eye1`) true false)
  (`SceneComponent.SetVisibility` (`self.eye0`) true false)
  (`ActorComponent.Activate` (`self.Fire`) false)
  (`SceneComponent.SetVisibility` (`self.PointLight`) true true)
  (set `self.OnFire` true)
  (for _array_element (`PrimitiveComponent.GetOverlappingActors` (`self.Capsule`) null)
    (`self.GetCramed` _array_element)))

(fn `UserConstructionScript`
  (`parent.UserConstructionScript`))