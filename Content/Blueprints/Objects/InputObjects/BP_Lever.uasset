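; Lever input object that players switch on and off to drive the objects in its Target array.
; Activation and Deactivation play a 2D sound from DT_Sound_List, then start the animation only if the row is found.
; A timeline plays forward or reverse to lerp the lever's roll, ignoring requests while animating.
; On finish, it updates Triggered and calls Activated or Deactivated on every target.
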(event `self.ReceiveBeginPlay`
  (bind (_relativerotation_roll _relativerotation_pitch _relativerotation_yaw) (`KismetMathLibrary.BreakRotator` (`SceneComponent.RelativeRotation` (`self.Lever`))))
  (set `self.OriginXRotation` _relativerotation_roll)
  (set `self.OriginYRotation` _relativerotation_pitch)
  (set `self.OriginZRotation` _relativerotation_yaw))

(event `Activate`
  (if (not (`self.IsAnimating`))
    (set `self.IsAnimating` true)
    (set `self.IsActivating` true)
    (bind (_direction _rotation) (`Timeline|LeverActivation` :!via `PlayFromStart` :!label _label)
      (:`Update`
        (`SceneComponent.K2_SetRelativeRotation` (`self.Lever`) (`KismetMathLibrary.MakeRotator` (`KismetMathLibrary.Lerp` (`self.OriginXRotation`) (`self.TargetRotation`) _rotation) (`self.OriginYRotation`) (`self.OriginZRotation`)) false false))
      (:`Finished`
        (set `self.IsAnimating` false)
        (if (`self.IsActivating`)
          (set `self.Triggered` true)
          (for _array_element (`self.Target`)
            (`/Game/Blueprints/Objects/OutputObjects/BP_Interacted_Object.Activated` _array_element self))
          (else
            (set `self.Triggered` false)
            (for _array_element_2 (`self.Target`)
              (`/Game/Blueprints/Objects/OutputObjects/BP_Interacted_Object.Deactivated` _array_element_2 self))))))))

(event `Deactivate`
  (if (not (`self.IsAnimating`))
    (set `self.IsAnimating` true)
    (set `self.IsActivating` false)
    (goto _label :!via `ReverseFromEnd`)))

(fn `Activation`
  (params (PlayerWhoActivated :type "/Game/Blueprints/Characters/BP_Character_Base Object Reference"))
  (bind _returnvalue (`|GetDataTableRow` "/Game/Sound/DT_Sound_List.DT_Sound_List" "A_Levier_Activation")
    (:`then`
      (`GameplayStatics.PlaySound2D` (break `/Game/Blueprints/Structures/SSound` _returnvalue) 1.0 1.0 0.0 null null)
      (`self.Activate`))))

(fn `Animation`
  (`parent.Animation`))

(fn `Deactivation`
  (params (PlayerWhoActivated :type "/Game/Blueprints/Characters/BP_Character_Base Object Reference") (A :type Boolean))
  (bind _returnvalue (`|GetDataTableRow` "/Game/Sound/DT_Sound_List.DT_Sound_List" "A_Lever_Deactivation")
    (:`then`
      (`GameplayStatics.PlaySound2D` (break `/Game/Blueprints/Structures/SSound` _returnvalue) 1.0 1.0 0.0 null null)
      (`self.Deactivate`))))

(fn `UserConstructionScript`
  (`parent.UserConstructionScript`))