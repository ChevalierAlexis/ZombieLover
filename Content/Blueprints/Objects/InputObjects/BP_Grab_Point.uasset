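; Grapple anchor interactable that the Top character hooks onto.
; On activation, if that character's ray trace is unobstructed, it nudges them, shows their grapple cable and attaches them to the point.
; Leaving range clears the interaction for non-Bottom characters, and a RetractGrapple timeline reels in and hides the cable.
; Swing physics is unfinished: Tick, jump and CutRope events are empty, and the force and release logic is disconnected.
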(event `RetractGrapple`
  (bind (_direction _cablelength) (`Timeline|RetractGrappleTimeline` :!via `PlayFromStart`)
    (:`Update`
      (bind _grabbingactor (`self.GrabbingActor`)
        (:`then`
          (set `CableComponent.CableLength` (`KismetMathLibrary.Lerp` (`/Game/Blueprints/Characters/Components/BP_Grapple_AC.CableTempLength` (`self.GetComponentByClass` (`self.GrabbingActor`) "/Game/Blueprints/Characters/Components/BP_Grapple_AC.BP_Grapple_AC_C")) 0.0 _cablelength) (`/Game/Blueprints/Characters/BP_Character_Top.GrappleCable` _grabbingactor)))
        (:`else`)))
    (:`Finished`
      (bind _grabbingactor_2 (`self.GrabbingActor`)
        (:`then`
          (bind _grapplecable (`/Game/Blueprints/Characters/BP_Character_Top.GrappleCable` _grabbingactor_2))
          (`SceneComponent.SetVisibility` _grapplecable false false)
          (set `CableComponent.bEnableCollision` false _grapplecable))
        (:`else`)))))

(event `EnhancedInput|/Game/Inputs/InputActions/IA_Jump`
  (params (ActionValue :type Boolean) (ElapsedSeconds :type "Float (double-precision)") (TriggeredSeconds :type "Float (double-precision)") (InputAction :type "InputAction Object Reference" :default "/Game/Inputs/InputActions/IA_Jump.IA_Jump")))

(event `Key|A`
  (params (Key :type "Key Structure")))

(event `EnhancedInput|/Game/Inputs/InputActions/IA_Jump_Stop`
  (params (ActionValue :type Boolean) (ElapsedSeconds :type "Float (double-precision)") (TriggeredSeconds :type "Float (double-precision)") (InputAction :type "InputAction Object Reference" :default "/Game/Inputs/InputActions/IA_Jump_Stop.IA_Jump_Stop")))

(event `CutRope`)

(event `self.ReceiveTick`
  (params (DeltaSeconds :type "Float (single-precision)")))

(event `self.InteractionRange.OnComponentEndOverlap`
  (params (OverlappedComponent :type "PrimitiveComponent Object Reference") (OtherActor :type "Actor Object Reference") (OtherComp :type "PrimitiveComponent Object Reference") (OtherBodyIndex :type Integer))
  (bind _needinteraction (`self.NeedInteraction`))
  (if (`self.NeedPlayer`)
    (bind _asbp_character_base (cast `/Game/Blueprints/Characters/BP_Character_Base` OtherActor))
    (cast `/Game/Blueprints/Characters/BP_Character_Bottom` _asbp_character_base
      (:`CastFailed`
        (if _needinteraction
          (if (== (`/Game/Blueprints/Characters/BP_Character_Base.Interactable` _asbp_character_base) self)
            (set `/Game/Blueprints/Characters/BP_Character_Base.Interactable` null _asbp_character_base))
          (if _needinteraction
            (`SceneComponent.SetVisibility` (`self.toucheA`) false false)
            (set `/Game/Blueprints/Characters/Components/BP_Grapple_AC.OwningActor` null (`self.GetComponentByClass` (`self.GrabbingActor`) "/Game/Blueprints/Characters/Components/BP_Grapple_AC.BP_Grapple_AC_C")))
          (else
            (`self.Interract`)))))))

(fn `Activation`
  (params (PlayerWhoActivated :type "/Game/Blueprints/Characters/BP_Character_Base Object Reference"))
  (bind _grabbingactor (`self.GrabbingActor`))
  (`parent.Activation` PlayerWhoActivated)
  (bind _asbp_character_top (cast `/Game/Blueprints/Characters/BP_Character_Top` PlayerWhoActivated))
  (bind _output_get (set `self.GrabbingActor` _asbp_character_top))
  (bind (_outhit _returnvalue) (`KismetSystemLibrary.LineTraceSingle` (`SceneComponent.K2_GetComponentLocation` (`/Game/Blueprints/Characters/BP_Character_Base.RaySource` _output_get)) (- (`SceneComponent.K2_GetComponentLocation` (`/Game/Blueprints/Characters/BP_Character_Base.RaySourceEnd` _output_get)) (0.0 0.0 0.0)) "TraceTypeQuery1"))
  (if (not _returnvalue)
    (`Character.LaunchCharacter` _output_get (25.0 0.0 0.0) false false)
    (bind (_outhit_2 _returnvalue_2) (`KismetSystemLibrary.LineTraceSingle` :`Start` (`self.K2_GetActorLocation` _asbp_character_top) :`End` (`SceneComponent.K2_GetComponentLocation` (`self.Hook`)) :`TraceChannel` "TraceTypeQuery1" :`DrawDebugType` "ForDuration"))
    (set `/Game/Blueprints/Characters/BP_Character_Top.IsCabling` true (`self.GrabbingActor`))
    (`SceneComponent.SetVisibility` (`/Game/Blueprints/Characters/BP_Character_Top.GrappleCable` _grabbingactor) true false)
    (`self.K2_AttachToActor` _grabbingactor self "None" "KeepWorld" "KeepWorld" "KeepWorld" true)))

(fn `UserConstructionScript`)