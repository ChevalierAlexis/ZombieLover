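; Grapple hook point that shows a target logo when it is the player character's best available grab point.
; Each tick it checks that it is the character's nearest grab point and that a Camera-channel line trace from its hook point hits the player.
; The logo stays hidden while the grapple component is already hooked to it.
; A separate event starts a short cooldown flag that a timer resets.
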(event `self.ReceiveTick`
  (params (DeltaSeconds :type "Float (single-precision)"))
  (bind _asbp_character_top (cast `/Game/Blueprints/Characters/BP_Character_Top` (`/Game/Blueprints/Library/BPFL_Fonction_Library.CastToPlayerCharacter`))
    (:`then`
      (bind _asbp_new_grab_point (`/Game/Blueprints/Characters/BP_Character_Top.Find Nearest Grab Point` _asbp_character_top))
      (`/Engine/EditorBlueprintResources/StandardMacros.IsValid` _asbp_new_grab_point
        (:`Is Valid`
          (bind _outhit (`KismetSystemLibrary.LineTraceSingle` :`Start` (`SceneComponent.K2_GetComponentLocation` (`self.HookPoint`)) :`End` (`self.K2_GetActorLocation` _asbp_character_top) :`TraceChannel` "TraceTypeQuery2" :`DrawTime` 1.0))
          (bind _returnvalue (== _asbp_new_grab_point self))
          (set `self.Targeted` (and (== (`.HitActor` (`GameplayStatics.BreakHitResult` _outhit)) (`/Game/Blueprints/Library/BPFL_Fonction_Library.CastToPlayerCharacter`)) _returnvalue)))
        (:`Is Not Valid`
          (set `self.Targeted` false)))
      (`SceneComponent.SetVisibility` (`self.targetLogo`) (and _returnvalue (!= (`/Game/Blueprints/Characters/Components/BP_Grapple_AC.GrabPointHooked` (`/Game/Blueprints/Characters/BP_Character_Top.BP_Grapple_AC` _asbp_character_top)) self) (`self.Targeted`)) false))
    (:`CastFailed`
      (set `self.Targeted` false)
      (`SceneComponent.SetVisibility` (`self.targetLogo`) false false))))

(event `StartCoolDown`
  (if (not (`self.CoolDown`))
    (set `self.CoolDown` true)
    (`KismetSystemLibrary.K2_SetTimerDelegate` (delegate `resetCoolDown`) 0.5)))

(event `resetCoolDown`
  (set `self.CoolDown` false))

(fn `UserConstructionScript`)