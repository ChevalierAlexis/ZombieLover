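; Base interactable that toggles a trigger state and calls Activated or Deactivated on its Target objects.
; When NeedPlayer is set, range overlaps accept characters other than BP_Character_Bottom.
; With NeedInteraction, it registers as the character's Interactable and shows a button prompt while Full or Top characters overlap; otherwise entering and leaving both call Interract.
; Interract is blocked while animating and optionally single-use; Animation is an empty stub.
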(event `self.InteractionRange.OnComponentBeginOverlap`
  (params (OverlappedComponent :type "PrimitiveComponent Object Reference") (OtherActor :type "Actor Object Reference") (OtherComp :type "PrimitiveComponent Object Reference") (OtherBodyIndex :type Integer) (bFromSweep :type Boolean) (SweepResult :type "HitResult Structure (by ref)"))
  (bind _combinearray (`self.combineArray`))
  (if (`self.NeedPlayer`)
    (bind _asbp_character_base (cast `/Game/Blueprints/Characters/BP_Character_Base` OtherActor))
    (cast `/Game/Blueprints/Characters/BP_Character_Bottom` _asbp_character_base
      (:`CastFailed`
        (set `self.Player` _asbp_character_base)
        (if (`self.NeedInteraction`)
          (set `/Game/Blueprints/Characters/BP_Character_Base.Interactable` self _asbp_character_base)
          (set `self.IsPlayerNear` false :!label _label)
          (`KismetArrayLibrary.Array_Clear` (`self.combineArray`))
          (`KismetArrayLibrary.Array_Append` _combinearray (`self.GetOverlappingActors` "/Game/Blueprints/Characters/BP_Character_Full.BP_Character_Full_C"))
          (`KismetArrayLibrary.Array_Append` _combinearray (`self.GetOverlappingActors` "/Game/Blueprints/Characters/BP_Character_Top.BP_Character_Top_C"))
          (for _ _combinearray
            (set `self.IsPlayerNear` true))
          (`SceneComponent.SetVisibility` (`self.toucheA`) (`self.IsPlayerNear`) false)
          (else
            (`self.Interract` :!label _label_2)))))))

(event `self.InteractionRange.OnComponentEndOverlap`
  (params (OverlappedComponent :type "PrimitiveComponent Object Reference") (OtherActor :type "Actor Object Reference") (OtherComp :type "PrimitiveComponent Object Reference") (OtherBodyIndex :type Integer))
  (if (`self.NeedPlayer`)
    (bind _asbp_character_base (cast `/Game/Blueprints/Characters/BP_Character_Base` OtherActor))
    (cast `/Game/Blueprints/Characters/BP_Character_Bottom` _asbp_character_base
      (:`CastFailed`
        (if (`self.NeedInteraction`)
          (if (== (`/Game/Blueprints/Characters/BP_Character_Base.Interactable` _asbp_character_base) self)
            (set `/Game/Blueprints/Characters/BP_Character_Base.Interactable` null _asbp_character_base)
            (goto _label)
            (else
              (goto _label)))
          (else
            (goto _label_2)))))))

(fn `Activation`
  (params (PlayerWhoActivated :type "/Game/Blueprints/Characters/BP_Character_Base Object Reference"))
  (`self.Animation`)
  (set `self.Triggered` true)
  (for _array_element (`self.Target`)
    (`/Game/Blueprints/Objects/OutputObjects/BP_Interacted_Object.Activated` _array_element)))

(fn `Animation`
  (if (`self.Triggered`)
    _))

(fn `Deactivation`
  (params (PlayerWhoActivated :type "/Game/Blueprints/Characters/BP_Character_Base Object Reference") (A :type Boolean))
  (`self.Animation`)
  (set `self.Triggered` false)
  (for _array_element (`self.Target`)
    (`/Game/Blueprints/Objects/OutputObjects/BP_Interacted_Object.Deactivated` _array_element)))

(fn `Interract`
  (if (`self.IsAnimating`)
    _
    (elif (`self.Unique`)
      (if (not (`self.HadBeenUsed`))
        (set `self.HadBeenUsed` true)
        (bind _output_get (set `self.Triggered` (not (`self.Triggered`)) :!label _label))
        (if _output_get
          (`self.Activation` (`self.Player`))
          (else
            (`self.Deactivation` (`self.Player`)))))
      (else
        (goto _label)))))

(fn `UserConstructionScript`)