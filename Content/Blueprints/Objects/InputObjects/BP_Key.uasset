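; Key object that unlocks its targeted BP_DoorLocked or BP_DoubleDoorLocked actors on Interract, then destroys itself.
; While enabled, it bobs vertically through the KeyMoving timeline, which flips direction on each finish.
; While falling, a short downward trace detects ground and replaces the key with a new disabled copy.
; That copy targets every BP_DoorLocked in the level, rather than the original targets.
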(event `self.ReceiveBeginPlay`
  (bind (_returnvalue_x _returnvalue_y _returnvalue_z) (`KismetMathLibrary.BreakVector` (`SceneComponent.K2_GetComponentLocation` (`self.DefaultSceneRoot`))))
  (set `self.KeyOriginXPosition` _returnvalue_x)
  (set `self.KeyOriginYPosition` _returnvalue_y)
  (set `self.KeyOriginZPosition` _returnvalue_z))

(event `self.ReceiveTick`
  (params (DeltaSeconds :type "Float (single-precision)"))
  (bind _returnvalue (`SceneComponent.K2_GetComponentLocation` (`self.Key`)))
  (if (`self.IsFalling`)
    (bind (_outhit _returnvalue_2) (`KismetSystemLibrary.LineTraceSingle` _returnvalue (`KismetMathLibrary.MakeVector` (.x _returnvalue) (.y _returnvalue) (- (.z _returnvalue) 10.0)) "TraceTypeQuery1"))
    (if _returnvalue_2
      (`KismetSystemLibrary.PrintString` "Falling")
      (`PrimitiveComponent.SetSimulatePhysics` (`self.Capsule`) false)
      (bind _outactors (`GameplayStatics.GetAllActorsOfClass` "/Game/Blueprints/Objects/OutputObjects/BP_DoorLocked.BP_DoorLocked_C"))
      (bind _returnvalue_3 (`|SpawnActorFromClass` "BP_Key_C" (`KismetMathLibrary.MakeTransform` (`SceneComponent.GetSocketLocation` (`self.Key`) "None")) "Undefined" "MultiplyWithRoot" self _outactors false null))
      (`KismetSystemLibrary.PrintString` (`KismetSystemLibrary.GetDisplayName` _returnvalue_3))
      (`self.K2_DestroyActor`))
    (elif (`self.Enabled`)
      ;[1 1 1] Oscillation de la clé
      (if (`self.Reverse`)
        (bind (_direction _height) (`Timeline|KeyMoving` :!via `Reverse` :!label _label)
          (:`Update`
            (`SceneComponent.K2_SetWorldLocation` (`self.DefaultSceneRoot`) (`KismetMathLibrary.MakeVector` (`self.KeyOriginXPosition`) (`self.KeyOriginYPosition`) (`KismetMathLibrary.Lerp` (`self.KeyOriginZPosition`) (`self.KeyTargetPosition`) _height)) false false))
          (:`Finished`
            (if (`self.Reverse`)
              (set `self.Reverse` false)
              (else
                (set `self.Reverse` true)))))
        (else
          (goto _label))))))

(fn `Interract`
  (for _array_element (`self.DoorTargeted`)
    (bind _asbp_door_locked (cast `/Game/Blueprints/Objects/OutputObjects/BP_DoorLocked` _array_element)
      (:`then`
        (set `/Game/Blueprints/Objects/OutputObjects/BP_DoorLocked.IsLocked` false _asbp_door_locked))
      (:`CastFailed`
        (bind _asbp_double_door_locked (cast `/Game/Blueprints/Objects/OutputObjects/BP_DoubleDoorLocked` _array_element))
        (set `/Game/Blueprints/Objects/OutputObjects/BP_DoubleDoorLocked.IsLocked` false _asbp_double_door_locked)))
    (`self.K2_DestroyActor`)))

(fn `UserConstructionScript`
  (`parent.UserConstructionScript`))