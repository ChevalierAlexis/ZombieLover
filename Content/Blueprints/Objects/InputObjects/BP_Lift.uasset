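; BP_Lift is an input object: a lever-operated lift that travels vertically between two heights.
; Activation and deactivation swing the Manche lever through a timeline, then run a second timeline forward or backward to move the whole actor root along Z.
; BeginPlay takes the placed height as the start, with GoesDown choosing which end that is.
; The Plane's collision is enabled only while the lift moves.
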(event `self.ReceiveBeginPlay`
  (bind (_relativerotation_roll _relativerotation_pitch _relativerotation_yaw) (`KismetMathLibrary.BreakRotator` (`SceneComponent.RelativeRotation` (`self.Manche`))))
  (bind _z (.z (`SceneComponent.K2_GetComponentLocation` (`self.DefaultSceneRoot`))))
  (`PrimitiveComponent.SetCollisionEnabled` (`self.Plane`) "NoCollision")
  (set `self.OriginXRotation` _relativerotation_roll)
  (set `self.OriginYRotation` _relativerotation_pitch)
  (set `self.OriginZRotation` _relativerotation_yaw)
  (set `self.LiftOriginYPosition` (.y (`SceneComponent.K2_GetComponentLocation` (`self.DefaultSceneRoot`))))
  (set `self.LiftOriginXPosition` (.x (`SceneComponent.K2_GetComponentLocation` (`self.DefaultSceneRoot`))))
  (if (`self.GoesDown?`)
    (bind _output_get (set `self.LiftEndPosition` _z))
    (set `self.LiftOriginZPosition` _output_get)
    (set `self.LiftTargetPosition` (`self.LiftBeginPosition`))
    (else
      (bind _output_get_2 (set `self.LiftBeginPosition` _z))
      (set `self.LiftOriginZPosition` _output_get_2)
      (set `self.LiftTargetPosition` (`self.LiftEndPosition`)))))

(event `Activate`
  (if (not (`self.IsAnimating`))
    (set `self.IsAnimating` true)
    (set `self.IsActivating` true)
    (bind (_direction _rotation) (`Timeline|LeverActivation` :!via `PlayFromStart` :!label _label)
      (:`Update`
        (`SceneComponent.K2_SetRelativeRotation` (`self.Manche`) (`KismetMathLibrary.MakeRotator` (`KismetMathLibrary.Lerp` (`self.OriginXRotation`) (`self.TargetRotation`) _rotation) (`self.OriginYRotation`) (`self.OriginZRotation`)) false false))
      (:`Finished`
        (set `self.IsAnimating` false)
        (if (`self.IsActivating`)
          (set `self.Triggered` true)
          (`self.LiftUp`)
          (else
            (set `self.Triggered` false)
            (`self.LiftDown`)))))))

(event `Deactivate`
  (if (not (`self.IsAnimating`))
    (set `self.IsAnimating` true)
    (set `self.IsActivating` false)
    (goto _label :!via `ReverseFromEnd`)))

(event `LiftUp`
  (`PrimitiveComponent.SetCollisionEnabled` (`self.Plane`) "QueryAndPhysics")
  (`TimelineComponent.SetPlayRate` (`self.LiftMoving`) (`self.MoveSpeed`))
  (bind (_direction _height) (`Timeline|LiftMoving` :!label _label_2)
    (:`Update`
      (`SceneComponent.K2_SetWorldLocation` (`self.DefaultSceneRoot`) (`KismetMathLibrary.MakeVector` (`self.LiftOriginXPosition`) (`self.LiftOriginYPosition`) (`KismetMathLibrary.Lerp` (`self.LiftOriginZPosition`) (`self.LiftTargetPosition`) _height)) false false))
    (:`Finished`
      (`PrimitiveComponent.SetCollisionEnabled` (`self.Plane`) "NoCollision"))))

(event `LiftDown`
  (`PrimitiveComponent.SetCollisionEnabled` (`self.Plane`) "QueryAndPhysics")
  (`TimelineComponent.SetPlayRate` (`self.LiftMoving`) (`self.MoveSpeed`))
  (goto _label_2 :!via `Reverse`))

(fn `Activation`
  (params (PlayerWhoActivated :type "/Game/Blueprints/Characters/BP_Character_Base Object Reference"))
  (`self.Activate`))

(fn `Animation`
  (`parent.Animation`))

(fn `Deactivation`
  (params (PlayerWhoActivated :type "/Game/Blueprints/Characters/BP_Character_Base Object Reference") (A :type Boolean))
  (`self.Deactivate`))

(fn `UserConstructionScript`
  (`parent.UserConstructionScript`))