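; Pressure plate input object that activates while enough weight rests on it and deactivates when the weight drops below the required minimum.
; Overlap begin and end on InteractionRange update a weighted count, with BP_Character_Full counting double any other actor.
; Crossing the threshold calls the parent's Activation or Deactivation and plays or reverses a timeline that sinks or raises the plate.
; A sound from DT_Sound_List plays when either movement finishes.
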(event `self.InteractionRange.OnComponentBeginOverlap`
  (params (OverlappedComponent :type "PrimitiveComponent Object Reference") (OtherActor :type "Actor Object Reference") (OtherComp :type "PrimitiveComponent Object Reference") (OtherBodyIndex :type Integer) (bFromSweep :type Boolean) (SweepResult :type "HitResult Structure (by ref)"))
  (bind _activated (`self.Activated`))
  (bind _amount_on_plate (`self.Amount on Plate`))
  ;[1 1 1] Activation
  (cast `/Game/Blueprints/Characters/BP_Character_Full` OtherActor
    (:`then`
      (set `self.Amount on Plate` (+ _amount_on_plate 2)))
    (:`CastFailed`
      (`/Engine/EditorBlueprintResources/StandardMacros.IncrementInt` _amount_on_plate
        (:`  `
          _))))
  (if (>= _amount_on_plate (`self.Minimum Requiered on Plate`)) :!label _label
    (if (not _activated)
      (set `self.Activated` true)
      (`self.Activation` null)
      (bind (_direction _height) (`Timeline|Plate Pressure` :!label _label_2)
        (:`Update`
          (`SceneComponent.K2_SetRelativeLocation` (`self.Plate`) (`KismetMathLibrary.MakeVector` 0.0 0.0 (`KismetMathLibrary.Lerp` 0.0 -2.0 _height)) false false))
        (:`Finished`
          (if (`self.Activated`)
            ;;[1 1 1] son activation/desactivation
            (bind _returnvalue (`|GetDataTableRow` "/Game/Sound/DT_Sound_List.DT_Sound_List" "A_Pressure_Plate")
              (:`then`
                (`GameplayStatics.PlaySound2D` (break `/Game/Blueprints/Structures/SSound` _returnvalue) 1.0 1.0 0.0 null null)))
            (else
              (bind _returnvalue_2 (`|GetDataTableRow` "/Game/Sound/DT_Sound_List.DT_Sound_List" "A_Pressure_Plate")
                (:`then`
                  (`GameplayStatics.PlaySound2D` (break `/Game/Blueprints/Structures/SSound` _returnvalue_2) 1.0 1.0 0.0 null null))))))))
    (elif _activated
      (set `self.Activated` false)
      (`self.Deactivation` null)
      (goto _label_2 :!via `Reverse`))))

(event `self.InteractionRange.OnComponentEndOverlap`
  (params (OverlappedComponent :type "PrimitiveComponent Object Reference") (OtherActor :type "Actor Object Reference") (OtherComp :type "PrimitiveComponent Object Reference") (OtherBodyIndex :type Integer))
  (bind _amount_on_plate (`self.Amount on Plate`))
  ;[1 1 1] Activation
  (cast `/Game/Blueprints/Characters/BP_Character_Full` OtherActor
    (:`then`
      (set `self.Amount on Plate` (- _amount_on_plate 2))
      (goto _label))
    (:`CastFailed`
      (`/Engine/EditorBlueprintResources/StandardMacros.DecrementInt` _amount_on_plate
        (:`  `
          (goto _label))))))

(fn `Activation`
  (params (PlayerWhoActivated :type "/Game/Blueprints/Characters/BP_Character_Base Object Reference"))
  (`parent.Activation` null))

(fn `Deactivation`
  (params (PlayerWhoActivated :type "/Game/Blueprints/Characters/BP_Character_Base Object Reference"))
  (`parent.Deactivation` null))

(fn `UserConstructionScript`
  (`parent.UserConstructionScript`))