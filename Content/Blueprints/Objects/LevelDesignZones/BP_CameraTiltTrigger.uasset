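; BP_CameraTiltTrigger is a level design trigger volume that changes the camera tilt when a character enters it.
; On box overlap by a BP_Character_Base, it resets that character's base camera and sets the camera manager's FuturCamTilt from NewCamTilt, shifted by -90 degrees.
; A separate SetCamOffSet event, not called in this file, runs a timeline that sets every character's spring arm to zero relative location.
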(event `self.Box.OnComponentBeginOverlap`
  (params (OverlappedComponent :type "PrimitiveComponent Object Reference") (OtherActor :type "Actor Object Reference") (OtherComp :type "PrimitiveComponent Object Reference") (OtherBodyIndex :type Integer) (bFromSweep :type Boolean) (SweepResult :type "HitResult Structure (by ref)"))
  (bind _asbp_character_base (cast `/Game/Blueprints/Characters/BP_Character_Base` OtherActor))
  (`/Game/Blueprints/Characters/BP_Character_Base.ResetBaseCam` _asbp_character_base)
  (set `/Game/Blueprints/CameraManager/BP_Camera_Manager.FuturCamTilt` (+ (`self.NewCamTilt`) -90.0) (`/Game/Blueprints/Library/BPFL_Fonction_Library.GetCameraManager`)))

(event `SetCamOffSet`
  (`Timeline|CamMove`
    (:`Update`
      (bind _outactors (`GameplayStatics.GetAllActorsOfClass` "/Game/Blueprints/Characters/BP_Character_Base.BP_Character_Base_C"))
      (for _array_element _outactors
        (`SceneComponent.K2_SetRelativeLocation` (`/Game/Blueprints/Characters/BP_Character_Base.SpringArm` _array_element) (0.0 0.0 0.0) false false)))))

(fn `UserConstructionScript`)