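; Level-design trigger box that plays a level sequence cutscene when a player-controlled character enters it, once until Respawn resets it.
; On overlap it unbinds the player controller's movement and action events, binds a placeholder jump handler, then starts the sequence.
; When the sequence stops, it rebinds those events, except Merge.
; The Skip event is empty, and its seek-to-end logic is disconnected.
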(event `self.Box.OnComponentBeginOverlap`
  (params (OverlappedComponent :type "PrimitiveComponent Object Reference") (OtherActor :type "Actor Object Reference") (OtherComp :type "PrimitiveComponent Object Reference") (OtherBodyIndex :type Integer) (bFromSweep :type Boolean) (SweepResult :type "HitResult Structure (by ref)"))
  (bind _playercontroller (`self.PlayerController`))
  (bind _sequenceplayer (`LevelSequenceActor.SequencePlayer` (`self.LevelSequencePlayer`)))
  (bind _asbp_character_base (cast `/Game/Blueprints/Characters/BP_Character_Base` OtherActor))
  (bind _asbp_player_controller (cast `/Game/Blueprints/Controllers/BP_Player_Controller` (`Pawn.GetController` _asbp_character_base)))
  (set `self.PlayerController` _asbp_player_controller)
  (`/Engine/EditorBlueprintResources/StandardMacros.IsValid` (`self.LevelSequencePlayer`)
    (:`Is Valid`
      (`/Engine/EditorBlueprintResources/StandardMacros.DoOnce` false :!label _label
        (:`Completed`
          (if true
            (clear `/Game/Blueprints/Controllers/BP_Player_Controller.OnRockCharge` _playercontroller)
            (clear `/Game/Blueprints/Controllers/BP_Player_Controller.OnRockRelease` _playercontroller)
            (clear `/Game/Blueprints/Controllers/BP_Player_Controller.OnMerge` _playercontroller)
            (clear `/Game/Blueprints/Controllers/BP_Player_Controller.OnMoveRight` _playercontroller)
            (clear `/Game/Blueprints/Controllers/BP_Player_Controller.OnMoveFront` _playercontroller)
            (clear `/Game/Blueprints/Controllers/BP_Player_Controller.OnSeparation` _playercontroller)
            (clear `/Game/Blueprints/Controllers/BP_Player_Controller.OnJump` _playercontroller)
            (clear `/Game/Blueprints/Controllers/BP_Player_Controller.OnInteraction` _playercontroller)
            (add `/Game/Blueprints/Controllers/BP_Player_Controller.OnJump` _playercontroller (`|CreateDelegate` :!event `Skip`)))
          (`MovieSceneSequencePlayer.Play` _sequenceplayer)
          (add `MovieSceneSequencePlayer.OnStop` _sequenceplayer (delegate `OnStop_Event`)))))))

(event `Respawn`
  (goto _label :!via `Reset`))

(event `OnStop_Event`
  (bind _playercontroller (`self.PlayerController`))
  (add `/Game/Blueprints/Controllers/BP_Player_Controller.OnSeparation` _playercontroller (`|CreateDelegate` _playercontroller :!event `OnSeparationEvent`))
  (add `/Game/Blueprints/Controllers/BP_Player_Controller.OnInteraction` _playercontroller (`|CreateDelegate` _playercontroller :!event `OnInteractionEvent`))
  (add `/Game/Blueprints/Controllers/BP_Player_Controller.OnMoveFront` _playercontroller (`|CreateDelegate` _playercontroller :!event `MoveFrontEvent`))
  (add `/Game/Blueprints/Controllers/BP_Player_Controller.OnMoveRight` _playercontroller (`|CreateDelegate` _playercontroller :!event `MoveRightEvent`))
  (add `/Game/Blueprints/Controllers/BP_Player_Controller.OnRockCharge` _playercontroller (`|CreateDelegate` _playercontroller :!event `OnRockChargeEvent`))
  (add `/Game/Blueprints/Controllers/BP_Player_Controller.OnRockRelease` _playercontroller (`|CreateDelegate` _playercontroller :!event `RockRelease`))
  (clear `/Game/Blueprints/Controllers/BP_Player_Controller.OnJump` _playercontroller)
  (add `/Game/Blueprints/Controllers/BP_Player_Controller.OnJump` _playercontroller (`|CreateDelegate` _playercontroller :!event `OnJumpEvent`)))

(event `Skip`)

(fn `UserConstructionScript`)