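; BP_Checkpoint is a level checkpoint that becomes current when the full character, or both top and bottom characters, have overlapped its box.
; It registers itself with the camera manager, then looks up the next checkpoint in BP_Checkpoint_List and stores its distance.
; TpToCheckPoint teleports a target to it, clearing zipline use and velocity and snapping the camera trigger.
; Tick tracks player distance to the next checkpoint, but the sun-pitch blend using it is disconnected.
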(event `self.Box.OnComponentBeginOverlap`
  (params (OverlappedComponent :type "PrimitiveComponent Object Reference") (OtherActor :type "Actor Object Reference") (OtherComp :type "PrimitiveComponent Object Reference") (OtherBodyIndex :type Integer) (bFromSweep :type Boolean) (SweepResult :type "HitResult Structure (by ref)"))
  (cast `/Game/Blueprints/Characters/BP_Character_Full` OtherActor
    (:`then`
      (bind (_asbp_camera_manager _pawntarget _checkpoint) (`/Game/Blueprints/Library/BPFL_Fonction_Library.GetCameraManager` :!label _label))
      (if (not (== self _checkpoint))
        (set `/Game/Blueprints/CameraManager/BP_Camera_Manager.CheckPoint` self _asbp_camera_manager)
        (bind _outactors (`GameplayStatics.GetAllActorsOfClass` "/Game/Blueprints/Objects/BP_Checkpoint_List.BP_Checkpoint_List_C"))
        (bind _outactors_2 (`GameplayStatics.GetAllActorsOfClass` "/Game/Blueprints/CameraManager/BP_Camera_Manager.BP_Camera_Manager_C"))
        (bind _checkpointlist (`/Game/Blueprints/Objects/BP_Checkpoint_List.CheckpointList` (`|GetArrayItem` _outactors)))
        (bind _returnvalue (`KismetArrayLibrary.Array_Find` _checkpointlist (`/Game/Blueprints/CameraManager/BP_Camera_Manager.CheckPoint` (`|GetArrayItem` _outactors_2))))
        (`KismetSystemLibrary.PrintString` (`KismetStringLibrary.Conv_IntToString` _returnvalue))
        (bind _output (`|GetArrayItem` _checkpointlist (+ _returnvalue 1)))
        (set `self.NextCheckpoint` _output)
        (set `self.OriginalDistance` (`self.GetDistanceTo` _output))))
    (:`CastFailed`
      (cast `/Game/Blueprints/Characters/BP_Character_Bottom` OtherActor
        (:`then`
          (set `self.BottomValid` true))
        (:`CastFailed`
          (cast `/Game/Blueprints/Characters/BP_Character_Top` OtherActor)
          (set `self.TopValid` true)))
      (if (and (`self.TopValid`) (`self.BottomValid`))
        (goto _label)))))

(event `TpToCheckPoint`
  (params (Target :type "Actor Object Reference"))
  (bind _camtriggerref (`self.CamTriggerRef`))
  (`self.K2_SetActorLocation` Target (`SceneComponent.K2_GetComponentLocation` (`self.PaperFlipbook`)) false false)
  (bind _asbp_character_base (cast `/Game/Blueprints/Characters/BP_Character_Base` Target))
  (bind _ziplineused (`/Game/Blueprints/Characters/BP_Character_Base.ZipLineUsed` _asbp_character_base))
  (`/Engine/EditorBlueprintResources/StandardMacros.IsValid` _ziplineused
    (:`Is Valid`
      (set `/Game/Blueprints/Objects/BP_ZipLine.IsUsedNow` false _ziplineused))
    (:`Is Not Valid`
      _))
  (set `MovementComponent.Velocity` (0.0 0.0 0.0) (`Character.CharacterMovement` _asbp_character_base))
  (`/Engine/EditorBlueprintResources/StandardMacros.IsValid` _camtriggerref
    (:`Is Valid`
      (`/Game/Blueprints/Objects/LevelDesignZones/BP_CameraTrigger.InstantCamUpdate` _camtriggerref (`/Game/Blueprints/Library/BPFL_Fonction_Library.CastToPlayerCharacter`)))))

(event `self.ReceiveTick`
  (params (DeltaSeconds :type "Float (single-precision)"))
  (bind _output_get (set `self.TempDistance` (`self.GetDistanceTo` (`GameplayStatics.GetPlayerCharacter` 0) (`self.NextCheckpoint`)))))

(fn `UserConstructionScript`)