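; Level design trigger zone that pops a tutorial UI when a BP_Character_Base enters its box.
; A selector enum picks the tutorial, and the overlap fires PopTuto on the camera manager's UiTuto widget only once, skipping one specific enum value.
; The construction script writes the selected enum name to a text render component as a label.
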(event `self.Box.OnComponentBeginOverlap`
  (params (OverlappedComponent :type "PrimitiveComponent Object Reference") (OtherActor :type "Actor Object Reference") (OtherComp :type "PrimitiveComponent Object Reference") (OtherBodyIndex :type Integer) (bFromSweep :type Boolean) (SweepResult :type "HitResult Structure (by ref)"))
  (bind _tutoselector (`self.TutoSelector`))
  (cast `/Game/Blueprints/Characters/BP_Character_Base` OtherActor)
  (if (`|EnumInequality` _tutoselector "NewEnumerator3")
    (`/Engine/EditorBlueprintResources/StandardMacros.DoOnce` false
      (:`Completed`
        (`/Game/Blueprints/UI/WPB_UI_Tuto.PopTuto` (`/Game/Blueprints/CameraManager/BP_Camera_Manager.UiTuto` (`/Game/Blueprints/Library/BPFL_Fonction_Library.GetCameraManager`)) _tutoselector true 1.0)))))

(event `self.ReceiveTick`
  (params (DeltaSeconds :type "Float (single-precision)")))

(fn `UserConstructionScript`
  (`TextRenderComponent.K2_SetText` (`self.TextRender`) (`KismetTextLibrary.Conv_StringToText` (`|GetEnumeratorNameAsString` (`self.TutoSelector`)))))