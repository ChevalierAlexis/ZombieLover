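; Falling trunk world object that helps characters stay centered on it and replaces itself with a fresh copy when its respawn component fires.
; An interaction range shows the ToucheA prompt only to the bottom character.
; Each tick, characters in SnapZone without forward input get a curve-driven Y force toward its center when airborne or moving sideways.
; Near the center, their sideways velocity is clamped to damp overshoot.
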(event `self.ReceiveBeginPlay`
  (add `/Game/Blueprints/Characters/Components/BP_Respawn_AC.Respawn` (`self.BP_Respawn_AC`) (delegate `RespawnEvent`)))

(event `RespawnEvent`
  (`|SpawnActorFromClass` "BP_FallingTrunk_C" (`self.GetTransform`) "Undefined" "MultiplyWithRoot" null null)
  (`self.K2_DestroyActor`))

(event `self.InteractionRange.OnComponentBeginOverlap`
  (params (OverlappedComponent :type "PrimitiveComponent Object Reference") (OtherActor :type "Actor Object Reference") (OtherComp :type "PrimitiveComponent Object Reference") (OtherBodyIndex :type Integer) (bFromSweep :type Boolean) (SweepResult :type "HitResult Structure (by ref)"))
  (cast `/Game/Blueprints/Characters/BP_Character_Bottom` OtherActor)
  (`SceneComponent.SetVisibility` (`self.ToucheA`) true false))

(event `self.InteractionRange.OnComponentEndOverlap`
  (params (OverlappedComponent :type "PrimitiveComponent Object Reference") (OtherActor :type "Actor Object Reference") (OtherComp :type "PrimitiveComponent Object Reference") (OtherBodyIndex :type Integer))
  (cast `/Game/Blueprints/Characters/BP_Character_Bottom` OtherActor)
  (`SceneComponent.SetVisibility` (`self.ToucheA`) false false))

(event `self.ReceiveTick`
  (params (DeltaSeconds :type "Float (single-precision)"))
  (bind _overlappingactors (`PrimitiveComponent.GetOverlappingActors` (`self.SnapZone`) "/Game/Blueprints/Characters/BP_Character_Base.BP_Character_Base_C"))
  (bind (_returnvalue_x _returnvalue_y) (`KismetMathLibrary.BreakVector` (`SceneComponent.K2_GetComponentLocation` (`self.SnapZone`))))
  ;[1 1 1] snapping
  (if (`KismetArrayLibrary.Array_IsNotEmpty` _overlappingactors)
    (for _array_element _overlappingactors
      (bind _asbp_character_base (cast `/Game/Blueprints/Characters/BP_Character_Base` _array_element))
      (bind (_ia_move_right _ia_move_front) (`/Game/Blueprints/Characters/BP_Character_Base.Get IA_Move` _asbp_character_base))
      (if (and (or (not (`/Game/Blueprints/Characters/BP_Character_Base.IsOnGround` _asbp_character_base)) (!= _ia_move_right 0.0)) (== _ia_move_front 0.0))
        (bind _charactermovement (`Character.CharacterMovement` _asbp_character_base))
        (bind (_returnvalue_x_2 _returnvalue_y_2) (`KismetMathLibrary.BreakVector` (`SceneComponent.K2_GetComponentLocation` (`Character.CapsuleComponent` _asbp_character_base))))
        (bind _returnvalue (`CurveFloat.GetFloatValue` (`self.curveSnap`) (`KismetMathLibrary.FClamp` (/ (- _returnvalue_y _returnvalue_y_2) 70.0) -1.0)))
        (`CharacterMovementComponent.AddForce` _charactermovement (`KismetMathLibrary.MakeVector` 0.0 (* _returnvalue 50000.0))))
      (if (< (- (`KismetMathLibrary.Abs` _returnvalue) 0.1) 0.0)
        (bind (_velocity_x _velocity_y _velocity_z) (`KismetMathLibrary.BreakVector` (`MovementComponent.Velocity` _charactermovement)))
        (set `MovementComponent.Velocity` (`KismetMathLibrary.MakeVector` _velocity_x (`KismetMathLibrary.FClamp` _velocity_y -40.0 40.0) _velocity_z) _charactermovement)))))

(fn `UserConstructionScript`)