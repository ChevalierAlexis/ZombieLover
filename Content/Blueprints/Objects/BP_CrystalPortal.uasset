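; BP_CrystalPortal is a portal object that continuously animates its Crystal component's height, starting on BeginPlay.
; A timeline curve lerps the crystal's relative Z between its starting height and Target, with sweep enabled.
; Each time the timeline finishes, it flips the On flag to choose between replaying from the start and reversing from the end, so the motion loops indefinitely.
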(event `self.ReceiveBeginPlay`
  (bind (_relativelocation_x _relativelocation_y _relativelocation_z) (`KismetMathLibrary.BreakVector` (`SceneComponent.RelativeLocation` (`self.Crystal`))))
  (set `self.origin` _relativelocation_z)
  (`self.Activation`))

(event `self.ReceiveTick`
  (params (DeltaSeconds :type "Float (single-precision)")))

(event `Activation`
  (bind (_direction _crystal) (`Timeline|Timeline` :!via `PlayFromStart` :!label _label)
    (:`Update`
      (`SceneComponent.K2_SetRelativeLocation` (`self.Crystal`) (`KismetMathLibrary.MakeVector` 0.0 0.0 (`KismetMathLibrary.Lerp` (`self.origin`) (`self.Target`) _crystal)) true false))
    (:`Finished`
      (bind _output_get (set `self.On` (not (`self.On`))))
      (if _output_get
        (`self.Activation`)
        (else
          (`self.deactivation`))))))

(event `deactivation`
  (goto _label :!via `ReverseFromEnd`))

(fn `UserConstructionScript`)