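; Camera trigger volume that blends the player camera to a new pitch, spring arm length and sensor width while a BP_Character_Base is inside.
; On begin overlap it caches the character's current values, then a timeline lerps them to the configured targets, preserving roll and yaw.
; End overlap reverses that timeline without checking which actor left.
; RotationSpeed sets the timeline's play rate at BeginPlay.
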(event `self.ReceiveBeginPlay`
  (`TimelineComponent.SetPlayRate` (`self.camRotaion`) (`self.RotationSpeed`)))

(event `self.Box.OnComponentBeginOverlap`
  (params (OverlappedComponent :type "PrimitiveComponent Object Reference") (OtherActor :type "Actor Object Reference") (OtherComp :type "PrimitiveComponent Object Reference") (OtherBodyIndex :type Integer) (bFromSweep :type Boolean) (SweepResult :type "HitResult Structure (by ref)"))
  (bind _asbp_character_base (cast `/Game/Blueprints/Characters/BP_Character_Base` OtherActor))
  (`|ExecutionSequence`
    (:`then_0`
      (set `self.Base sensor width` (`/Game/Blueprints/Characters/BP_Character_Base.Sensor Width (Mm)` _asbp_character_base)))
    (:`then_1`
      (bind _springarm (`/Game/Blueprints/Characters/BP_Character_Base.SpringArm` _asbp_character_base))
      (set `self.BaseCameraDistance` (`SpringArmComponent.TargetArmLength` _springarm)))
    (:`then_2`
      (set `self.BaseRotation` (.pitch (`SpringArmComponent.GetTargetRotation` _springarm))))
    (:`then_3`
      (bind (_direction _alpha) (`Timeline|camRotaion` :!via `PlayFromStart` :!label _label)
        (:`Update`
          (`|ExecutionSequence`
            (:`then_0`
              (`SceneComponent.K2_SetWorldRotation` _springarm (`KismetMathLibrary.MakeRotator` (.roll (`SpringArmComponent.GetTargetRotation` _springarm)) (`KismetMathLibrary.Lerp` (`self.BaseRotation`) (`self.newRotation`) _alpha) (.yaw (`SpringArmComponent.GetTargetRotation` _springarm))) false false))
            (:`then_1`
              (set `/Game/Blueprints/Characters/BP_Character_Base.Sensor Width (Mm)` (`KismetMathLibrary.Lerp` (`self.Base sensor width`) (`self.NewSensorWidth`) _alpha) _asbp_character_base))
            (:`then_2`
              (set `SpringArmComponent.TargetArmLength` (`KismetMathLibrary.Lerp` (`self.BaseCameraDistance`) (`self.NewCameraDistance`) _alpha) (`/Game/Blueprints/Characters/BP_Character_Base.SpringArm` _asbp_character_base)))))))))

(event `self.Box.OnComponentEndOverlap`
  (params (OverlappedComponent :type "PrimitiveComponent Object Reference") (OtherActor :type "Actor Object Reference") (OtherComp :type "PrimitiveComponent Object Reference") (OtherBodyIndex :type Integer))
  (goto _label :!via `Reverse`))

(fn `UserConstructionScript`)