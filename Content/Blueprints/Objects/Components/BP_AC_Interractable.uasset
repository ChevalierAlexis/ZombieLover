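; Interaction component that makes its owning actor interactable by broadcasting OnInterractAction with the player avatar and controller when Interract is called.
; On BeginPlay it reuses the owner's sphere component, or adds a scaled one if none exists, and binds its overlap events.
; Begin overlap caches the BP_Character_Full as PlayerAvatar, which is never cleared.
; Registration and removal with the zombie player controller are disconnected, so overlaps never notify it.
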(event `self.ReceiveBeginPlay`
  (bind _returnvalue (`Actor.GetComponentByClass` (`self.Owner`) "/Script/Engine.SphereComponent"))
  (set `self.Owner` (`self.GetOwner`))
  (`|ExecutionSequence`
    (:`then_0`
      ;[1 0.6841 0] Add and Set Sphere collider
      (`/Engine/EditorBlueprintResources/StandardMacros.IsValid` _returnvalue
        (:`Is Valid`
          (set `self.SphereCollider` _returnvalue))
        (:`Is Not Valid`
          (bind _returnvalue_2 (`|AddComponentByClass` (`self.Owner`) "/Script/Engine.SphereComponent" false (`KismetMathLibrary.MakeTransform` (0.0 0.0 0.0) (struct) (1.0 10.0 10.0))))
          (set `self.SphereCollider` _returnvalue_2))))
    (:`then_1`
      (add `PrimitiveComponent.OnComponentBeginOverlap` (`self.SphereCollider`) (`|CreateDelegate` :!event `OnOverlapSphere`))
      (add `PrimitiveComponent.OnComponentEndOverlap` (`self.SphereCollider`) (`|CreateDelegate` :!event `OnEndOverlapSphere`)))))

(fn `Interract`
  (params (Controller :type "/Game/Blueprints/Controllers/BP_Player_Controller Object Reference"))
  (`self.OnInterractAction` (`self.PlayerAvatar`) Controller))

(fn `OnEndOverlapSphere`
  (params (OverlappedComponent :type "PrimitiveComponent Object Reference") (OtherActor :type "Actor Object Reference") (OtherComp :type "PrimitiveComponent Object Reference") (OtherBodyIndex :type Integer))
  (cast `/Game/Blueprints/Characters/BP_Character_Full` OtherActor))

(fn `OnOverlapSphere`
  (params (OverlappedComponent :type "PrimitiveComponent Object Reference") (OtherActor :type "Actor Object Reference") (OtherComp :type "PrimitiveComponent Object Reference") (OtherBodyIndex :type Integer) (bFromSweep :type Boolean) (SweepResult :type "HitResult Structure (by ref)"))
  (bind _asbp_character_full (cast `/Game/Blueprints/Characters/BP_Character_Full` OtherActor))
  (set `self.PlayerAvatar` _asbp_character_full))