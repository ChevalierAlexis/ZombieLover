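; Short-range projectile that alerts enemy AI to its thrower or triggers other stonable objects on overlap.
; The construction script feeds its Velocity into ProjectileMovement, and the capsule ignores the instigator while moving.
; Overlaps act only on actors with BP_Stonable_AC, calling OnActivation on non-enemies.
; For enemies, it suspends AI perception for a few seconds and forces blackboard line of sight, with the instigator as Player.
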(event `self.ReceiveBeginPlay`
  (`PrimitiveComponent.IgnoreActorWhenMoving` (`self.Capsule`) (`self.Instigator`) true))

(event `self.ReceiveTick`
  (params (DeltaSeconds :type "Float (single-precision)")))

(event `self.Capsule.OnComponentBeginOverlap`
  (params (OverlappedComponent :type "PrimitiveComponent Object Reference") (OtherActor :type "Actor Object Reference") (OtherComp :type "PrimitiveComponent Object Reference") (OtherBodyIndex :type Integer) (bFromSweep :type Boolean) (SweepResult :type "HitResult Structure (by ref)"))
  (bind _returnvalue (`self.GetComponentByClass` OtherActor "/Game/Blueprints/Characters/Components/BP_Stonable_AC.BP_Stonable_AC_C"))
  (bind _returnvalue_2 (`AIBlueprintHelperLibrary.GetAIController` OtherActor))
  (bind _returnvalue_3 (`self.GetComponentByClass` _returnvalue_2 "/Script/AIModule.BlackboardComponent"))
  (bind _returnvalue_4 (`self.GetComponentByClass` _returnvalue_2 "/Script/AIModule.AIPerceptionComponent"))
  (`/Engine/EditorBlueprintResources/StandardMacros.IsValid` _returnvalue
    (:`Is Valid`
      (if (`/Game/Blueprints/Characters/Components/BP_Stonable_AC.IsEnnemi` _returnvalue)
        (`ActorComponent.Deactivate` _returnvalue_4)
        (`BlackboardComponent.SetValueAsBool` _returnvalue_3 "HasLineOfSight" true)
        (`BlackboardComponent.SetValueAsObject` _returnvalue_3 "Player" (`self.GetInstigator`))
        (`KismetSystemLibrary.Delay` 5.0)
        (`ActorComponent.Activate` _returnvalue_4 false)
        (else
          (`/Game/Blueprints/Characters/Components/BP_Stonable_AC.OnActivation` _returnvalue))))))

(fn `UserConstructionScript`
  (set `MovementComponent.Velocity` (`self.Velocity`) (`self.ProjectileMovement`)))