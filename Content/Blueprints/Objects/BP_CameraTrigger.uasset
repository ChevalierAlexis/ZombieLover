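; Camera trigger volume that changes a character's spring arm pitch, arm length and sensor width on entering its box.
; A timeline blends from the captured current values to the trigger's targets, and the character records its active trigger to ignore re-entry.
; Unless Gate is set, exiting the active trigger with collision enabled reverses the blend toward hard-coded defaults.
; InstantCamUpdate snaps straight to the target values.
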(event `self.ReceiveBeginPlay`
  (`TimelineComponent.SetPlayRate` (`self.camRotation`) (`self.RotationSpeed`)))

(event `self.Box.OnComponentBeginOverlap`
  (params (OverlappedComponent :type "PrimitiveComponent Object Reference") (OtherActor :type "Actor Object Reference") (OtherComp :type "PrimitiveComponent Object Reference") (OtherBodyIndex :type Integer) (bFromSweep :type Boolean) (SweepResult :type "HitResult Structure (by ref)"))
  (bind _asbp_character_base (cast `/Game/Blueprints/Characters/BP_Character_Base` OtherActor))
  (bind _output_get (set `self.ActorTargeted` _asbp_character_base))
  (bind _currentcameratrigger (`/Game/Blueprints/Characters/BP_Character_Base.CurrentCameraTrigger` _output_get))
  ;[1 1 1] Overide le précédent movement de cam et ne fais rien si c'est la même
  (`/Engine/EditorBlueprintResources/StandardMacros.IsValid` _currentcameratrigger
    (:`Is Valid`
      (if (not (== _currentcameratrigger self))
        (`self.CancelCamMovement`)
        (set `/Game/Blueprints/Characters/BP_Character_Base.CurrentCameraTrigger` self _output_get :!label _label)
        (`self.SetBaseVariable` _output_get)
        (bind (_direction _alpha) (`Timeline|camRotation` :!via `PlayFromStart` :!label _label_2)
          (:`Update`
            (`/Engine/EditorBlueprintResources/StandardMacros.IsValid` _output_get
              (:`Is Valid`
                (`|ExecutionSequence`
                  (:`then_0`
                    (bind _springarm (`/Game/Blueprints/Characters/BP_Character_Base.SpringArm` _output_get))
                    (`SceneComponent.K2_SetWorldRotation` _springarm (`KismetMathLibrary.MakeRotator` (.roll (`SpringArmComponent.GetTargetRotation` _springarm)) (`KismetMathLibrary.Lerp` (`self.BaseRotation`) (`self.newRotationY`) _alpha) (.yaw (`SpringArmComponent.GetTargetRotation` _springarm))) false false)
                    (`/Game/Blueprints/Characters/BP_Character_Base.FocusUpdate` (`self.ActorTargeted`)))
                  (:`then_1`
                    (set `/Game/Blueprints/Characters/BP_Character_Base.Sensor Width (Mm)` (`KismetMathLibrary.Lerp` (`self.Base sensor width`) (`self.NewSensorWidth`) _alpha) _output_get))
                  (:`then_2`
                    (set `SpringArmComponent.TargetArmLength` (`KismetMathLibrary.Lerp` (`self.BaseCameraDistance`) (`self.NewCameraDistance`) _alpha) _springarm)))))))))
    (:`Is Not Valid`
      (goto _label))))

(event `CancelCamMovement`
  (goto _label_2 :!via `Stop`))

(event `ReverseCamMovement`
  (goto _label_2 :!via `ReverseFromEnd`))

(event `self.Box.OnComponentEndOverlap`
  (params (OverlappedComponent :type "PrimitiveComponent Object Reference") (OtherActor :type "Actor Object Reference") (OtherComp :type "PrimitiveComponent Object Reference") (OtherBodyIndex :type Integer))
  (if (not (`self.Gate`))
    (bind _asbp_character_base (cast `/Game/Blueprints/Characters/BP_Character_Base` OtherActor))
    (bind _output_get (set `self.ActorTargeted` _asbp_character_base))
    (bind _currentcameratrigger (`/Game/Blueprints/Characters/BP_Character_Base.CurrentCameraTrigger` _output_get))
    (`/Engine/EditorBlueprintResources/StandardMacros.IsValid` _currentcameratrigger
      (:`Is Valid`
        (if (== _currentcameratrigger self)
          (if (not (== (`KismetMathLibrary.Conv_ByteToDouble` (`PrimitiveComponent.GetCollisionEnabled` (`Character.CapsuleComponent` _output_get))) 0.0))
            (`self.SetBaseVariAbleToDefault`)
            (`self.ReverseCamMovement`)
            (set `/Game/Blueprints/Characters/BP_Character_Base.CurrentCameraTrigger` null (`self.ActorTargeted`))))))))

(event `SetBaseVariable`
  (params (Target :type "/Game/Blueprints/Characters/BP_Character_Base Object Reference"))
  (bind _springarm (`/Game/Blueprints/Characters/BP_Character_Base.SpringArm` Target))
  ;[1 1 1] setBaseVar
  (set `self.Base sensor width` (`/Game/Blueprints/Characters/BP_Character_Base.Sensor Width (Mm)` Target))
  (set `self.BaseCameraDistance` (`SpringArmComponent.TargetArmLength` _springarm))
  (set `self.BaseRotation` (.pitch (`SpringArmComponent.GetTargetRotation` _springarm))))

(event `SetBaseVariableToDefault`
  ;[1 1 1] setBaseVar
  (set `self.Base sensor width` 30.0)
  (set `self.BaseCameraDistance` 1500.0)
  (set `self.BaseRotation` -9.0))

(event `InstantCamUpdate`
  (params (CharacterTarget :type "/Game/Blueprints/Characters/BP_Character_Base Object Reference"))
  (bind _springarm (`/Game/Blueprints/Characters/BP_Character_Base.SpringArm` CharacterTarget))
  ;[1 1 1] Instant cam update
  (`self.CancelCamMovement`)
  (`|ExecutionSequence`
    (:`then_0`
      (`SceneComponent.K2_SetWorldRotation` _springarm (`KismetMathLibrary.MakeRotator` (.roll (`SpringArmComponent.GetTargetRotation` _springarm)) (`self.newRotationY`) (.yaw (`SpringArmComponent.GetTargetRotation` _springarm))) false false))
    (:`then_1`
      (set `SpringArmComponent.TargetArmLength` (`self.NewCameraDistance`) _springarm))
    (:`then_2`
      (set `/Game/Blueprints/Characters/BP_Character_Base.Sensor Width (Mm)` (`self.NewSensorWidth`) CharacterTarget))))

(fn `UserConstructionScript`)