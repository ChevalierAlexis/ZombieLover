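; BP_Climb is a climbable volume, optionally a ladder, that switches the player into climbing movement while inside its InteractionRange.
; Capsule overlaps from a BP_Character_Base toggle IsClimbed and call Activation or Deactivation.
; Activation rebinds the player controller's forward-move delegate, drops right-move for ladders and sets Flying mode.
; Deactivation rebinds both move delegates and restores Walking; the interact event is an empty stub.
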(event `self.InteractionRange.OnComponentBeginOverlap`
  (params (OverlappedComponent :type "PrimitiveComponent Object Reference") (OtherActor :type "Actor Object Reference") (OtherComp :type "PrimitiveComponent Object Reference") (OtherBodyIndex :type Integer) (bFromSweep :type Boolean) (SweepResult :type "HitResult Structure (by ref)"))
  (if (not (`self.IsClimbed`))
    (bind _asbp_character_base (cast `/Game/Blueprints/Characters/BP_Character_Base` OtherActor))
    (if (== (`Character.CapsuleComponent` _asbp_character_base) OtherComp)
      (set `self.IsClimbed` true)
      (`self.Activation`))))

(event `self.InteractionRange.OnComponentEndOverlap`
  (params (OverlappedComponent :type "PrimitiveComponent Object Reference") (OtherActor :type "Actor Object Reference") (OtherComp :type "PrimitiveComponent Object Reference") (OtherBodyIndex :type Integer))
  (if (`self.IsClimbed`)
    (bind _asbp_character_base (cast `/Game/Blueprints/Characters/BP_Character_Base` OtherActor))
    (if (== (`Character.CapsuleComponent` _asbp_character_base) OtherComp)
      (set `self.IsClimbed` false)
      (`self.Deactivation`))))

(event `self.BP_AC_Interractable.OnInterractAction`
  (params (Avatar :type "/Game/Blueprints/Characters/BP_Character_Full Object Reference") (Controller :type "/Game/Blueprints/BP_Player_Controller Object Reference")))

(fn `Activation`
  (`KismetSystemLibrary.PrintString` "In")
  (bind _asbp_player_controller (cast `/Game/Blueprints/BP_Player_Controller` (`GameplayStatics.GetPlayerController` 0)))
  (`/Engine/EditorBlueprintResources/StandardMacros.IsValid` _asbp_player_controller
    (:`Is Valid`
      (clear `/Game/Blueprints/BP_Player_Controller.OnMoveFront` _asbp_player_controller)
      (if (`self.IsLadder`)
        (clear `/Game/Blueprints/BP_Player_Controller.OnMoveRight` _asbp_player_controller))
      (add `/Game/Blueprints/BP_Player_Controller.OnMoveFront` _asbp_player_controller (`|CreateDelegate` _asbp_player_controller :!event `Grounded Climbing`))
      (set `/Game/Blueprints/BP_Player_Controller.Ladder` (`self.IsLadder`) _asbp_player_controller)
      (`CharacterMovementComponent.SetMovementMode` (`Character.CharacterMovement` (`/Game/Blueprints/Library/BPFL_Fonction_Library.CastToPlayerCharacter`)) "MOVE_Flying" 0))))

(fn `Deactivation`
  (`KismetSystemLibrary.PrintString` "Out")
  (bind _asbp_player_controller (cast `/Game/Blueprints/BP_Player_Controller` (`GameplayStatics.GetPlayerController` 0)))
  (`/Engine/EditorBlueprintResources/StandardMacros.IsValid` _asbp_player_controller
    (:`Is Valid`
      (clear `/Game/Blueprints/BP_Player_Controller.OnMoveFront` _asbp_player_controller)
      (clear `/Game/Blueprints/BP_Player_Controller.OnMoveRight` _asbp_player_controller)
      (add `/Game/Blueprints/BP_Player_Controller.OnMoveFront` _asbp_player_controller (`|CreateDelegate` _asbp_player_controller :!event `MoveFrontEvent`))
      (add `/Game/Blueprints/BP_Player_Controller.OnMoveRight` _asbp_player_controller (`|CreateDelegate` _asbp_player_controller :!event `MoveRightEvent`))
      (`CharacterMovementComponent.SetMovementMode` (`Character.CharacterMovement` (`/Game/Blueprints/Library/BPFL_Fonction_Library.CastToPlayerCharacter`)) "MOVE_Walking" 0))))

(fn `UserConstructionScript`)