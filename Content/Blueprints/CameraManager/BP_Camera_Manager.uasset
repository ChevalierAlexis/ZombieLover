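; Player camera manager that also owns the game's tutorial, death, pause and options widgets.
; BeginPlay creates the widgets, showing tutorial and death popup in the viewport.
; PopDeathUi pauses and toggles the popup; PopPauseMenu either dismisses it and respawns the player or, if allowed, toggles pause menu, cursor and input mode.
; BlueprintUpdateCamera derives a view from the pawn's camera with pinned Y, but returns false, leaving default camera logic active.
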(event `self.ReceiveBeginPlay`
  (bind _returnvalue (`GameplayStatics.GetPlayerController` 0))
  (bind _returnvalue_2 (`|CreateWidget` "/Game/Blueprints/UI/WPB_UI_Tuto.WPB_UI_Tuto_C" _returnvalue))
  (bind _output_get (set `self.UiTuto` _returnvalue_2))
  (`UserWidget.AddToViewport` _output_get 0)
  (bind _returnvalue_3 (`|CreateWidget` "/Game/Blueprints/UI/WBP_UI_Death_PopUp.WBP_UI_Death_PopUp_C" _returnvalue))
  (bind _output_get_2 (set `self.UiDeathPopUp` _returnvalue_3))
  (`UserWidget.AddToViewport` _output_get_2 0)
  (bind _returnvalue_4 (`|CreateWidget` "/Game/Blueprints/UI/WBP_UI_Pause.WBP_UI_Pause_C" _returnvalue))
  (set `self.UiPause` _returnvalue_4)
  (bind _returnvalue_5 (`|CreateWidget` "/Game/Blueprints/UI/WBP_UI_Options.WBP_UI_Options_C" _returnvalue))
  (set `self.UiOptions` _returnvalue_5))

(event `PopDeathUi`
  (params (Visible :type Boolean))
  (bind _uideathpopup (`self.UiDeathPopUp`))
  (`GameplayStatics.SetGamePaused` Visible)
  (if Visible
    (`Widget.SetVisibility` _uideathpopup "Visible")
    (else
      (`Widget.SetVisibility` _uideathpopup "Hidden"))))

(event `PopPauseMenu`
  (bind _uipause (`self.UiPause`))
  (bind _uipause_2 (`self.UiPause`))
  (bind _returnvalue (`Widget.GetOwningPlayer` _uipause_2))
  (bind _returnvalue_2 (`Widget.IsInViewport` _uipause))
  (bind _returnvalue_3 (not _returnvalue_2))
  (if (`|EnumEquality` (`Widget.Visibility` (`self.UiDeathPopUp`)) "Visible")
    (`self.PopDeathUi` false)
    (`/Game/Blueprints/Characters/BP_Character_Base.Respawn` (`/Game/Blueprints/Library/BPFL_Fonction_Library.CastToPlayerCharacter`))
    (elif (`self.CanPause`)
      (`GameplayStatics.SetGamePaused` _returnvalue_3)
      (set `PlayerController.bShowMouseCursor` _returnvalue_3 (`Widget.GetOwningPlayer` _uipause))
      (if _returnvalue_2
        (`Widget.RemoveFromParent` _uipause_2)
        (`WidgetBlueprintLibrary.SetInputMode_GameOnly` _returnvalue)
        (else
          (`UserWidget.AddToViewport` _uipause_2 0)
          (`WidgetBlueprintLibrary.SetInputMode_GameAndUIEx` _returnvalue (`self.UiPause`)))))))

(fn `BlueprintUpdateCamera`
  (params (CameraTarget :type "Actor Object Reference"))
  (returns (NewCameraLocation :type "Vector Structure") (NewCameraRotation :type "Rotator Structure") (NewCameraFOV :type "Float (single-precision)") (ReturnValue :type Boolean))
  (bind _pawntarget (`self.PawnTarget`))
  (bind _camera (`/Game/Blueprints/Characters/BP_Character_Base.Camera` _pawntarget))
  (bind (_returnvalue_location _returnvalue_rotation) (`KismetMathLibrary.BreakTransform` (`SceneComponent.K2_GetComponentToWorld` _camera)))
  (bind _returnvalue (+ (`SpringArmComponent.TargetArmLength` (`/Game/Blueprints/Characters/BP_Character_Base.SpringArm` _pawntarget)) 1000.0))
  (`/Engine/EditorBlueprintResources/StandardMacros.IsValid` _pawntarget
    (:`Is Valid`
      (return (`KismetMathLibrary.MakeVector` (.x _returnvalue_location) (`KismetMathLibrary.FClamp` (.y _returnvalue_location) _returnvalue _returnvalue) (.z _returnvalue_location)) _returnvalue_rotation (`CameraComponent.FieldOfView` _camera) false))
    (:`Is Not Valid`
      (return (0.0 0.0 0.0) (struct) 0.0 false))))

(fn `UserConstructionScript`)